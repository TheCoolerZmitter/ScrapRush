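; Actor component that manages health, damage, healing and status effects for players and enemies.
; TakeDamage filters hits through immunity, invincibility and blocking, handles lifesteal, death and kill credit, and fires block, death and response dispatchers.
; Fire and poison follow lethal or interrupting hits, looping on Delays that re-enter TakeDamage as Projectile damage to avoid reapplying themselves.
; It also provides timed invulnerability, temporary Strength weakening, and Niagara visuals for burning and immunities.
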(event `GrantFireImmunity`
  (bind _fireimmune (`self.FireImmune`))
  (set `self.ImmuneToFire` true)
  (`/Engine/EditorBlueprintResources/StandardMacros.IsValid` _fireimmune
    (:`Is Valid`
      (`self.K2_DestroyComponent` _fireimmune))
    (:`Is Not Valid`
      _))
  (bind _returnvalue (`NiagaraFunctionLibrary.SpawnSystemAttached` "/Game/M5VFXVOL2/Niagara/Reference/Fire/8_Nflame_pt.8_Nflame_pt" (`Actor.RootComponent` (`self.GetOwner`)) "None" (0.0 0.0 -5.0) (struct) "KeepRelativeOffset"))
  (set `self.FireImmune` _returnvalue))

(event `Unweaken`
  (params (Amount :type "Float (double-precision)") (Duration :type "Float (double-precision)"))
  (`KismetSystemLibrary.Delay` Duration)
  (set `self.Strength` (* (`self.Strength`) Amount)))

(event `OnFire`
  (params (Length :type Integer) (`Damage Info Greater Lifesteal` :type Boolean) (`Damage Info Attacker` :type "Actor Object Reference"))
  (bind _returnvalue (`self.GetOwner`))
  (bind _fire (`self.Fire`))
  (bind _fire_2 (`self.Fire`))
  (bind _fire_3 (`self.Fire`))
  (bind _rootcomponent (`Actor.RootComponent` _returnvalue))
  (if (`self.ImmuneToFire`)
    _
    (elif (`self.Environment`)
      (if (not (`self.IsDead`))
        (set `self.FireTick` (`KismetMathLibrary.FCeil` (* (`self.MaxHealth`) 2.0)))
        (if (not (`self.IsOnFireBool`))
          (`SceneComponent.SetWorldScale3D` _rootcomponent (/ (`SceneComponent.K2_GetComponentScale` _rootcomponent) 0.999999))
          (set `self.IsOnFireBool` true)
          (`/Engine/EditorBlueprintResources/StandardMacros.IsValid` _fire_2
            (:`Is Valid`
              (`self.Deactivate` _fire_2)
              (`self.K2_DestroyComponent` _fire_2))
            (:`Is Not Valid`
              _))
          (bind _returnvalue_2 (`NiagaraFunctionLibrary.SpawnSystemAttached` "/Game/M5VFXVOL2/Niagara/Fire/NFire_12.NFire_12" _rootcomponent "None" (0.0 0.0 -5.0) (struct) "KeepRelativeOffset"))
          (set `self.Fire` _returnvalue_2)
          (`KismetSystemLibrary.Delay` 0.1 :!label _label)
          (if (or (== (`self.FireTick`) 0) (`self.ImmuneToFire`))
            (`self.Deactivate` _fire)
            (`self.K2_DestroyComponent` _fire)
            (set `self.IsOnFireBool` false)
            (`SceneComponent.SetWorldScale3D` _rootcomponent (* (`SceneComponent.K2_GetComponentScale` _rootcomponent) 0.999999))
            (else
              (set `self.FireTick` (- (`self.FireTick`) 1))
              (`self.TakeDamage` (make `/Game/Characters/DamageSystem/S_DamageInfo` 0.5 "NewEnumerator2" "NewEnumerator1" false false false true 0 `Damage Info Greater Lifesteal` `Damage Info Attacker`))
              (goto _label)))))
      (else
        (set `self.FireTick` (+ (`KismetMathLibrary.FCeil` (* (`KismetMathLibrary.Conv_IntToDouble` Length) 1.25)) (`self.FireTick`)))
        (if (not (`self.IsOnFireBool`))
          (`SceneComponent.SetWorldScale3D` _rootcomponent (/ (`SceneComponent.K2_GetComponentScale` _rootcomponent) 0.999999))
          (set `self.IsOnFireBool` true)
          (`/Engine/EditorBlueprintResources/StandardMacros.IsValid` _fire_3
            (:`Is Valid`
              (`self.Deactivate` _fire_3)
              (`self.K2_DestroyComponent` _fire_3))
            (:`Is Not Valid`
              _))
          (cast `/Game/Characters/Enemies/BP_EnemyGunhead_Base` _returnvalue
            (:`then`
              (bind _returnvalue_3 (`NiagaraFunctionLibrary.SpawnSystemAttached` "/Game/M5VFXVOL2/Niagara/Reference/Fireloop/3_Nblowingfire_fwd_pt.3_Nblowingfire_fwd_pt" _rootcomponent "None" (50.0 0.0 -100.0) (struct) "KeepRelativeOffset"))
              (set `self.Fire` _returnvalue_3)
              (goto _label))
            (:`CastFailed`
              (cast `/Game/Characters/Player/BP_Player` _returnvalue)
              (bind _returnvalue_4 (`NiagaraFunctionLibrary.SpawnSystemAttached` "/Game/M5VFXVOL2/Niagara/Fire/NFire_00.NFire_00" _rootcomponent "None" (50.0 0.0 -100.0) (struct) "KeepRelativeOffset"))
              (set `self.Fire` _returnvalue_4)
              (goto _label))))))))

(event `Invinsible`
  (params (Time :type "Float (double-precision)"))
  (set `self.IsInvincible` true)
  (`KismetSystemLibrary.K2_SetTimerDelegate` (delegate `Vulnerable`) (`KismetMathLibrary.FMin` (/ Time 2.0) 0.04)))

(event `Vulnerable`
  (set `self.IsInvincible` false))

(event `PutOutFire`
  (if (`self.IsOnFireBool`)
    (set `self.FireTick` 0)
    (set `self.IsOnFireBool` false)))

(event `GrantPoisonImmunity`
  (bind _poison (`self.Poison`))
  (set `self.ImmuneToPoison` true)
  (`/Engine/EditorBlueprintResources/StandardMacros.IsValid` _poison
    (:`Is Valid`
      (`self.K2_DestroyComponent` _poison))
    (:`Is Not Valid`
      _))
  (bind _returnvalue (`NiagaraFunctionLibrary.SpawnSystemAttached` "/Game/M5VFXVOL2/Niagara/Reference/Fire/8_Nflame_pt.8_Nflame_pt" (`Actor.RootComponent` (`self.GetOwner`)) "None" (0.0 0.0 -5.0) (struct) "KeepRelativeOffset"))
  (set `self.PoisonImmune` _returnvalue))

(event `Poisoned`
  (params (Strength :type Integer) (`Damage Info Greater Lifesteal` :type Boolean) (`Damage Info Attacker` :type "Actor Object Reference"))
  (bind _returnvalue (/ Strength 6))
  (if (`self.ImmuneToPoison`)
    _
    (elif (< (`self.PoisonTick`) 9)
      (set `self.PoisonTick` 9)
      (if (`self.IsPoisonedBool`)
        (set `self.PoisonDamage` (+ (`self.PoisonDamage`) _returnvalue) :!label _label_2)
        (else
          (set `self.IsPoisonedBool` true)
          (set `self.PoisonDamage` _returnvalue)
          (`KismetSystemLibrary.Delay` 0.5 :!label _label_3)
          (if (or (== (`self.PoisonTick`) 0) (`self.ImmuneToPoison`))
            (set `self.IsPoisonedBool` false)
            (else
              (set `self.PoisonTick` (- (`self.PoisonTick`) 1))
              (`self.TakeDamage` (make `/Game/Characters/DamageSystem/S_DamageInfo` (`KismetMathLibrary.Conv_IntToDouble` (`self.PoisonDamage`)) "NewEnumerator2" "NewEnumerator1" false false false true 0 `Damage Info Greater Lifesteal` `Damage Info Attacker`))
              (goto _label_3)))))
      (else
        (goto _label_2)))))

(event `LethalPoison`
  (set `self.PoisonTick` 2147483647))

(fn `Heal`
  (params (Amount :type "Float (double-precision)"))
  (returns (NewHealth :type "Float (double-precision)"))
  (if (`self.IsDead`)
    (return 0.0)
    (else
      (bind _output_get (set `self.Health` (`KismetMathLibrary.FClamp` (+ Amount (`self.Health`)) 0.0 (`self.MaxHealth`))))
      (return _output_get))))

(fn `Invulnerability`
  (params (Time :type "Float (double-precision)"))
  (`self.Invinsible` Time))

(fn `IsOnFire`
  (returns (OnFire :type Boolean))
  (return (`self.IsOnFireBool`)))

(fn `TakeDamage`
  (params (DamageInfo :type "/Game/Characters/DamageSystem/S_DamageInfo Structure"))
  (returns (WasDamaged :type Boolean))
  (bind (_amount _damagetype _damageresponse _shoulddamageinvinsible _canbeblocked _canbeparried _shouldforceinterupt _lifesteal _greaterlifesteal _attacker) (break `/Game/Characters/DamageSystem/S_DamageInfo` DamageInfo))
  (bind _returnvalue (`self.GetOwner`))
  (bind _returnvalue_2 (`KismetMathLibrary.FCeil` _amount))
  (bind _returnvalue_3 (/ _amount 5.0))
  (switch `/Game/Characters/DamageSystem/E_DamageType` _damagetype
    (:`NewEnumerator1`
      (if (not (`self.ImmuneToPoison`))
        (`self.CanBeDamaged` _shoulddamageinvinsible _canbeblocked :!label _label
          (:`BlockDamage`
            (`self.OnBlocked` _canbeparried)
            (return false))
          (:`TakeDamage`
            (if _greaterlifesteal
              (if (!= _returnvalue _attacker)
                (cast `/Game/Characters/Enemies/BP_Enemy_Base` _returnvalue
                  (:`then`
                    (bind _asbp_player (cast `/Game/Characters/Player/BP_Player` _attacker :!label _label_2)
                      (:`then`
                        (`self.Heal` (`/Game/Characters/Player/BP_Player.BPC_DamageSystem` _asbp_player) _returnvalue_3))
                      (:`CastFailed`
                        (bind _asbp_enemy_base (cast `/Game/Characters/Enemies/BP_Enemy_Base` _attacker)
                          (:`then`
                            (`self.Heal` (`/Game/Characters/Enemies/BP_Enemy_Base.BPC_DamageSystem` _asbp_enemy_base) _returnvalue_3))
                          (:`CastFailed`
                            _)))))
                  (:`CastFailed`
                    (cast `/Game/Characters/Player/BP_Player` _returnvalue
                      (:`then`
                        (goto _label_2))
                      (:`CastFailed`
                        _))))))
            (if (not (`self.IsDead`))
              (bind _output_get (set `self.Health` (- (`self.Health`) _amount)))
              (if (<= _output_get 0.0)
                (set `self.IsDead` true)
                (`self.OnDeath`)
                (bind _asbp_player_2 (cast `/Game/Characters/Player/BP_Player` (`GameplayStatics.GetPlayerPawn` 0))
                  (:`then`
                    _)
                  (:`CastFailed`
                    _))
                (cast `/Game/Characters/Enemies/BP_Enemy_Base` (`self.GetOwner`)
                  (:`then`
                    (`/Game/Characters/Player/BP_Player.AddKill` _asbp_player_2)
                    (`self.Heal` (`/Game/Characters/Player/BP_Player.BPC_DamageSystem` _asbp_player_2) (`KismetMathLibrary.Conv_IntToDouble` _lifesteal)))
                  (:`CastFailed`
                    _))
                (switch `/Game/Characters/DamageSystem/E_DamageType` _damagetype :!label _label_3
                  (:`NewEnumerator0`
                    (return false))
                  (:`NewEnumerator1`
                    (`self.Poisoned` _returnvalue_2 _greaterlifesteal _attacker))
                  (:`NewEnumerator2`
                    _)
                  (:`NewEnumerator3`
                    (`self.OnFire` _returnvalue_2 _greaterlifesteal _attacker))
                  (:`NewEnumerator4`
                    _))
                (return true)
                (elif (or (`self.IsInterruptable`) _shouldforceinterupt)
                  (`self.OnDamageResponse` _damageresponse)
                  (goto _label_3)))))
          (:`NoDamage`
            (return false)))))
    (:`NewEnumerator2`
      (goto _label))
    (:`NewEnumerator3`
      (if (not (`self.ImmuneToFire`))
        (goto _label)))
    (:`NewEnumerator4`
      (goto _label))))

(fn `Weaken`
  (params (Amount :type "Float (double-precision)") (Duration :type "Float (double-precision)"))
  (set `self.Strength` (/ (`self.Strength`) Amount))
  (`self.Unweaken` Amount Duration))