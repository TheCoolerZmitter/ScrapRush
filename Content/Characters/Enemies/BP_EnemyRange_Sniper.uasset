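; Sniper variant of a ranged enemy that fires explosive hitscan shots at its AI controller's attack target.
; On the attack montage notify, a line trace finds the impact point, where an explosion effect, sound, AI noise and radial sphere trace damage each pawn once.
; The sniper also damages itself if the blast lands close to it.
; It also defines its movement speeds and long attack and defend ranges.
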(event `/Game/Characters/Enemies/AI/BPI_EnemyAI.Attack`
  (bind _s_damageinfo (make `/Game/Characters/DamageSystem/S_DamageInfo` 20.0 "NewEnumerator3" "NewEnumerator4" false false false true))
  (bind _hitlocation (`self.HitLocation`))
  (bind _damagearrayindex (`self.DamageArrayIndex`))
  (bind _hitlocation_2 (`self.HitLocation`))
  (bind _notifyname (`|PlayMontage` (`self.Mesh`) "/Game/Characters/Mannequins/Animations/Manny/AttackRangedMontage.AttackRangedMontage")
    (:`OnCompleted`
      (`self.OnAttackEnd` :!label _label))
    (:`OnInterrupted`
      (goto _label))
    (:`OnNotifyBegin`
      (switch `name` _notifyname
        (:`Fire`
          (bind _attack_target (`/Game/Characters/Enemies/AI/AIC_Enemy_Base.Attack Target` (cast `/Game/Characters/Enemies/AI/AIC_Enemy_Base` (`AIBlueprintHelperLibrary.GetAIController` self) :!pure true))
            (:`then`
              (bind _returnvalue (`self.K2_GetActorLocation` _attack_target))
              (bind (_outhit _returnvalue_2) (`KismetSystemLibrary.LineTraceSingle` (+ (`self.K2_GetActorLocation`) (0.0 0.0 60.0)) (+ _returnvalue (0.0 0.0 60.0)) "TraceTypeQuery1"))
              (if _returnvalue_2
                (set `self.HitLocation` (`.Location` (`GameplayStatics.BreakHitResult` _outhit)))
                (else
                  (set `self.HitLocation` _returnvalue)))
              (`GameplayStatics.SpawnEmitterAtLocation` "/Game/M5VFXVOL2/Particles/Explosion/Fire_Exp_00.Fire_Exp_00" _hitlocation (struct) (1.0 1.0 1.0) true "AutoRelease")
              (`GameplayStatics.PlaySoundAtLocation` "/Game/StarterContent/Audio/Explosion_Cue.Explosion_Cue" _hitlocation (struct) 1.0 1.0 0.0 null null null null)
              (bind _outhits (`KismetSystemLibrary.SphereTraceMultiForObjects` _hitlocation _hitlocation 300.0 (`|MakeArray` "ObjectTypeQuery3" :!type "EObjectTypeQuery Enum")))
              (for _array_element _outhits
                (bind (_bblockinghit _binitialoverlap _time _distance _location _impactpoint _normal _impactnormal _physmat _hitactor) (`GameplayStatics.BreakHitResult` _array_element))
                (if (not (`KismetArrayLibrary.Array_Contains` (`self.DamageArray`) _hitactor))
                  (message `/Game/Characters/DamageSystem/BPI_Damagable.TakeDamage` _hitactor _s_damageinfo)
                  (`AISense_Damage.ReportDamageEvent` _hitactor self 20.0 (`self.K2_GetActorLocation`))
                  (`KismetArrayLibrary.Array_Insert` (`self.DamageArray`) _hitactor _damagearrayindex)
                  (set `self.DamageArrayIndex` (+ _damagearrayindex 1))))
              (`KismetArrayLibrary.Array_Clear` (`self.DamageArray`))
              (set `self.DamageArrayIndex` 0)
              (`self.MakeNoise` 1.0 null _hitlocation_2)
              (if (<= (`KismetMathLibrary.Vector_Distance` _hitlocation_2 (`self.K2_GetActorLocation`)) 300.0)
                (message `/Game/Characters/DamageSystem/BPI_Damagable.TakeDamage` self _s_damageinfo)))
            (:`else`)))))))

(fn `GetIdealRange`
  (returns (AttackRadius :type "Float (double-precision)") (DefendRadius :type "Float (double-precision)"))
  (return 1500.0 2000.0))

(fn `SetMovementSpeed`
  (params (Speed :type "/Game/Characters/Enemies/AI/Enums/E_MovementSpeed Enum" :default "NewEnumerator0"))
  (returns (`Speed Value` :type "Float (double-precision)"))
  (set `CharacterMovementComponent.MaxWalkSpeed` (select `/Game/Characters/Enemies/AI/Enums/E_MovementSpeed` Speed :`NewEnumerator1` 200.0 :`NewEnumerator2` 300.0 :`NewEnumerator3` 600.0 :!type "Float (single-precision)") (`self.CharacterMovement`))
  (return 0.0))

(fn `UserConstructionScript`
  (`parent.UserConstructionScript`))