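; Base enemy character that carries a health bar widget and works with an AIC_Enemy_Base controller, exposing patrol route, combat ranges and movement speeds.
; Health, damage, healing and status calls forward to BPCDamageSystem, whose death event triggers ragdoll, stops AI logic and destroys the actor after a delay.
; Freeze temporarily scales walk speed through a stun multiplier.
; Colliding with a burning damageable actor deals damage, reduced if already burning.
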(event `self.ReceiveBeginPlay`
  (bind _bpc_damagesystem (`self.BPC_DamageSystem`))
  (bind _returnvalue (`|CreateWidget` "/Game/Characters/DamageSystem/W_HealthBar.W_HealthBar_C" null self))
  (`WidgetComponent.SetWidget` (`self.HealthBar`) _returnvalue)
  (add `/Game/Characters/DamageSystem/BPC_DamageSystem.OnDeath` _bpc_damagesystem (`|CreateDelegate` :!event `Death`))
  (add `/Game/Characters/DamageSystem/BPC_DamageSystem.OnDamageResponse` _bpc_damagesystem (`|CreateDelegate` :!event `HitResponse`))
  (`KismetSystemLibrary.DelayUntilNextTick`)
  (bind _asaic_enemy_base (cast `/Game/Characters/Enemies/AI/AIC_Enemy_Base` (`AIBlueprintHelperLibrary.GetAIController` self)))
  (bind _output_get (set `self.AIC Enemy Base` _asaic_enemy_base))
  (set `/Game/Characters/Enemies/AI/AIC_Enemy_Base.SelfActor` self _output_get))

(event `Death`
  (bind _mesh (`self.Mesh`))
  (bind _aic_enemy_base (`self.AIC Enemy Base`))
  (`PrimitiveComponent.SetSimulatePhysics` _mesh true)
  (`PrimitiveComponent.SetCollisionEnabled` _mesh "QueryAndPhysics")
  (`PrimitiveComponent.SetCollisionEnabled` (`self.CapsuleComponent`) "NoCollision")
  (`BrainComponent.StopLogic` (`AIController.BrainComponent` _aic_enemy_base) "")
  (`/Game/Characters/Enemies/AI/AIC_Enemy_Base.SetStateAsDead` _aic_enemy_base)
  (`ActorComponent.K2_DestroyComponent` (`self.HealthBar`))
  (`KismetSystemLibrary.Delay` 5.0)
  (`self.K2_DestroyActor`))

(event `HitResponse`
  (params (DamageResponse :type "/Game/Characters/DamageSystem/E_DamageResponse Enum" :default "NewEnumerator0")))

(event `Freeze`
  (params (Duration :type "Float (double-precision)") (Strength :type "Float (double-precision)"))
  (set `self.StunAmount` (/ 5.0 Strength))
  (`/Game/Characters/Enemies/AI/BPI_EnemyAI.SetMovementSpeed` "NewEnumerator3")
  (`KismetSystemLibrary.K2_SetTimerDelegate` (delegate `Unfreeze`) Duration))

(event `Unfreeze`
  (set `self.StunAmount` 1.0)
  (`/Game/Characters/Enemies/AI/BPI_EnemyAI.SetMovementSpeed` "NewEnumerator3"))

(event `self.CapsuleComponent.OnComponentHit`
  (params (HitComponent :type "PrimitiveComponent Object Reference") (OtherActor :type "Actor Object Reference") (OtherComp :type "PrimitiveComponent Object Reference") (NormalImpulse :type "Vector Structure") (Hit :type "HitResult Structure (by ref)"))
  (bind _asbpi_damagable (cast `/Game/Characters/DamageSystem/BPI_Damagable` OtherActor))
  (bind _onfire (`/Game/Characters/DamageSystem/BPI_Damagable.GetOnFire` _asbpi_damagable))
  (if _onfire
    (bind _onfire_2 (`self.GetOnFire`))
    (if _onfire_2
      (`/Game/Characters/DamageSystem/BPC_DamageSystem.TakeDamage` (`self.BPC_DamageSystem`) (make `/Game/Characters/DamageSystem/S_DamageInfo` 2.5 "NewEnumerator3" "NewEnumerator2" false false false true 0 false null))
      (else
        (`/Game/Characters/DamageSystem/BPC_DamageSystem.TakeDamage` (`self.BPC_DamageSystem`) (make `/Game/Characters/DamageSystem/S_DamageInfo` 18.0 "NewEnumerator3" "NewEnumerator2" false false false true 0 false null))))))

(event `/Game/Characters/DamageSystem/BPI_Damagable.PutOutFire`
  (`/Game/Characters/DamageSystem/BPC_DamageSystem.PutOutFire` (`self.BPC_DamageSystem`)))

(event `/Game/Characters/DamageSystem/BPI_Damagable.LethalPoison`
  (`/Game/Characters/DamageSystem/BPC_DamageSystem.LethalPoison` (`self.BPC_DamageSystem`)))

(event `/Game/Characters/DamageSystem/BPI_Damagable.Weaken`
  (params (Amount :type "Float (double-precision)") (Duration :type "Float (double-precision)"))
  (`/Game/Characters/DamageSystem/BPC_DamageSystem.Weaken` (`self.BPC_DamageSystem`) Amount Duration))

(fn `GetCurrentHealth`
  (returns (Health :type "Float (double-precision)"))
  (return (`/Game/Characters/DamageSystem/BPC_DamageSystem.Health` (`self.BPC_DamageSystem`))))

(fn `GetIdealRange`
  (returns (AttackRadius :type "Float (double-precision)") (DefendRadius :type "Float (double-precision)"))
  (return 150.0 350.0))

(fn `GetMaxHealth`
  (returns (MaxHealth :type "Float (double-precision)"))
  (return (`/Game/Characters/DamageSystem/BPC_DamageSystem.MaxHealth` (`self.BPC_DamageSystem`))))

(fn `GetOnFire`
  (returns (OnFire :type Boolean))
  (bind _onfire (`/Game/Characters/DamageSystem/BPC_DamageSystem.IsOnFire` (`self.BPC_DamageSystem`)))
  (return _onfire))

(fn `GetPatrolRoute`
  (returns (PatrolRoute :type "/Game/Characters/Enemies/AI/BP_PatrolRoute Object Reference"))
  (return (`self.PatrolRoute`)))

(fn `Heal`
  (params (Amount :type "Float (double-precision)"))
  (returns (NewHealth :type "Float (double-precision)"))
  (bind _newhealth (`/Game/Characters/DamageSystem/BPC_DamageSystem.Heal` (`self.BPC_DamageSystem`) Amount))
  (return _newhealth))

(fn `IsDead`
  (returns (IsDead :type Boolean))
  (return (`/Game/Characters/DamageSystem/BPC_DamageSystem.IsDead` (`self.BPC_DamageSystem`))))

(fn `SetMovementSpeed`
  (params (Speed :type "/Game/Characters/Enemies/AI/Enums/E_MovementSpeed Enum" :default "NewEnumerator0"))
  (returns (`Speed Value` :type "Float (double-precision)"))
  (bind _output_get (set `CharacterMovementComponent.MaxWalkSpeed` (* (select `/Game/Characters/Enemies/AI/Enums/E_MovementSpeed` Speed :`NewEnumerator1` 200.0 :`NewEnumerator2` 400.0 :`NewEnumerator3` 700.0 :!type "Float (single-precision)") (`self.StunAmount`)) (`self.CharacterMovement`)))
  (return _output_get))

(fn `TakeDamage`
  (params (DamageInfo :type "/Game/Characters/DamageSystem/S_DamageInfo Structure"))
  (returns (WasDamaged :type Boolean))
  (bind _wasdamaged (`/Game/Characters/DamageSystem/BPC_DamageSystem.TakeDamage` (`self.BPC_DamageSystem`) DamageInfo))
  (return _wasdamaged))

(fn `UserConstructionScript`)