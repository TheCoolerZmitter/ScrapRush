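; Melee enemy child Blueprint that overrides the attack with a montage-driven forward area strike.
; Attack plays the melee montage, making the damage system uninterruptable until it completes or is interrupted, then signals attack end.
; On montage notify, a debug-drawn sphere trace finds pawns ahead and damages each once, using a temporary array to skip duplicates.
; Hits force interruption and report AI damage events, whose amount differs from the damage dealt.
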(event `/Game/Characters/Enemies/AI/BPI_EnemyAI.Attack`
  (bind _returnvalue (`self.K2_GetActorLocation`))
  (bind _damagearrayindex (`self.DamageArrayIndex`))
  (bind _bpc_damagesystem (`self.BPC_DamageSystem`))
  (bind _notifyname (`|PlayMontage` (`self.Mesh`) "/Game/Characters/Mannequins/Animations/Manny/AttackMeleeMontage.AttackMeleeMontage")
    (:`then`
      (set `/Game/Characters/DamageSystem/BPC_DamageSystem.IsInterruptable` false _bpc_damagesystem))
    (:`OnCompleted`
      (`self.OnAttackEnd` :!label _label)
      (set `/Game/Characters/DamageSystem/BPC_DamageSystem.IsInterruptable` true _bpc_damagesystem))
    (:`OnInterrupted`
      (goto _label))
    (:`OnNotifyBegin`
      (switch `name` _notifyname
        (:`Boom`
          (bind _outhits (`KismetSystemLibrary.SphereTraceMultiForObjects` :`Start` _returnvalue :`End` (+ _returnvalue (* (`self.GetActorForwardVector`) 300.0)) :`Radius` 300.0 :`ObjectTypes` (`|MakeArray` "ObjectTypeQuery3" :!type "EObjectTypeQuery Enum") :`DrawDebugType` "ForDuration"))
          (for _array_element _outhits
            (bind (_bblockinghit _binitialoverlap _time _distance _location _impactpoint _normal _impactnormal _physmat _hitactor) (`GameplayStatics.BreakHitResult` _array_element))
            (if (not (`KismetArrayLibrary.Array_Contains` (`self.DamageArray`) _hitactor))
              (message `/Game/Characters/DamageSystem/BPI_Damagable.TakeDamage` _hitactor (make `/Game/Characters/DamageSystem/S_DamageInfo` 15.0 "NewEnumerator1" "NewEnumerator1" false false false true))
              (`AISense_Damage.ReportDamageEvent` _hitactor self 20.0 (`self.K2_GetActorLocation`))
              (`KismetArrayLibrary.Array_Insert` (`self.DamageArray`) _hitactor _damagearrayindex)
              (set `self.DamageArrayIndex` (+ _damagearrayindex 1))))
          (`KismetArrayLibrary.Array_Clear` (`self.DamageArray`))
          (set `self.DamageArrayIndex` 0))))))

(fn `UserConstructionScript`
  (`parent.UserConstructionScript`))