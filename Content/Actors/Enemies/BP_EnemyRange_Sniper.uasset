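; Sniper ranged enemy that fires an explosive hitscan attack at its AI controller's attack target.
; Attack plays a montage whose notify runs a Visibility line trace toward the target, then signals attack end on completion or interruption.
; A blocked trace explodes at the impact point without damage, while a clear one explodes on the target and applies interrupting damage.
; It also maps movement states to walk speeds and supplies long attack and defend ranges.
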(event `/Game/Actors/Enemies/AI/BPI_EnemyAI.Attack`
  (bind _notifyname (`|PlayMontage` (`self.Mesh`) "/Game/Characters/Mannequins/Animations/Manny/AttackRangedMontage.AttackRangedMontage")
    (:`OnCompleted`
      (`self.OnAttackEnd` :!label _label))
    (:`OnInterrupted`
      (goto _label))
    (:`OnNotifyBegin`
      (switch `name` _notifyname
        (:`Fire`
          (bind _attack_target (`/Game/Actors/Enemies/AI/AIC_Enemy_Base.Attack Target` (cast `/Game/Actors/Enemies/AI/AIC_Enemy_Base` (`AIBlueprintHelperLibrary.GetAIController` self) :!pure true))
            (:`then`
              (bind _returnvalue (+ (`self.K2_GetActorLocation` _attack_target) (0.0 0.0 60.0)))
              (bind (_outhit _returnvalue_2) (`KismetSystemLibrary.LineTraceSingle` :`Start` (+ (`self.K2_GetActorLocation`) (0.0 0.0 60.0)) :`End` _returnvalue :`TraceChannel` "TraceTypeQuery1" :`DrawDebugType` "ForDuration"))
              (if _returnvalue_2
                (bind (_bblockinghit _binitialoverlap _time _distance _location) (`GameplayStatics.BreakHitResult` _outhit))
                (`GameplayStatics.SpawnEmitterAtLocation` "/Game/M5VFXVOL2/Particles/Explosion/Fire_Exp_00.Fire_Exp_00" _location)
                (`GameplayStatics.PlaySoundAtLocation` "/Game/StarterContent/Audio/Explosion_Cue.Explosion_Cue" _location (struct) 1.0 1.0 0.0 null null null null)
                (else
                  (`GameplayStatics.SpawnEmitterAtLocation` "/Game/M5VFXVOL2/Particles/Explosion/Fire_Exp_00.Fire_Exp_00" _returnvalue)
                  (`GameplayStatics.PlaySoundAtLocation` "/Game/StarterContent/Audio/Explosion_Cue.Explosion_Cue" _returnvalue (struct) 1.0 1.0 0.0 null null null null)
                  (message `/Game/Actors/DamageSystem/BPI_Damagable.TakeDamage` _attack_target (make `/Game/Actors/DamageSystem/S_DamageInfo` 20.0 "NewEnumerator3" "NewEnumerator4" false false false true)))))
            (:`else`)))))))

(fn `GetIdealRange`
  (returns (AttackRadius :type "Float (double-precision)") (DefendRadius :type "Float (double-precision)"))
  (return 1500.0 2000.0))

(fn `SetMovementSpeed`
  (params (Speed :type "/Game/Actors/Enemies/AI/Enums/E_MovementSpeed Enum" :default "NewEnumerator0"))
  (returns (`Speed Value` :type "Float (double-precision)"))
  (set `CharacterMovementComponent.MaxWalkSpeed` (select `/Game/Actors/Enemies/AI/Enums/E_MovementSpeed` Speed :`NewEnumerator1` 200.0 :`NewEnumerator2` 300.0 :`NewEnumerator3` 600.0 :!type "Float (single-precision)") (`self.CharacterMovement`))
  (return 0.0))

(fn `UserConstructionScript`
  (`parent.UserConstructionScript`))