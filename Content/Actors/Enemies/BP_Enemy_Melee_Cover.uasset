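; Melee enemy Blueprint that defines an Attack event for a forward strike.
; Attack plays the melee montage, and a montage notify fires a short forward sphere trace for Pawns with debug drawing on.
; A hit actor receives an interrupt-forcing damage struct through a TakeDamage message.
; Montage completion or interruption both broadcast OnAttackEnd.
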(event `/Game/Actors/Enemies/AI/BPI_EnemyAI.Attack`
  (bind _returnvalue (`self.K2_GetActorLocation`))
  (bind _notifyname (`|PlayMontage` (`self.Mesh`) "/Game/Characters/Mannequins/Animations/Manny/AttackMeleeMontage.AttackMeleeMontage")
    (:`OnCompleted`
      (`self.OnAttackEnd` :!label _label))
    (:`OnInterrupted`
      (goto _label))
    (:`OnNotifyBegin`
      (switch `name` _notifyname
        (:`Boom`
          (bind (_outhit _returnvalue_2) (`KismetSystemLibrary.SphereTraceSingleForObjects` :`Start` _returnvalue :`End` (+ _returnvalue (* (`self.GetActorForwardVector`) 300.0)) :`Radius` 100.0 :`ObjectTypes` (`|MakeArray` "ObjectTypeQuery3" :!type "EObjectTypeQuery Enum") :`DrawDebugType` "ForDuration"))
          (if _returnvalue_2
            (message `/Game/Actors/DamageSystem/BPI_Damagable.TakeDamage` (`.HitActor` (`GameplayStatics.BreakHitResult` _outhit)) (make `/Game/Actors/DamageSystem/S_DamageInfo` 15.0 "NewEnumerator1" "NewEnumerator1" false false false true))))))))

(fn `UserConstructionScript`
  (`parent.UserConstructionScript`))