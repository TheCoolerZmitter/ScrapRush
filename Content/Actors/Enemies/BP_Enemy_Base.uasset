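; Base enemy character that takes damage, reacts to hits and dies, working with its AIC_Enemy_Base AI controller.
; BPCDamageSystem handles health, damage and healing behind wrapper functions, and a widget component shows the health bar.
; Hits stop movement and freeze the AI during a montage before it resumes attacking the last known target; death ragdolls, stops AI logic, then destroys the actor.
; It also exposes patrol route, ideal combat ranges and enum-based movement speeds.
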(event `self.ReceiveBeginPlay`
  (bind _bpc_damagesystem (`self.BPC_DamageSystem`))
  (bind _returnvalue (`|CreateWidget` "/Game/Actors/DamageSystem/W_HealthBar.W_HealthBar_C" null self))
  (`WidgetComponent.SetWidget` (`self.HealthBar`) _returnvalue)
  (add `/Game/Actors/DamageSystem/BPC_DamageSystem.OnDeath` _bpc_damagesystem (`|CreateDelegate` :!event `Death`))
  (add `/Game/Actors/DamageSystem/BPC_DamageSystem.OnDamageResponse` _bpc_damagesystem (`|CreateDelegate` :!event `HitResponse`))
  (bind _asaic_enemy_base (cast `/Game/Actors/Enemies/AI/AIC_Enemy_Base` (`AIBlueprintHelperLibrary.GetAIController` self)))
  (set `self.AIC Enemy Base` _asaic_enemy_base))

(event `Death`
  (bind _mesh (`self.Mesh`))
  (bind _aic_enemy_base (`self.AIC Enemy Base`))
  (`PrimitiveComponent.SetSimulatePhysics` _mesh true)
  (`PrimitiveComponent.SetCollisionEnabled` _mesh "QueryAndPhysics")
  (`BrainComponent.StopLogic` (`AIController.BrainComponent` _aic_enemy_base) "")
  (`/Game/Actors/Enemies/AI/AIC_Enemy_Base.SetStateAsDead` _aic_enemy_base)
  (`KismetSystemLibrary.Delay` 5.0)
  (`self.K2_DestroyActor`))

(event `HitResponse`
  (params (DamageResponse :type "/Game/Actors/DamageSystem/E_DamageResponse Enum" :default "NewEnumerator0"))
  (`MovementComponent.StopMovementImmediately` (`self.CharacterMovement`))
  (`/Game/Actors/Enemies/AI/AIC_Enemy_Base.SetStateAsFrozen` (`self.AIC Enemy Base`))
  (`|PlayMontage` (`self.Mesh`) (`self.HitReactionMontage`)
    (:`OnCompleted`
      _)
    (:`OnInterrupted`
      _))
  (`/Game/Actors/Enemies/AI/AIC_Enemy_Base.SetStateAsAttacking` (`self.AIC Enemy Base`) null true))

(fn `GetCurrentHealth`
  (returns (Health :type "Float (double-precision)"))
  (return (`/Game/Actors/DamageSystem/BPC_DamageSystem.Health` (`self.BPC_DamageSystem`))))

(fn `GetIdealRange`
  (returns (AttackRadius :type "Float (double-precision)") (DefendRadius :type "Float (double-precision)"))
  (return 150.0 350.0))

(fn `GetMaxHealth`
  (returns (MaxHealth :type "Float (double-precision)"))
  (return (`/Game/Actors/DamageSystem/BPC_DamageSystem.MaxHealth` (`self.BPC_DamageSystem`))))

(fn `GetPatrolRoute`
  (returns (PatrolRoute :type "/Game/Actors/Enemies/AI/BP_PatrolRoute Object Reference"))
  (return (`self.PatrolRoute`)))

(fn `Heal`
  (params (Amount :type "Float (double-precision)"))
  (returns (NewHealth :type "Float (double-precision)"))
  (bind _newhealth (`/Game/Actors/DamageSystem/BPC_DamageSystem.Heal` (`self.BPC_DamageSystem`) Amount))
  (return _newhealth))

(fn `IsDead`
  (returns (IsDead :type Boolean))
  (return (`/Game/Actors/DamageSystem/BPC_DamageSystem.IsDead` (`self.BPC_DamageSystem`))))

(fn `SetMovementSpeed`
  (params (Speed :type "/Game/Actors/Enemies/AI/Enums/E_MovementSpeed Enum" :default "NewEnumerator0"))
  (returns (`Speed Value` :type "Float (double-precision)"))
  (bind _output_get (set `CharacterMovementComponent.MaxWalkSpeed` (select `/Game/Actors/Enemies/AI/Enums/E_MovementSpeed` Speed :`NewEnumerator1` 200.0 :`NewEnumerator2` 400.0 :`NewEnumerator3` 700.0 :!type "Float (single-precision)") (`self.CharacterMovement`)))
  (return _output_get))

(fn `TakeDamage`
  (params (DamageInfo :type "/Game/Actors/DamageSystem/S_DamageInfo Structure"))
  (returns (WasDamaged :type Boolean))
  (bind _wasdamaged (`/Game/Actors/DamageSystem/BPC_DamageSystem.TakeDamage` (`self.BPC_DamageSystem`) DamageInfo))
  (return _wasdamaged))

(fn `UserConstructionScript`)