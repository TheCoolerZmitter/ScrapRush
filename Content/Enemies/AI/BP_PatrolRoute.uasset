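; BP_PatrolRoute is a spline-based patrol path, filed with the enemy AI assets.
; It tracks a current point index and exposes that spline point's world position.
; IncrementPatrolRoute steps the index along the spline and flips direction at the last and first points, so the route runs back and forth rather than looping.
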(event `IncrementPatrolRoute`
  (bind _output_get (set `self.PatrolIndex` (+ (`self.PatrolIndex`) (`self.Direction`))))
  (if (== _output_get (- (`SplineComponent.GetNumberOfSplinePoints` (`self.PatrolRoute`)) 1))
    (set `self.Direction` -1)
    (elif (== _output_get 0)
      (set `self.Direction` 1))))

(fn `GetSplinePointAsWorldPosition`
  (returns (Location :type "Vector Structure"))
  (return (`SplineComponent.GetLocationAtSplinePoint` (`self.PatrolRoute`) (`self.PatrolIndex`) "World")))

(fn `UserConstructionScript`)