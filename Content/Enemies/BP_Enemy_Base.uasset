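; Base enemy character Blueprint that provides health, death state, patrol route access and movement speed control.
; Damage and healing clamp health between zero and max; healing accepts a flat amount or fraction of max, and damage sets a dead flag at zero.
; Getter functions expose health, patrol route and fixed attack and defend radii.
; SetMovementSpeed maps a speed state from idle to sprinting onto the character's max walk speed.
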(event `self.ReceiveAnyDamage`
  (params (Damage :type "Float (single-precision)") (DamageType :type "DamageType Object Reference") (InstigatedBy :type "Controller Object Reference") (DamageCauser :type "Actor Object Reference"))
  (bind _output_get (set `self.CurrentHealth` (`KismetMathLibrary.FClamp` (- (`self.CurrentHealth`) Damage) 0.0 (`self.MaxHealth`))))
  (if (<= _output_get 0.0)
    (set `self.IsDead` true)))

(event `/Game/Enemies/AI/BPI_EnemyAI.Heal`
  (params (HealBy :type "Float (double-precision)") (UsePercentage :type Boolean))
  (bind _maxhealth (`self.MaxHealth`))
  (if UsePercentage
    (set `self.CurrentHealth` (`KismetMathLibrary.FClamp` (+ (`self.CurrentHealth`) (* _maxhealth HealBy)) 0.0 _maxhealth))
    (else
      (set `self.CurrentHealth` (`KismetMathLibrary.FClamp` (+ HealBy (`self.CurrentHealth`)) 0.0 (`self.MaxHealth`))))))

(fn `GetCurrentHealth`
  (returns (CurrentHealth :type "Float (double-precision)"))
  (return (`self.CurrentHealth`)))

(fn `GetIdealRange`
  (returns (AttackRadius :type "Float (double-precision)") (DefendRadius :type "Float (double-precision)"))
  (return 150.0 350.0))

(fn `GetMaxHealth`
  (returns (MaxHealth :type "Float (double-precision)"))
  (return (`self.MaxHealth`)))

(fn `GetPatrolRoute`
  (returns (PatrolRoute :type "/Game/Enemies/AI/BP_PatrolRoute Object Reference"))
  (return (`self.PatrolRoute`)))

(fn `SetMovementSpeed`
  (params (Speed :type "/Game/Enemies/AI/Enums/E_MovementSpeed Enum" :default "NewEnumerator0"))
  (returns (`Speed Value` :type "Float (double-precision)"))
  (bind _output_get (set `CharacterMovementComponent.MaxWalkSpeed` (select `/Game/Enemies/AI/Enums/E_MovementSpeed` Speed :`NewEnumerator1` 200.0 :`NewEnumerator2` 400.0 :`NewEnumerator3` 700.0 :!type "Float (single-precision)") (`self.CharacterMovement`)))
  (return _output_get))

(fn `UserConstructionScript`)