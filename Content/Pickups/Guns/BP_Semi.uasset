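; Gun pickup Blueprint that fires a timed burst of projectiles per Shoot call, aimed along the looking component or at a target actor.
; FireBullet spawns a projectile at the barrel, passes it the gun's stats, then loops through QuadFire while KeepFiring holds.
; QuadFire adjusts the aim point for gun movement and rotation between shots.
; CooldownRecovery ends the burst a third into the cooldown, then resets modifiers and re-enables shooting.
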(event `self.PlayAnimation`
  (`SkeletalMeshComponent.PlayAnimation` (`self.SkeletalMesh`) "/Game/Pickups/MilitaryWeapSilver/Weapons/Animations/Fire_GrenadeLauncher_W.Fire_GrenadeLauncher_W" false))

(event `self.CooldownRecovery`
  (params (CooldownTime :type "Float (double-precision)"))
  (bind _returnvalue (/ CooldownTime 3.0))
  (set `self.CanShoot` false)
  (`KismetSystemLibrary.Delay` _returnvalue)
  (set `self.KeepFiring` false)
  (`KismetSystemLibrary.Delay` (* _returnvalue 2.0))
  (`self.ResetAfterModifiers`)
  (set `self.CanShoot` true))

(event `QuadFire`
  (params (BulletBP :type "Actor Class Reference"))
  (bind _returnvalue (`self.K2_GetActorLocation`))
  (bind _returnvalue_2 (`self.K2_GetActorRotation`))
  (if (`self.KeepFiring`)
    (`KismetSystemLibrary.Delay` (/ (`self.Cooldown`) (`self.SubCooldown`)))
    (set `self.HitLocation` (`KismetMathLibrary.GreaterGreater_VectorRotator` (`KismetMathLibrary.GreaterGreater_VectorRotator` (+ (`self.HitLocation`) (- (`self.PositionLastBullet`) _returnvalue)) (`KismetMathLibrary.InverseTransformRotation` (`KismetMathLibrary.MakeTransform` (0.0 0.0 0.0) (`self.RotationLastBullet`)))) _returnvalue_2))
    (set `self.RotationLastBullet` _returnvalue_2)
    (set `self.PositionLastBullet` _returnvalue)
    (`/Game/Pickups/Guns/BPI_Weapons.FireBullet` BulletBP)
    (else
      (`/Game/Pickups/Guns/BPI_Weapons.NextBullet`))))

(fn `FireBullet`
  (params (BulletBP :type "Actor Class Reference"))
  (returns (Fired :type Boolean))
  (bind _statis (`self.Statis`))
  (bind _returnvalue (`SceneComponent.GetSocketLocation` (`self.SkeletalMesh`) "barrel"))
  (bind _returnvalue_2 (`|SpawnActorFromClass` BulletBP (`KismetMathLibrary.MakeTransform` _returnvalue) "Undefined" "MultiplyWithRoot" (`self.GetOwner`) null))
  (bind _asbp_projectile_base (cast `/Game/Pickups/Bullets/BP_ProjectileBase` _returnvalue_2))
  (`/Game/Pickups/Bullets/BP_ProjectileBase.SetStats` _asbp_projectile_base (`KismetMathLibrary.Normal` (- (`self.HitLocation`) _returnvalue) 0.0) (`self.BulletVelocity`) (`self.Lifetime`) (`self.Damage`) (`self.Piercing`) (`self.Gravity`) _statis (`self.Bounce`) (`self.PhaseEnemies`))
  (if _statis
    (`KismetArrayLibrary.Array_Add` (`self.BulletsInStatis`) _asbp_projectile_base))
  (set `self.Cooldown` (* (`self.Cooldown`) (`/Game/Pickups/Bullets/BP_ProjectileBase.CooldownMultiply` _asbp_projectile_base)))
  (`self.QuadFire` BulletBP)
  (return true))

(fn `Shoot`
  (params (LookingActor :type "SceneComponent Object Reference") (Target :type "Actor Object Reference"))
  (returns (Fired :type Boolean))
  (if (`self.CanShoot`)
    (set `self.PositionLastBullet` (`self.K2_GetActorLocation`))
    (set `self.RotationLastBullet` (`self.K2_GetActorRotation`))
    (`/Engine/EditorBlueprintResources/StandardMacros.IsValid` LookingActor
      (:`Is Valid`
        (set `self.HitLocation` (+ (`SceneComponent.K2_GetComponentLocation` LookingActor) (* (`KismetMathLibrary.GetForwardVector` (`SceneComponent.GetSocketRotation` LookingActor "None")) 20000.0))))
      (:`Is Not Valid`
        (set `self.HitLocation` (+ (`self.K2_GetActorLocation` Target) (0.0 0.0 50.0)))))
    (set `self.KeepFiring` true)
    (bind _fired (`/Game/Pickups/Guns/BPI_Weapons.SelectBullet`))
    (if _fired
      (`self.PlayAnimation`)
      (`self.CooldownRecovery` (`self.Cooldown`))
      (return _fired)
      (else
        (`self.CooldownRecovery` 0.5)))
    (else
      (return false))))

(fn `UserConstructionScript`
  (`parent.UserConstructionScript`))