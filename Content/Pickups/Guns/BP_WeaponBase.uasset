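; Base gun that fires a programmable sequence of inventory slots holding bullet types and modifiers.
; Shoot calls SelectBullet, which recursively applies stat, Twin, Chain, Piercing and Stasis modifiers until FireBullet spawns projectiles scaled by the accumulated multipliers.
; Stasis projectiles are tracked until an Un Statis slot releases them.
; CooldownRecovery blocks firing, then restores Cooldown, BulletVelocity, Damage and Lifetime from BeginPlay copies; Piercing is not reset.
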(event `self.ReceiveBeginPlay`
  (`KismetSystemLibrary.DelayUntilNextTick`)
  (set `self.CooldownStore` (`self.Cooldown`))
  (set `self.BulletVelocityStore` (`self.BulletVelocity`))
  (set `self.DamageStore` (`self.Damage`))
  (set `self.LifetimeStore` (`self.Lifetime`)))

(event `CooldownRecovery`
  (params (CooldownTime :type "Float (double-precision)"))
  (set `self.CanShoot` false)
  (`KismetSystemLibrary.Delay` CooldownTime)
  (`self.ResetAfterModifiers`)
  (set `self.CanShoot` true))

(event `Empty`
  (`GameplayStatics.SpawnSoundAttached` "/Game/Pickups/MilitaryWeapSilver/Sound/GrenadeLauncher/Wavs/GrenadeLauncher_Reload02.GrenadeLauncher_Reload02" (`self.SkeletalMesh`) "None" (0.0 0.0 0.0) (struct) "KeepRelativeOffset" false 1.0 1.0 0.0 null null)
  (`self.K2_SetActorRelativeRotation` (struct :`Pitch` 10.0 :`Yaw` -80.0 :`Roll` 10.0))
  (`KismetSystemLibrary.Delay` 0.3)
  (`self.K2_SetActorRelativeRotation` (struct :`Yaw` -90.0)))

(event `/Game/Pickups/Guns/BPI_Weapons.NextBullet`
  (bind _output_get (set `self.CurrentBulletIndex` (+ (`self.CurrentBulletIndex`) 1) :!label _label))
  (if (>= _output_get (`self.NumSlots`))
    (set `self.CurrentBulletIndex` 0)
    (elif (`|EnumEquality` (`|GetArrayItem` (`self.Inventory`) (`self.CurrentBulletIndex`)) (enumliteral `/Game/Pickups/Bullets/E_BulletTypes` "NewEnumerator21"))
      (goto _label))))

(event `ResetAfterModifiers`
  (set `self.Cooldown` (`self.CooldownStore`))
  (set `self.BulletVelocity` (`self.BulletVelocityStore`))
  (set `self.Damage` (`self.DamageStore`))
  (set `self.Lifetime` (`self.LifetimeStore`)))

(fn `CheckNextBulletAfterModifier`
  (returns (`Return Early` :type Boolean))
  (`/Game/Pickups/Guns/BPI_Weapons.NextBullet`)
  (if (== (`self.CurrentBulletIndex`) 0)
    (`self.Empty`)
    (return true)
    (else
      (return false))))

(fn `FireBullet`
  (params (BulletBP :type "Actor Class Reference"))
  (returns (Fired :type Boolean))
  (bind _returnvalue (`SceneComponent.GetSocketLocation` (`self.SkeletalMesh`) "barrel"))
  (bind _returnvalue_2 (`|SpawnActorFromClass` BulletBP (`KismetMathLibrary.MakeTransform` _returnvalue) "Undefined" "MultiplyWithRoot" (`self.GetOwner`) null))
  (bind _asbp_projectile_base (cast `/Game/Pickups/Bullets/BP_ProjectileBase` _returnvalue_2))
  (bind _output_get (set `/Game/Pickups/Bullets/BP_ProjectileBase.Direction` (* (`KismetMathLibrary.Normal` (- (`self.HitLocation`) _returnvalue) 0.0) (* (`/Game/Pickups/Bullets/BP_ProjectileBase.Velocity` _asbp_projectile_base) (`self.BulletVelocity`))) _asbp_projectile_base))
  (bind _output_get_2 (set `MovementComponent.Velocity` _output_get (`/Game/Pickups/Bullets/BP_ProjectileBase.ProjectileMovement` _asbp_projectile_base)))
  (set `/Game/Pickups/Bullets/BP_ProjectileBase.Damage` (* (`/Game/Pickups/Bullets/BP_ProjectileBase.Damage` _asbp_projectile_base) (`self.Damage`)) _asbp_projectile_base)
  (set `/Game/Pickups/Bullets/BP_ProjectileBase.Lifetime` (* (`/Game/Pickups/Bullets/BP_ProjectileBase.Lifetime` _asbp_projectile_base) (`self.Lifetime`)) _asbp_projectile_base)
  (set `/Game/Pickups/Bullets/BP_ProjectileBase.Piercing` (or (`self.Piercing`) (`/Game/Pickups/Bullets/BP_ProjectileBase.Piercing` _asbp_projectile_base)) _asbp_projectile_base)
  (bind _output_get_3 (set `/Game/Pickups/Bullets/BP_ProjectileBase.Statis` (`self.Statis`) _asbp_projectile_base))
  (if _output_get_3
    (`KismetArrayLibrary.Array_Add` (`self.BulletsInStatis`) _asbp_projectile_base))
  (set `self.Cooldown` (* (`self.Cooldown`) (`/Game/Pickups/Bullets/BP_ProjectileBase.CooldownMultiply` _asbp_projectile_base)))
  (if (not (< (`KismetMathLibrary.VSize` _output_get_2) 6000.0))
    (set `/Game/Pickups/Bullets/BP_ProjectileBase.DoPhysicsCalculation` false _asbp_projectile_base))
  (return true))

(fn `SelectBullet`
  (returns (Fired :type Boolean))
  (locals (LastIndex :type Integer))
  (bind _returnvalue (`self.K2_GetActorLocation`))
  (bind _returnvalue_2 (* (`KismetMathLibrary.Normal` (- (`self.HitLocation`) _returnvalue) 0.0) 20000.0))
  (`KismetSystemLibrary.LineTraceSingle` (`SceneComponent.GetSocketLocation` (`self.SkeletalMesh`) "barrel") (`self.HitLocation`) "TraceTypeQuery1")
  (switch `/Game/Pickups/Bullets/E_BulletTypes` (`|GetArrayItem` (`self.Inventory`) (`self.CurrentBulletIndex`))
    (:`NewEnumerator21`
      ;[1 1 1] Current Slot is empty
      (`/Game/Pickups/Guns/BPI_Weapons.NextBullet`)
      (if (== (`self.CurrentBulletIndex`) 0)
        (`self.Empty`)
        (return false)
        (else
          (bind _fired (`/Game/Pickups/Guns/BPI_Weapons.SelectBullet`))
          (return _fired))))
    (:`NewEnumerator0`
      (bind _fired_2 (`/Game/Pickups/Guns/BPI_Weapons.FireBullet` "/Game/Pickups/Bullets/BP_RegularBullet.BP_RegularBullet_C"))
      (return _fired_2))
    (:`NewEnumerator1`
      (bind _fired_3 (`/Game/Pickups/Guns/BPI_Weapons.FireBullet` "/Game/Pickups/Bullets/BP_Explosive.BP_Explosive_C"))
      (return _fired_3))
    (:`NewEnumerator3`
      (bind _fired_4 (`/Game/Pickups/Guns/BPI_Weapons.FireBullet` "/Game/Pickups/Bullets/BP_Sawblade.BP_Sawblade_C"))
      (return _fired_4))
    (:`NewEnumerator4`
      (bind _fired_5 (`/Game/Pickups/Guns/BPI_Weapons.FireBullet` "/Game/Pickups/Bullets/BP_Ice.BP_Ice_C"))
      (return _fired_5))
    (:`NewEnumerator6`
      (bind _fired_6 (`/Game/Pickups/Guns/BPI_Weapons.FireBullet` "/Game/Pickups/Bullets/BP_Electric.BP_Electric_C"))
      (return _fired_6))
    (:`NewEnumerator10`
      (bind _fired_7 (`/Game/Pickups/Guns/BPI_Weapons.FireBullet` "/Game/Pickups/Bullets/BP_Shockwave.BP_Shockwave_C"))
      (return _fired_7))
    (:`NewEnumerator12`
      (bind _fired_8 (`/Game/Pickups/Guns/BPI_Weapons.FireBullet` "/Game/Pickups/Bullets/BP_Teleport.BP_Teleport_C"))
      (return _fired_8))
    (:`NewEnumerator13`
      (bind _fired_9 (`/Game/Pickups/Guns/BPI_Weapons.FireBullet` "/Game/Pickups/Bullets/BP_Rocket.BP_Rocket_C"))
      (return _fired_9))
    (:`NewEnumerator32`
      (bind _fired_10 (`/Game/Pickups/Guns/BPI_Weapons.FireBullet` "/Game/Pickups/Bullets/BP_Force.BP_Force_C"))
      (return _fired_10))
    (:`NewEnumerator26`
      ;[1 1 1] Statis
      (set `self.Statis` true)
      (`/Game/Pickups/Guns/BPI_Weapons.NextBullet`)
      (bind _fired_11 (`/Game/Pickups/Guns/BPI_Weapons.SelectBullet`))
      (return _fired_11))
    (:`NewEnumerator27`
      ;[1 1 1] UnStatis
      (set `self.Statis` false)
      (for _array_element (`self.BulletsInStatis`)
        (`/Game/Pickups/Bullets/BP_ProjectileBase.UnStatis` _array_element))
      (`KismetArrayLibrary.Array_Clear` (`self.BulletsInStatis`))
      (return true))
    (:`NewEnumerator17`
      ;[1 1 1] Cooldown Down
      (bind _return_early (`self.CheckNextBulletAfterModifier`))
      (if _return_early
        (return false)
        (else
          (set `self.Cooldown` (/ (`self.Cooldown`) 1.5))
          (bind _fired_12 (`/Game/Pickups/Guns/BPI_Weapons.SelectBullet`))
          (return _fired_12))))
    (:`NewEnumerator18`
      ;[1 1 1] Speed Up
      (bind _return_early_2 (`self.CheckNextBulletAfterModifier`))
      (if _return_early_2
        (return false)
        (else
          (set `self.BulletVelocity` (* (`self.BulletVelocity`) 2.0))
          (bind _fired_13 (`/Game/Pickups/Guns/BPI_Weapons.SelectBullet`))
          (return _fired_13))))
    (:`NewEnumerator19`
      ;[1 1 1] Speed Down
      (bind _return_early_3 (`self.CheckNextBulletAfterModifier`))
      (if _return_early_3
        (return false)
        (else
          (set `self.BulletVelocity` (/ (`self.BulletVelocity`) 2.0))
          (bind _fired_14 (`/Game/Pickups/Guns/BPI_Weapons.SelectBullet`))
          (return _fired_14))))
    (:`NewEnumerator20`
      ;[1 1 1] Damage Up
      (bind _return_early_4 (`self.CheckNextBulletAfterModifier`))
      (if _return_early_4
        (return false)
        (else
          (set `self.Damage` (* (`self.Damage`) 1.75))
          (bind _fired_15 (`/Game/Pickups/Guns/BPI_Weapons.SelectBullet`))
          (return _fired_15))))
    (:`NewEnumerator30`
      ;[1 1 1] Lifetime Up
      (bind _return_early_5 (`self.CheckNextBulletAfterModifier`))
      (if _return_early_5
        (return false)
        (else
          (set `self.Lifetime` (* (`self.Lifetime`) 2.0))
          (bind _fired_16 (`/Game/Pickups/Guns/BPI_Weapons.SelectBullet`))
          (return _fired_16))))
    (:`NewEnumerator31`
      ;[1 1 1] Lifetime Down
      (bind _return_early_6 (`self.CheckNextBulletAfterModifier`))
      (if _return_early_6
        (return false)
        (else
          (set `self.Lifetime` (/ (`self.Lifetime`) 2.0))
          (bind _fired_17 (`/Game/Pickups/Guns/BPI_Weapons.SelectBullet`))
          (return _fired_17))))
    (:`NewEnumerator22`
      ;[1 1 1] Twin
      (bind _return_early_7 (`self.CheckNextBulletAfterModifier`))
      (if _return_early_7
        (return false)
        (else
          (set `self.HitLocation` (+ _returnvalue (`KismetMathLibrary.RotateAngleAxis` _returnvalue_2 (+ (`KismetMathLibrary.RandomFloat`) 5.5) (+ (/ (`KismetMathLibrary.RandomUnitVector`) 3.0) (0.0 0.0 1.0)))))
          (`/Game/Pickups/Guns/BPI_Weapons.SelectBullet`)
          (set `self.HitLocation` (+ _returnvalue (`KismetMathLibrary.RotateAngleAxis` _returnvalue_2 (+ (* (`KismetMathLibrary.RandomFloat`) 2.0) -11.0) (+ (/ (`KismetMathLibrary.RandomUnitVector`) 3.0) (0.0 0.0 1.0)))))
          (bind _fired_18 (`/Game/Pickups/Guns/BPI_Weapons.SelectBullet`))
          (return _fired_18))))
    (:`NewEnumerator23`
      ;[1 1 1] Chain
      (bind _return_early_8 (`self.CheckNextBulletAfterModifier`))
      (if _return_early_8
        (return false)
        (else
          (bind _fired_19 (`/Game/Pickups/Guns/BPI_Weapons.SelectBullet`))
          (`/Game/Pickups/Guns/BPI_Weapons.NextBullet`)
          (if (== (`self.CurrentBulletIndex`) 0)
            (return _fired_19)
            (else
              (`/Game/Pickups/Guns/BPI_Weapons.SelectBullet`)
              (if (== (`self.CurrentBulletIndex`) 0)
                (set `self.CurrentBulletIndex` -1)
                (return true)
                (else
                  (return true))))))))
    (:`NewEnumerator29`
      ;[1 1 1] Piercing
      (bind _return_early_9 (`self.CheckNextBulletAfterModifier`))
      (if _return_early_9
        (return false)
        (else
          (set `self.Piercing` true)
          (bind _fired_20 (`/Game/Pickups/Guns/BPI_Weapons.SelectBullet`))
          (return _fired_20))))))

(fn `Shoot`
  (params (HitLocation :type "Vector Structure"))
  (returns (Fired :type Boolean))
  (if (`self.CanShoot`)
    (set `self.HitLocation` HitLocation)
    (bind _fired (`/Game/Pickups/Guns/BPI_Weapons.SelectBullet`))
    (`/Game/Pickups/Guns/BPI_Weapons.NextBullet`)
    (`self.CooldownRecovery` (`self.Cooldown`))
    (return _fired)
    (else
      (return false))))

(fn `UserConstructionScript`)