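; Invulnerability pickup Blueprint that triggers invulnerability on its owning actor, then destroys itself.
; Both the CollisionBehavior event and the UnStatis function find BPC_DamageSystem on the owner and call Invulnerability, passing Cooldown.
; The target is the pickup's owner rather than an overlapped actor, and the overlap and tick events are unused.
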(event `self.CollisionBehavior`
  (params (Location :type "Vector Structure") (DamagedActor :type "Actor Object Reference"))
  (`/Game/Characters/DamageSystem/BPC_DamageSystem.Invulnerability` (`self.GetComponentByClass` (`self.GetOwner`) "/Game/Characters/DamageSystem/BPC_DamageSystem.BPC_DamageSystem_C") (`self.Cooldown`))
  (`self.K2_DestroyActor`))

(fn `UnStatis`
  (`/Game/Characters/DamageSystem/BPC_DamageSystem.Invulnerability` (`self.GetComponentByClass` (`self.GetOwner`) "/Game/Characters/DamageSystem/BPC_DamageSystem.BPC_DamageSystem_C") (`self.Cooldown`))
  (`self.K2_DestroyActor`))

(fn `UserConstructionScript`
  (`parent.UserConstructionScript`))