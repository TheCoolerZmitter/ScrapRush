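; Shockwave bullet Blueprint that applies a radial force impulse at a point rather than acting as a lasting projectile.
; Leaving stasis sets the owner and starts KillEventually, which waits one tick and, unless deletion is cancelled, triggers collision behavior at the owner's location, or its own, then destroys the actor.
; Collision behavior moves the RadialForce component there, fires it and destroys the actor unless Piercing is set.
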(event `self.KillEventually`
  (bind _returnvalue (`self.GetOwner`))
  (`KismetSystemLibrary.DelayUntilNextTick`)
  (if (not (`self.CancelDeletion`))
    (`/Engine/EditorBlueprintResources/StandardMacros.IsValid` _returnvalue
      (:`Is Valid`
        (`self.CollisionBehavior` (`self.K2_GetActorLocation` _returnvalue)))
      (:`Is Not Valid`
        (`self.CollisionBehavior` (`self.K2_GetActorLocation`))))
    (`self.K2_DestroyActor`)))

(event `self.CollisionBehavior`
  (params (Location :type "Vector Structure") (DamagedActor :type "Actor Object Reference"))
  (bind _radialforce (`self.RadialForce`))
  (`SceneComponent.K2_SetWorldLocation` _radialforce Location false false)
  (`RadialForceComponent.FireImpulse` _radialforce)
  (if (not (`self.Piercing`))
    (`self.K2_DestroyActor`)))

(fn `UnStatis`
  (`self.SetOwner` null)
  (`self.KillEventually`))

(fn `UserConstructionScript`
  (`parent.UserConstructionScript`))