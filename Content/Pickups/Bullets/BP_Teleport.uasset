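; Teleport projectile that moves its owner to the point of impact and damages hit actors other than the owner.
; The collision event sends damage to BPI_Damagable targets and reports it, then zeroes the owning Character's vertical velocity and teleports it.
; A failed teleport retries slightly higher.
; The projectile then destroys itself if still moving, or immediately if the owner is invalid.
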(event `self.CollisionBehavior`
  (params (Location :type "Vector Structure") (DamagedActor :type "Actor Object Reference"))
  (bind _returnvalue (`self.GetOwner`))
  (bind _returnvalue_2 (`self.GetOwner`))
  (bind _returnvalue_3 (`self.GetOwner`))
  (if (not (== DamagedActor (`self.GetOwner`)))
    (cast `/Game/Characters/DamageSystem/BPI_Damagable` DamagedActor
      (:`then`
        (message `/Game/Characters/DamageSystem/BPI_Damagable.TakeDamage` DamagedActor (make `/Game/Characters/DamageSystem/S_DamageInfo` (`self.Damage`) "NewEnumerator2" "NewEnumerator1" false false false true))
        (`AISense_Damage.ReportDamageEvent` DamagedActor (`self.GetOwner`) (`self.Damage`) Location))
      (:`CastFailed`
        _)))
  (`/Engine/EditorBlueprintResources/StandardMacros.IsValid` _returnvalue_2
    (:`Is Valid`
      (bind _ascharacter (cast `Character` _returnvalue_2))
      (bind _charactermovement (`Character.CharacterMovement` _ascharacter))
      (bind (_velocity_x _velocity_y) (`KismetMathLibrary.BreakVector` (`MovementComponent.Velocity` _charactermovement)))
      (set `MovementComponent.Velocity` (`KismetMathLibrary.MakeVector` _velocity_x _velocity_y) _charactermovement)
      (bind _returnvalue_4 (`self.K2_TeleportTo` _returnvalue_3 Location (`self.K2_GetActorRotation` _returnvalue_3)))
      (if (not _returnvalue_4)
        (`self.K2_TeleportTo` _returnvalue (+ Location (0.0 0.0 200.0)) (`self.K2_GetActorRotation` _returnvalue)))
      (if (not (== (`MovementComponent.Velocity` (`self.ProjectileMovement`)) (0.0 0.0 0.0)))
        (`self.K2_DestroyActor`)))
    (:`Is Not Valid`
      (`self.K2_DestroyActor`))))

(fn `UserConstructionScript`
  (`parent.UserConstructionScript`))