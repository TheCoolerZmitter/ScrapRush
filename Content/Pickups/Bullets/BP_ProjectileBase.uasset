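; Base projectile actor for bullets, which damages actors implementing BPI_Damagable and reports a damage event.
; Hits come from Sphere overlaps when physics calculation is on, or from a single multi-line trace along the velocity for fast shots.
; Options add gravity, bouncing, piercing and a frozen "Statis" state that UnStatis releases along a stored direction.
; Traced BP_Devastation hits absorb or collide with the projectile, and misses expire after a lifetime unless deletion is cancelled.
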(event `self.ReceiveBeginPlay`
  (bind _sphere (`self.Sphere`))
  (bind _output_get (set `self.StartPos` (`self.K2_GetActorLocation`)))
  (`KismetSystemLibrary.DelayUntilNextTick`)
  (`self.K2_TeleportTo` _output_get (`self.K2_GetActorRotation`))
  (set `ProjectileMovementComponent.ProjectileGravityScale` (`self.Gravity`) (`self.ProjectileMovement`))
  (if (`self.Bounce`)
    (set `ProjectileMovementComponent.bShouldBounce` true (`self.ProjectileMovement`))
    (`PrimitiveComponent.SetCollisionResponseToChannel` _sphere "ECC_WorldStatic" "ECR_Block")
    (`PrimitiveComponent.SetCollisionResponseToChannel` _sphere "ECC_PhysicsBody" "ECR_Block"))
  (if (`self.Statis`)
    (`ProjectileMovementComponent.SetVelocityInLocalSpace` (`self.ProjectileMovement`) (0.0 0.0 0.0))
    (elif (`self.DoPhysicsCalculation`)
      (set `PrimitiveComponent.bGenerateOverlapEvents` true (`self.Sphere`))
      (`self.KillEventually`)
      (else
        (`self.DoLineTrace`)))))

(event `DoLineTrace`
  ;[1 1 1] Use line trace if velocity is high
  (`KismetSystemLibrary.DelayUntilNextTick`)
  (bind _outhits (`KismetSystemLibrary.LineTraceMultiForObjects` (`self.StartPos`) (* (+ (`MovementComponent.Velocity` (`self.ProjectileMovement`)) (`self.StartPos`)) (`self.Lifetime`)) (`|MakeArray` "ObjectTypeQuery1" "ObjectTypeQuery2" "ObjectTypeQuery3" "ObjectTypeQuery4" "ObjectTypeQuery6" :!type "EObjectTypeQuery Enum") false (`|MakeArray` (`self.GetOwner`))))
  (if (`self.Piercing`)
    (for _array_element _outhits
      (bind (_bblockinghit _binitialoverlap _time _distance _location _impactpoint _normal _impactnormal _physmat _hitactor) (`GameplayStatics.BreakHitResult` _array_element))
      (bind _asbp_devastation (cast `/Game/Pickups/Bullets/BP_Devastation` _hitactor)
        (:`then`
          (`/Game/Pickups/Bullets/BP_Devastation.AbsorbOrCollide` _asbp_devastation self)
          (break))
        (:`CastFailed`
          (if (not (`KismetArrayLibrary.Array_Contains` (`self.HitArray`) _hitactor))
            (`KismetArrayLibrary.Array_Add` (`self.HitArray`) _hitactor)
            (`self.CollisionBehavior` _impactpoint _hitactor)))))
    (`self.KillEventually`)
    (elif (`KismetArrayLibrary.Array_IsValidIndex` _outhits)
      (bind (_bblockinghit_2 _binitialoverlap_2 _time_2 _distance_2 _location_2 _impactpoint_2 _normal_2 _impactnormal_2 _physmat_2 _hitactor_2) (`GameplayStatics.BreakHitResult` (`|GetArrayItem` _outhits)))
      (bind _asbp_devastation_2 (cast `/Game/Pickups/Bullets/BP_Devastation` _hitactor_2)
        (:`then`
          (`/Game/Pickups/Bullets/BP_Devastation.AbsorbOrCollide` _asbp_devastation_2 self))
        (:`CastFailed`
          (`self.CollisionBehavior` _impactpoint_2 _hitactor_2)))
      (else
        (`self.KillEventually`)))))

(event `self.Sphere.OnComponentBeginOverlap`
  (params (OverlappedComponent :type "PrimitiveComponent Object Reference") (OtherActor :type "Actor Object Reference") (OtherComp :type "PrimitiveComponent Object Reference") (OtherBodyIndex :type Integer) (bFromSweep :type Boolean) (SweepResult :type "HitResult Structure (by ref)"))
  ;[1 1 1] Collision function
  (`KismetSystemLibrary.DelayUntilNextTick`)
  (if (not (`self.Statis`))
    (cast `/Game/Pickups/Bullets/BP_ProjectileBase` OtherActor
      (:`CastFailed`
        (`self.CollisionBehavior` (`self.K2_GetActorLocation`) OtherActor)))))

(event `KillEventually`
  ;[1 1 1] Destroy after certain amount of time
  (`KismetSystemLibrary.Delay` (`self.Lifetime`))
  (if (not (`self.CancelDeletion`))
    (`self.K2_DestroyActor`)))

(event `CollisionBehavior`
  (params (Location :type "Vector Structure") (DamagedActor :type "Actor Object Reference"))
  ;[1 1 1] Unique bullet behavior
  (cast `/Game/Characters/DamageSystem/BPI_Damagable` DamagedActor)
  (message `/Game/Characters/DamageSystem/BPI_Damagable.TakeDamage` DamagedActor (make `/Game/Characters/DamageSystem/S_DamageInfo` (`self.Damage`) "NewEnumerator2" "NewEnumerator1" false false false true))
  (`AISense_Damage.ReportDamageEvent` DamagedActor (`self.GetOwner`) (`self.Damage`))
  (if (not (`self.Piercing`))
    (`self.K2_DestroyActor`)))

(fn `UnStatis`
  (set `MovementComponent.Velocity` (`self.Direction`) (`self.ProjectileMovement`))
  (set `self.Statis` false)
  (if (`self.DoPhysicsCalculation`)
    (set `PrimitiveComponent.bGenerateOverlapEvents` true (`self.Sphere`))
    (`self.KillEventually`)
    (else
      (`self.DoLineTrace`))))

(fn `UserConstructionScript`)