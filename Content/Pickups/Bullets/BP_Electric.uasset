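; Electric bullet that chains damage between nearby damageable pawns when it collides.
; Its collision event damages and reports the hit actor, or seeds the chain with itself, then repeatedly sphere-traces from the last link for a new living target, excluding the player.
; Velocity sets jump radius and Lifetime caps the jumps, with debug line traces drawing each link.
; Non-piercing bullets destroy themselves afterward; explosion sound nodes are left unwired.
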(event `self.CollisionBehavior`
  (params (Location :type "Vector Structure") (DamagedActor :type "Actor Object Reference"))
  (bind _damagedactors (`self.DamagedActors`))
  (cast `/Game/Characters/DamageSystem/BPI_Damagable` DamagedActor
    (:`then`
      (message `/Game/Characters/DamageSystem/BPI_Damagable.TakeDamage` DamagedActor (make `/Game/Characters/DamageSystem/S_DamageInfo` (`self.Damage`) "NewEnumerator4" "NewEnumerator1" false false false true))
      (`AISense_Damage.ReportDamageEvent` DamagedActor (`self.GetOwner`) 20.0 Location)
      (`KismetArrayLibrary.Array_Add` (`self.DamagedActors`) DamagedActor))
    (:`CastFailed`
      (`KismetArrayLibrary.Array_Add` (`self.DamagedActors`) self)))
  (for _index (range (+ (`KismetMathLibrary.FTrunc` (* (+ (`self.Lifetime`) 1.0) 3.0)) 1))
    (bind _returnvalue (`self.K2_GetActorLocation` (`|GetArrayItem` (`self.DamagedActors`) _index)))
    (bind _outhits (`KismetSystemLibrary.SphereTraceMultiForObjects` _returnvalue _returnvalue (* (`self.Velocity`) 4.0) (`|MakeArray` "ObjectTypeQuery3" :!type "EObjectTypeQuery Enum") false (`|MakeArray` (`GameplayStatics.GetPlayerPawn` 0) :!type "Actor Object Reference")))
    (for _array_element _outhits
      (bind (_bblockinghit _binitialoverlap _time _distance _location _impactpoint _normal _impactnormal _physmat _hitactor) (`GameplayStatics.BreakHitResult` _array_element))
      (cast `/Game/Characters/DamageSystem/BPI_Damagable` _hitactor)
      (if (not (`KismetArrayLibrary.Array_Contains` (`self.DamagedActors`) _hitactor))
        (bind _isdead (message `/Game/Characters/DamageSystem/BPI_Damagable.IsDead` _hitactor))
        (if (not _isdead)
          (message `/Game/Characters/DamageSystem/BPI_Damagable.TakeDamage` _hitactor (make `/Game/Characters/DamageSystem/S_DamageInfo` (`self.Damage`) "NewEnumerator4" "NewEnumerator1" false false false true))
          (`AISense_Damage.ReportDamageEvent` _hitactor (`self.GetOwner`) 20.0 Location)
          (bind _returnvalue_2 (`KismetArrayLibrary.Array_Add` (`self.DamagedActors`) _hitactor))
          (`KismetSystemLibrary.LineTraceSingle` :`Start` (`self.K2_GetActorLocation` (`|GetArrayItem` _damagedactors _returnvalue_2)) :`End` (`self.K2_GetActorLocation` (`|GetArrayItem` _damagedactors (- _returnvalue_2 1))) :`TraceChannel` "TraceTypeQuery1" :`DrawDebugType` "ForDuration")
          (break))))
    (if (not (== (- (`KismetArrayLibrary.Array_Length` (`self.DamagedActors`)) 2) _index))
      (break)))
  (if (not (`self.Piercing`))
    (`self.K2_DestroyActor`)))

(fn `UserConstructionScript`
  (`parent.UserConstructionScript`))