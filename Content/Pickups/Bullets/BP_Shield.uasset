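; Shield projectile that, on hitting anything other than another projectile, spawns three ShieldObjects in a ring.
; The ring centers below the hit player or enemy, or below the impact point otherwise, with radius scaled by Lifetime and health set from Damage.
; Overlaps are time-throttled and capped before self-destruction, and impacts destroy it unless Piercing.
; Stasis suppresses impacts; UnStatis restores velocity and resumes overlap or line-trace detection.
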(event `self.Sphere.OnComponentBeginOverlap`
  (params (OverlappedComponent :type "PrimitiveComponent Object Reference") (OtherActor :type "Actor Object Reference") (OtherComp :type "PrimitiveComponent Object Reference") (OtherBodyIndex :type Integer) (bFromSweep :type Boolean) (SweepResult :type "HitResult Structure (by ref)"))
  (bind _returnvalue (`KismetSystemLibrary.GetGameTimeInSeconds`))
  (if (>= (- _returnvalue (`self.CurrentTime`)) 0.045)
    (set `self.CurrentTime` _returnvalue)
    (bind _output_get (set `self.NumCollisions` (+ (`self.NumCollisions`) 1)))
    (if (<= _output_get 25)
      (if (`self.ValuesUpdated`)
        (if (not (`self.Statis`))
          (cast `/Game/Pickups/Bullets/BP_ProjectileBase` OtherActor
            (:`CastFailed`
              (`self.CollisionBehavior` (`self.K2_GetActorLocation`) OtherActor))))
        (else
          (`KismetSystemLibrary.DelayUntilNextTick`)))
      (else
        (`self.K2_DestroyActor`)))))

(event `self.CollisionBehavior`
  (params (Location :type "Vector Structure") (DamagedActor :type "Actor Object Reference"))
  (bind _damage (`self.Damage`))
  (bind _damage_2 (`self.Damage`))
  (bind _damage_3 (`self.Damage`))
  (bind (_returnvalue_roll _returnvalue_pitch _returnvalue_yaw) (`KismetMathLibrary.BreakRotator` (`KismetMathLibrary.MakeRotFromX` (`self.OwnerForward`))))
  (bind (_returnvalue_roll_2 _returnvalue_pitch_2 _returnvalue_yaw_2) (`KismetMathLibrary.BreakRotator` (`KismetMathLibrary.MakeRotFromX` (`self.OwnerForward`))))
  (bind (_returnvalue_roll_3 _returnvalue_pitch_3 _returnvalue_yaw_3) (`KismetMathLibrary.BreakRotator` (`KismetMathLibrary.MakeRotFromX` (`self.OwnerForward`))))
  (cast `/Game/Characters/Player/BP_Player` DamagedActor
    (:`then`
      (bind _output_get (set `self.Actor` DamagedActor :!label _label))
      (set `self.OwnerLocation` (- (`self.K2_GetActorLocation` _output_get) (0.0 0.0 225.0)))
      (set `self.OwnerForward` (`self.GetActorForwardVector` _output_get)))
    (:`CastFailed`
      (cast `/Game/Characters/Enemies/BP_Enemy_Base` DamagedActor
        (:`then`
          (goto _label))
        (:`CastFailed`
          (set `self.OwnerLocation` (- Location (0.0 0.0 130.0)))
          (set `self.OwnerForward` (`KismetMathLibrary.Normal` (* (`self.GetActorForwardVector`) (1.0 1.0 0.0)) 0.0))))))
  (set `self.Distance` (+ (* (`self.Lifetime`) 50.0) 100.0))
  (bind _returnvalue (`|SpawnActorFromClass` "/Game/Pickups/Bullets/ShieldObject.ShieldObject_C" (`KismetMathLibrary.MakeTransform` (+ (`self.OwnerLocation`) (* (`KismetMathLibrary.RotateAngleAxis` (`self.OwnerForward`) -19.0 (0.0 0.0 1.0)) (`self.Distance`))) (`KismetMathLibrary.MakeRotator` 0.0 0.0 (+ _returnvalue_yaw_2 200.0))) "Undefined" "MultiplyWithRoot" null null))
  (`/Engine/EditorBlueprintResources/StandardMacros.IsValid` _returnvalue
    (:`Is Valid`
      (set `/Game/Pickups/Bullets/ShieldObject.MaxHealth` _damage_3 _returnvalue)
      (set `/Game/Pickups/Bullets/ShieldObject.Health` _damage_3 _returnvalue))
    (:`Is Not Valid`
      _))
  (bind _returnvalue_2 (`|SpawnActorFromClass` "/Game/Pickups/Bullets/ShieldObject.ShieldObject_C" (`KismetMathLibrary.MakeTransform` (+ (`self.OwnerLocation`) (* (`KismetMathLibrary.RotateAngleAxis` (`self.OwnerForward`) -139.0 (0.0 0.0 1.0)) (`self.Distance`))) (`KismetMathLibrary.MakeRotator` 0.0 0.0 (+ _returnvalue_yaw_3 80.0))) "Undefined" "MultiplyWithRoot" null null))
  (`/Engine/EditorBlueprintResources/StandardMacros.IsValid` _returnvalue_2
    (:`Is Valid`
      (set `/Game/Pickups/Bullets/ShieldObject.MaxHealth` _damage_2 _returnvalue_2)
      (set `/Game/Pickups/Bullets/ShieldObject.Health` _damage_2 _returnvalue_2))
    (:`Is Not Valid`
      _))
  (bind _returnvalue_3 (`|SpawnActorFromClass` "/Game/Pickups/Bullets/ShieldObject.ShieldObject_C" (`KismetMathLibrary.MakeTransform` (+ (`self.OwnerLocation`) (* (`KismetMathLibrary.RotateAngleAxis` (`self.OwnerForward`) 101.0 (0.0 0.0 1.0)) (`self.Distance`))) (`KismetMathLibrary.MakeRotator` 0.0 0.0 (+ _returnvalue_yaw 320.0))) "Undefined" "MultiplyWithRoot" null null))
  (`/Engine/EditorBlueprintResources/StandardMacros.IsValid` _returnvalue_3
    (:`Is Valid`
      (set `/Game/Pickups/Bullets/ShieldObject.MaxHealth` _damage _returnvalue_3)
      (set `/Game/Pickups/Bullets/ShieldObject.Health` _damage _returnvalue_3))
    (:`Is Not Valid`
      _))
  (if (not (>= (`self.Piercing`) 1))
    (`self.K2_DestroyActor`)))

(fn `CustomStasis`
  (set `self.OwnerForward` (`KismetMathLibrary.Normal` (* (`self.GetActorForwardVector`) (1.0 1.0 0.0)) 0.0)))

(fn `UnStatis`
  (set `MovementComponent.Velocity` (`self.Direction`) (`self.ProjectileMovement`))
  (set `self.Statis` false)
  (if (`self.DoPhysicsCalculation`)
    (set `PrimitiveComponent.bGenerateOverlapEvents` true (`self.Sphere`))
    (`self.KillEventually`)
    (else
      (`self.DoLineTrace`))))

(fn `UserConstructionScript`
  (`parent.UserConstructionScript`))