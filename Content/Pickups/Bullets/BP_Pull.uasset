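; BP_Pull is a bullet variant, built on a parent Blueprint, that fires a radial force impulse where it collides or expires.
; CollisionBehavior moves the RadialForce component to the given location, fires the impulse, and destroys the actor unless it is Piercing.
; KillEventually waits out Lifetime and, unless CancelDeletion is set, runs CollisionBehavior at the actor's location before destroying it.
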(event `self.KillEventually`
  (`KismetSystemLibrary.Delay` (`self.Lifetime`))
  (if (not (`self.CancelDeletion`))
    (`self.CollisionBehavior` (`self.K2_GetActorLocation`))
    (`self.K2_DestroyActor`)))

(event `self.CollisionBehavior`
  (params (Location :type "Vector Structure") (DamagedActor :type "Actor Object Reference"))
  (`SceneComponent.K2_SetWorldLocation` (`self.RadialForce`) Location false false)
  (`RadialForceComponent.FireImpulse` (`self.RadialForce`))
  (if (not (`self.Piercing`))
    (`self.K2_DestroyActor`)))

(fn `UserConstructionScript`
  (`parent.UserConstructionScript`))