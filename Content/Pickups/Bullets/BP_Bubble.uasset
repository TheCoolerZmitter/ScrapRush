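; BP_Bubble is a slowing bubble projectile that can capture another projectile and carry it.
; On overlap it absorbs the first non-piercing BP_ProjectileBase, disabling its collision and attaching it; further or piercing projectiles pop the bubble.
; Damageable actors take damage and pop it unless PhaseEnemies is set, as do other actors unless it has Piercing.
; Popping or lifetime expiry releases the held bullet, restores its collision and destroys the bubble.
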(event `self.ReceiveTick`
  (params (DeltaSeconds :type "Float (single-precision)"))
  (bind _projectilemovement (`self.ProjectileMovement`))
  (set `MovementComponent.Velocity` (* (`MovementComponent.Velocity` _projectilemovement) 0.98) _projectilemovement))

(event `self.Sphere.OnComponentBeginOverlap`
  (params (OverlappedComponent :type "PrimitiveComponent Object Reference") (OtherActor :type "Actor Object Reference") (OtherComp :type "PrimitiveComponent Object Reference") (OtherBodyIndex :type Integer) (bFromSweep :type Boolean) (SweepResult :type "HitResult Structure (by ref)"))
  (`self.AbsorbOrCollide` OtherActor))

(event `AbsorbOrCollide`
  (params (Actor :type "Actor Object Reference"))
  (cast `/Game/Characters/DamageSystem/BPI_Damagable` Actor
    (:`then`
      (if (not (`self.PhaseEnemies`))
        (`self.CollisionBehavior` (`self.K2_GetActorLocation` Actor) Actor :!label _label)))
    (:`CastFailed`
      (bind _asbp_projectile_base (cast `/Game/Pickups/Bullets/BP_ProjectileBase` Actor)
        (:`then`
          (if (== (`/Game/Pickups/Bullets/BP_ProjectileBase.Piercing` _asbp_projectile_base) 0)
            (`/Engine/EditorBlueprintResources/StandardMacros.IsValid` (`self.InnerBullet`)
              (:`Is Valid`
                (goto _label))
              (:`Is Not Valid`
                (`PrimitiveComponent.SetCollisionEnabled` (`/Game/Pickups/Bullets/BP_ProjectileBase.Sphere` _asbp_projectile_base) "NoCollision")
                (set `self.InnerBullet` _asbp_projectile_base)
                (set `/Game/Pickups/Bullets/BP_ProjectileBase.DoPhysicsCalculation` true _asbp_projectile_base)
                (bind _projectilemovement (`/Game/Pickups/Bullets/BP_ProjectileBase.ProjectileMovement` _asbp_projectile_base))
                (`ProjectileMovementComponent.SetVelocityInLocalSpace` _projectilemovement (0.0 0.0 0.0))
                (set `ProjectileMovementComponent.ProjectileGravityScale` 0.0 _projectilemovement)
                (set `/Game/Pickups/Bullets/BP_ProjectileBase.CancelDeletion` true _asbp_projectile_base)
                (`self.K2_AttachToActor` _asbp_projectile_base self "None" "SnapToTarget" "KeepWorld" "SnapToTarget" true)))
            (else
              (goto _label))))
        (:`CastFailed`
          (if (not (>= (`self.Piercing`) 1))
            (goto _label)))))))

(event `self.KillNow`
  (bind _innerbullet (`self.InnerBullet`))
  (`/Engine/EditorBlueprintResources/StandardMacros.IsValid` _innerbullet :!label _label_2
    (:`Is Valid`
      (`self.UnStatis` _innerbullet)
      (`PrimitiveComponent.SetCollisionEnabled` (`/Game/Pickups/Bullets/BP_ProjectileBase.Sphere` _innerbullet) "QueryOnly")
      (`self.CollisionBehavior` _innerbullet (`self.K2_GetActorLocation`) null null)
      (`self.K2_DestroyActor`))
    (:`Is Not Valid`
      (`self.K2_DestroyActor`))))

(event `self.KillEventually`
  (`KismetSystemLibrary.Delay` (`self.Lifetime`))
  (goto _label_2))

(event `self.CollisionBehavior`
  (params (Location :type "Vector Structure") (DamagedActor :type "Actor Object Reference") (HitComponent :type "PrimitiveComponent Object Reference"))
  (bind _innerbullet (`self.InnerBullet`))
  (cast `/Game/Characters/DamageSystem/BPI_Damagable` DamagedActor
    (:`then`
      (message `/Game/Characters/DamageSystem/BPI_Damagable.TakeDamage` DamagedActor (make `/Game/Characters/DamageSystem/S_DamageInfo` (`self.Damage`) "NewEnumerator2" "NewEnumerator1" false false false true))
      (`AISense_Damage.ReportDamageEvent` DamagedActor (`self.GetOwner`) (`self.Damage`) Location))
    (:`CastFailed`
      _))
  (`/Engine/EditorBlueprintResources/StandardMacros.IsValid` _innerbullet
    (:`Is Valid`
      (`self.UnStatis` _innerbullet)
      (`PrimitiveComponent.SetCollisionEnabled` (`/Game/Pickups/Bullets/BP_ProjectileBase.Sphere` _innerbullet) "QueryOnly")
      (`self.CollisionBehavior` (`self.K2_GetActorLocation`))
      (`self.K2_DestroyActor`))
    (:`Is Not Valid`
      (`self.K2_DestroyActor`))))

(fn `UserConstructionScript`
  (`parent.UserConstructionScript`))