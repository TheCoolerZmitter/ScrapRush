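; BP_Health is a bullet Blueprint that heals in an area where it hits, using inherited or member Damage as the heal amount.
; CollisionBehavior spawns an explosion emitter, then sphere-traces for Pawn and WorldDynamic objects around the location.
; Each hit actor implementing BPI_Damagable receives Heal and is recorded in HealArray to avoid repeat healing.
; The bullet then destroys itself unless Piercing is at least one.
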(event `self.CollisionBehavior`
  (params (Location :type "Vector Structure") (DamagedActor :type "Actor Object Reference"))
  (`GameplayStatics.SpawnEmitterAtLocation` "/Game/M5VFXVOL2/Particles/Explosion/Fire_Exp_00.Fire_Exp_00" Location)
  (bind _outhits (`KismetSystemLibrary.SphereTraceMultiForObjects` Location Location 200.0 (`|MakeArray` "ObjectTypeQuery3" "ObjectTypeQuery2" :!type "EObjectTypeQuery Enum")))
  (for _array_element _outhits
    (if (not (`KismetArrayLibrary.Array_Contains` (`self.HealArray`) (`.HitActor` (`GameplayStatics.BreakHitResult` _array_element))))
      (bind _asbpi_damagable (cast `/Game/Characters/DamageSystem/BPI_Damagable` (`.HitActor` (`GameplayStatics.BreakHitResult` _array_element))))
      (`/Game/Characters/DamageSystem/BPI_Damagable.Heal` _asbpi_damagable (`self.Damage`))
      (`KismetArrayLibrary.Array_Insert` (`self.HealArray`) (`.HitActor` (`GameplayStatics.BreakHitResult` _array_element)))))
  (if (not (>= (`self.Piercing`) 1))
    (`self.K2_DestroyActor`)))

(fn `UserConstructionScript`
  (`parent.UserConstructionScript`))