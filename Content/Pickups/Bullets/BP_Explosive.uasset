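; Explosive bullet Blueprint that deals area damage through its collision behavior, which also fires when its lifetime expires unless deletion is cancelled.
; The collision behavior plays explosion effects, makes noise, then sphere-traces for pawns and dynamic objects.
; Each hit actor receives interrupting damage once per blast via a damage message, plus a reported damage event.
; Piercing rounds clear the hit list after exploding, while others destroy themselves.
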(event `self.KillEventually`
  (`KismetSystemLibrary.Delay` (`self.Lifetime`))
  (if (not (`self.CancelDeletion`))
    (`self.CollisionBehavior` (`self.K2_GetActorLocation`))
    (`self.K2_DestroyActor`)))

(event `self.CollisionBehavior`
  (params (Location :type "Vector Structure") (DamagedActor :type "Actor Object Reference"))
  (`GameplayStatics.SpawnEmitterAtLocation` "/Game/M5VFXVOL2/Particles/Explosion/Fire_Exp_00.Fire_Exp_00" Location (struct) (1.0 1.0 1.0) true "AutoRelease")
  (`GameplayStatics.PlaySoundAtLocation` "/Game/StarterContent/Audio/Explosion_Cue.Explosion_Cue" Location (struct) 1.0 1.0 0.0 null null null null)
  (`self.MakeNoise` 1.0 null Location)
  (bind _outhits (`KismetSystemLibrary.SphereTraceMultiForObjects` Location Location 350.0 (`|MakeArray` "ObjectTypeQuery3" "ObjectTypeQuery2" :!type "EObjectTypeQuery Enum")))
  (for _array_element _outhits
    (bind (_bblockinghit _binitialoverlap _time _distance _location _impactpoint _normal _impactnormal _physmat _hitactor) (`GameplayStatics.BreakHitResult` _array_element))
    (if (not (`KismetArrayLibrary.Array_Contains` (`self.DamageArray`) _hitactor))
      (message `/Game/Characters/DamageSystem/BPI_Damagable.TakeDamage` _hitactor (make `/Game/Characters/DamageSystem/S_DamageInfo` (`self.Damage`) "NewEnumerator3" "NewEnumerator4" false false false true))
      (`AISense_Damage.ReportDamageEvent` _hitactor (`self.GetOwner`) 20.0 Location)
      (`KismetArrayLibrary.Array_Insert` (`self.DamageArray`) _hitactor)))
  (if (>= (`self.Piercing`) 1)
    (`KismetArrayLibrary.Array_Clear` (`self.DamageArray`))
    (else
      (`self.K2_DestroyActor`))))

(fn `UserConstructionScript`
  (`parent.UserConstructionScript`))