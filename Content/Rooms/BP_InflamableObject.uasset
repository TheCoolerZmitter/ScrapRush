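; BP_InflamableObject is a flammable room object that can receive damage and report whether it is on fire.
; It exposes damage-interface style functions, forwarding TakeDamage, GetOnFire and IsDead to its BPCDamageSystem component.
; GetCurrentHealth, GetMaxHealth and Heal are stubs returning zero, and TakeDamage always returns false after forwarding the damage.
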(fn `GetCurrentHealth`
  (returns (Health :type "Float (double-precision)"))
  (return 0.0))

(fn `GetMaxHealth`
  (returns (MaxHealth :type "Float (double-precision)"))
  (return 0.0))

(fn `GetOnFire`
  (returns (OnFire :type Boolean))
  (bind _onfire (`/Game/Characters/DamageSystem/BPC_DamageSystem.IsOnFire` (`self.BPC_DamageSystem`)))
  (return _onfire))

(fn `Heal`
  (params (Amount :type "Float (double-precision)"))
  (returns (NewHealth :type "Float (double-precision)"))
  (return 0.0))

(fn `IsDead`
  (returns (IsDead :type Boolean))
  (bind _isdead (message `/Game/Characters/DamageSystem/BPI_Damagable.IsDead` (`self.BPC_DamageSystem`)))
  (return _isdead))

(fn `TakeDamage`
  (params (DamageInfo :type "/Game/Characters/DamageSystem/S_DamageInfo Structure"))
  (returns (WasDamaged :type Boolean))
  (`/Game/Characters/DamageSystem/BPC_DamageSystem.TakeDamage` (`self.BPC_DamageSystem`) DamageInfo)
  (return false))

(fn `UserConstructionScript`)