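; BP_Health is a bullet that damages what it hits and also rewrites that target's maximum health.
; Its CollisionBehavior event sends damagable actors a damage message carrying lifesteal and attacker data, then reports the damage event.
; For players and base enemies, it then sets the damage component's MaxHealth to BaseHealth plus the bullet's Damage.
; The bullet destroys itself on collision unless Piercing is at least one.
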(event `self.CollisionBehavior`
  (params (Location :type "Vector Structure") (DamagedActor :type "Actor Object Reference") (HitComponent :type "PrimitiveComponent Object Reference"))
  (cast `/Game/Characters/DamageSystem/BPI_Damagable` DamagedActor
    (:`then`
      (message `/Game/Characters/DamageSystem/BPI_Damagable.TakeDamage` DamagedActor (make `/Game/Characters/DamageSystem/S_DamageInfo` (`self.Damage`) (`self.DamageType`) "NewEnumerator1" false false false true (`self.Lifesteal`) (`self.GreaterLifesteal`) (`self.GetOwner`)))
      (`AISense_Damage.ReportDamageEvent` null (`self.GetOwner`) (`self.Damage`))
      (bind _asbp_player (cast `/Game/Characters/Player/BP_Player` DamagedActor)
        (:`then`
          (bind _bpc_damagesystem (`/Game/Characters/Player/BP_Player.BPC_DamageSystem` _asbp_player))
          (set `/Game/Characters/DamageSystem/BPC_DamageSystem.MaxHealth` (+ (`self.Damage`) (`/Game/Characters/DamageSystem/BPC_DamageSystem.BaseHealth` _bpc_damagesystem)) _bpc_damagesystem))
        (:`CastFailed`
          (bind _asbp_enemy_base (cast `/Game/Characters/Enemies/BP_Enemy_Base` DamagedActor)
            (:`then`
              (bind _bpc_damagesystem_2 (`/Game/Characters/Enemies/BP_Enemy_Base.BPC_DamageSystem` _asbp_enemy_base))
              (set `/Game/Characters/DamageSystem/BPC_DamageSystem.MaxHealth` (+ (`self.Damage`) (`/Game/Characters/DamageSystem/BPC_DamageSystem.BaseHealth` _bpc_damagesystem_2)) _bpc_damagesystem_2))
            (:`CastFailed`
              _)))))
    (:`CastFailed`
      _))
  (if (not (>= (`self.Piercing`) 1))
    (`self.K2_DestroyActor`)))

(fn `UserConstructionScript`
  (`parent.UserConstructionScript`))