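; BP_Weakness is a bullet that damages and weakens the damageable actors it hits.
; It overrides the collision behavior to send damage info with lifesteal through BPI_Damagable and report a damage event for its owner.
; The weaken strength scales from the bullet's damage, and its duration reuses the Lifetime value.
; The bullet destroys itself on hitting a valid actor unless it has piercing.
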(event `self.CollisionBehavior`
  (params (Location :type "Vector Structure") (DamagedActor :type "Actor Object Reference") (HitComponent :type "PrimitiveComponent Object Reference"))
  (bind _damage (`self.Damage`))
  (bind _asbpi_damagable (cast `/Game/Characters/DamageSystem/BPI_Damagable` DamagedActor)
    (:`then`
      (message `/Game/Characters/DamageSystem/BPI_Damagable.TakeDamage` DamagedActor (make `/Game/Characters/DamageSystem/S_DamageInfo` (`self.Damage`) (`self.DamageType`) "NewEnumerator1" false false false true (`self.Lifesteal`) (`self.GreaterLifesteal`) (`self.GetOwner`)))
      (`AISense_Damage.ReportDamageEvent` null (`self.GetOwner`) _damage)
      (`/Game/Characters/DamageSystem/BPI_Damagable.Weaken` _asbpi_damagable (/ _damage 5.0) (`self.Lifetime`)))
    (:`CastFailed`
      _))
  (if (not (or (>= (`self.Piercing`) 1) (not (`KismetSystemLibrary.IsValid` DamagedActor))))
    (`self.K2_DestroyActor`)))

(fn `UserConstructionScript`
  (`parent.UserConstructionScript`))