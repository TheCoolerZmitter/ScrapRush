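; Ice bullet, a child projectile that damages and freezes what it hits.
; Its collision event sends damage with forced interrupt and lifesteal to damageable actors, then reports a damage event credited to the owner.
; Enemies and players also receive Freeze, which reuses the bullet's Lifetime as duration and Damage as strength.
; The bullet destroys itself on hitting any valid actor unless it has Piercing of at least one.
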(event `self.CollisionBehavior`
  (params (Location :type "Vector Structure") (DamagedActor :type "Actor Object Reference") (HitComponent :type "PrimitiveComponent Object Reference"))
  (bind _lifetime (`self.Lifetime`))
  (bind _damage (`self.Damage`))
  (cast `/Game/Characters/DamageSystem/BPI_Damagable` DamagedActor
    (:`then`
      (message `/Game/Characters/DamageSystem/BPI_Damagable.TakeDamage` DamagedActor (make `/Game/Characters/DamageSystem/S_DamageInfo` (`self.Damage`) (`self.DamageType`) "NewEnumerator1" false false false true (`self.Lifesteal`) (`self.GreaterLifesteal`) (`self.GetOwner`)))
      (`AISense_Damage.ReportDamageEvent` null (`self.GetOwner`) (`self.Damage`))
      (bind _asbp_enemy_base (cast `/Game/Characters/Enemies/BP_Enemy_Base` DamagedActor)
        (:`then`
          (`/Game/Characters/Enemies/BP_Enemy_Base.Freeze` _asbp_enemy_base _lifetime _damage))
        (:`CastFailed`
          (bind _asbp_player (cast `/Game/Characters/Player/BP_Player` DamagedActor)
            (:`then`
              (`/Game/Characters/Player/BP_Player.Freeze` _asbp_player _lifetime _damage))
            (:`CastFailed`
              _)))))
    (:`CastFailed`
      _))
  (if (not (or (>= (`self.Piercing`) 1) (not (`KismetSystemLibrary.IsValid` DamagedActor))))
    (`self.K2_DestroyActor`)))

(fn `UserConstructionScript`
  (`parent.UserConstructionScript`))