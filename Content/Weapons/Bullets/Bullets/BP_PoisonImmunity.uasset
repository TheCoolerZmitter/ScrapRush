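; BP_PoisonImmunity is a bullet that damages what it hits and grants that target poison immunity.
; Its CollisionBehavior event calls DealDamage on actors implementing BPI_Damagable, then calls GrantPoisonImmunity on the damage system component of a BP_Player or BP_Enemy_Base.
; After any collision it destroys itself unless its Piercing value is at least one.
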(event `self.CollisionBehavior`
  (params (Location :type "Vector Structure") (DamagedActor :type "Actor Object Reference") (HitComponent :type "PrimitiveComponent Object Reference"))
  (cast `/Game/Characters/DamageSystem/BPI_Damagable` DamagedActor
    (:`then`
      (`self.DealDamage` DamagedActor)
      (bind _asbp_player (cast `/Game/Characters/Player/BP_Player` DamagedActor)
        (:`then`
          (`/Game/Characters/DamageSystem/BPC_DamageSystem.GrantPoisonImmunity` (`/Game/Characters/Player/BP_Player.BPC_DamageSystem` _asbp_player)))
        (:`CastFailed`
          (bind _asbp_enemy_base (cast `/Game/Characters/Enemies/BP_Enemy_Base` DamagedActor)
            (:`then`
              (`/Game/Characters/DamageSystem/BPC_DamageSystem.GrantPoisonImmunity` (`/Game/Characters/Enemies/BP_Enemy_Base.BPC_DamageSystem` _asbp_enemy_base)))
            (:`CastFailed`
              _)))))
    (:`CastFailed`
      _))
  (if (not (>= (`self.Piercing`) 1))
    (`self.K2_DestroyActor`)))

(fn `UserConstructionScript`
  (`parent.UserConstructionScript`))