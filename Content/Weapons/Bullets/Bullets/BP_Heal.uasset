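; BP_Heal is a bullet whose collision behavior heals the damageable actor it hits by its Damage value.
; After calling Heal through BPI_Damagable, it also sends that actor a damage message carrying the same amount, lifesteal values and a forced interrupt.
; It then reports a damage event credited to its owner and destroys itself on a valid hit unless it has Piercing.
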(event `self.CollisionBehavior`
  (params (Location :type "Vector Structure") (DamagedActor :type "Actor Object Reference") (HitComponent :type "PrimitiveComponent Object Reference"))
  (bind _asbpi_damagable (cast `/Game/Characters/DamageSystem/BPI_Damagable` DamagedActor))
  (`/Game/Characters/DamageSystem/BPI_Damagable.Heal` _asbpi_damagable (`self.Damage`))
  (message `/Game/Characters/DamageSystem/BPI_Damagable.TakeDamage` DamagedActor (make `/Game/Characters/DamageSystem/S_DamageInfo` (`self.Damage`) (`self.DamageType`) "NewEnumerator1" false false false true (`self.Lifesteal`) (`self.GreaterLifesteal`) (`self.GetOwner`)))
  (`AISense_Damage.ReportDamageEvent` null (`self.GetOwner`) (`self.Damage`))
  (if (not (or (>= (`self.Piercing`) 1) (not (`KismetSystemLibrary.IsValid` DamagedActor))))
    (`self.K2_DestroyActor`)))

(fn `UserConstructionScript`
  (`parent.UserConstructionScript`))