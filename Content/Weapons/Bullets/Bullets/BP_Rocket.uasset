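; Rocket projectile Blueprint that explodes on collision, dealing direct and area damage with lifesteal data.
; CollisionBehavior damages the hit actor, spawns scaled explosion effects and makes noise, then sphere-traces Pawns and WorldDynamic objects within Radius.
; DamageArray prevents repeat area hits, though not overlap with the direct hit; damage is also reported to AI perception.
; With Piercing or no valid hit actor, it clears that array and survives; otherwise it destroys itself.
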(event `self.CollisionBehavior`
  (params (Location :type "Vector Structure") (DamagedActor :type "Actor Object Reference") (HitComponent :type "PrimitiveComponent Object Reference"))
  (cast `/Game/Characters/DamageSystem/BPI_Damagable` DamagedActor
    (:`then`
      (message `/Game/Characters/DamageSystem/BPI_Damagable.TakeDamage` DamagedActor (make `/Game/Characters/DamageSystem/S_DamageInfo` (`self.Damage`) (`self.DamageType`) "NewEnumerator4" false false false true (`self.Lifesteal`) (`self.GreaterLifesteal`) (`self.GetOwner`)))
      (`AISense_Damage.ReportDamageEvent` null (`self.GetOwner`) 20.0 Location))
    (:`CastFailed`
      _))
  (`GameplayStatics.SpawnEmitterAtLocation` "/Game/M5VFXVOL2/Particles/Explosion/Fire_Exp_00.Fire_Exp_00" Location (struct) (`KismetMathLibrary.Conv_DoubleToVector` (/ (`self.Radius`) 300.0)) true "AutoRelease")
  (`GameplayStatics.PlaySoundAtLocation` "/Game/StarterContent/Audio/Explosion_Cue.Explosion_Cue" Location (struct) 1.0 1.0 0.0 null null null null)
  (`self.MakeNoise` 1.0 null Location)
  (bind _outhits (`KismetSystemLibrary.SphereTraceMultiForObjects` Location Location (`self.Radius`) (`|MakeArray` "ObjectTypeQuery3" "ObjectTypeQuery2" :!type "EObjectTypeQuery Enum")))
  (for _array_element _outhits
    (bind (_bblockinghit _binitialoverlap _time _distance _location _impactpoint _normal _impactnormal _physmat _hitactor) (`GameplayStatics.BreakHitResult` _array_element))
    (if (not (`KismetArrayLibrary.Array_Contains` (`self.DamageArray`) _hitactor))
      (message `/Game/Characters/DamageSystem/BPI_Damagable.TakeDamage` _hitactor (make `/Game/Characters/DamageSystem/S_DamageInfo` (`self.Damage`) (`self.DamageType`) "NewEnumerator4" false false false true (`self.Lifesteal`) (`self.GreaterLifesteal`) (`self.GetOwner`)))
      (`AISense_Damage.ReportDamageEvent` _hitactor (`self.GetOwner`) 20.0 Location)
      (`KismetArrayLibrary.Array_Insert` (`self.DamageArray`) _hitactor)))
  (if (or (>= (`self.Piercing`) 1) (not (`KismetSystemLibrary.IsValid` DamagedActor)))
    (`KismetArrayLibrary.Array_Clear` (`self.DamageArray`))
    (else
      (`self.K2_DestroyActor`))))

(fn `UserConstructionScript`
  (`parent.UserConstructionScript`))