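; Water projectile that damages and extinguishes whatever lies within a radius of its impact, overriding behavior from a parent bullet.
; Collision runs a sphere trace over pawns and dynamic objects, sending fire-out and damage messages once per actor and reporting damage to AI perception.
; Piercing shots clear the hit list and continue; others destroy themselves on valid hits.
; Lifetime expiry, unless cancelled, or an immediate kill triggers the same burst before destruction.
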(event `self.KillEventually`
  (`KismetSystemLibrary.Delay` (`self.Lifetime`))
  (if (not (`self.CancelDeletion`))
    (`self.CollisionBehavior` (`SceneComponent.K2_GetComponentLocation` (`self.Collider`)) :!label _label)
    (`self.K2_DestroyActor`)))

(event `self.KillNow`
  (goto _label))

(event `self.CollisionBehavior`
  (params (Location :type "Vector Structure") (DamagedActor :type "Actor Object Reference") (HitComponent :type "PrimitiveComponent Object Reference"))
  (bind _outhits (`KismetSystemLibrary.SphereTraceMultiForObjects` Location Location (`self.Radius`) (`|MakeArray` "ObjectTypeQuery3" "ObjectTypeQuery2" :!type "EObjectTypeQuery Enum")))
  (for _array_element _outhits
    (bind (_bblockinghit _binitialoverlap _time _distance _location _impactpoint _normal _impactnormal _physmat _hitactor) (`GameplayStatics.BreakHitResult` _array_element))
    (if (not (`KismetArrayLibrary.Array_Contains` (`self.DamageArray`) _hitactor))
      (message `/Game/Characters/DamageSystem/BPI_Damagable.PutOutFire` _hitactor)
      (message `/Game/Characters/DamageSystem/BPI_Damagable.TakeDamage` _hitactor (make `/Game/Characters/DamageSystem/S_DamageInfo` (`self.Damage`) (`self.DamageType`) "NewEnumerator2" false false false true (`self.Lifesteal`)))
      (`AISense_Damage.ReportDamageEvent` _hitactor (`self.GetOwner`) 20.0 Location)
      (`KismetArrayLibrary.Array_Insert` (`self.DamageArray`) _hitactor)))
  (if (or (>= (`self.Piercing`) 1) (not (`KismetSystemLibrary.IsValid` DamagedActor)))
    (`KismetArrayLibrary.Array_Clear` (`self.DamageArray`))
    (else
      (`self.K2_DestroyActor`))))

(fn `UserConstructionScript`
  (`parent.UserConstructionScript`))