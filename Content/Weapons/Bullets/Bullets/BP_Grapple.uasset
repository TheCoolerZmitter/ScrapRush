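; Grappling-hook bullet that launches its owner toward the point where the bullet collides or expires.
; CollisionBehavior applies a Damage-scaled impulse to the owning player or enemy's CharacterMovement, then destroys the bullet unless Piercing is at least 1.
; KillNow, or KillEventually after Lifetime unless CancelDeletion is set, runs the same pull at the bullet's current location before destroying it.
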(event `self.KillNow`
  (`self.CollisionBehavior` (`self.K2_GetActorLocation`) :!label _label)
  (`self.K2_DestroyActor`))

(event `self.KillEventually`
  (`KismetSystemLibrary.Delay` (`self.Lifetime`))
  (if (not (`self.CancelDeletion`))
    (goto _label)))

(event `self.CollisionBehavior`
  (params (Location :type "Vector Structure") (DamagedActor :type "Actor Object Reference") (HitComponent :type "PrimitiveComponent Object Reference"))
  (bind _returnvalue (`self.GetOwner`))
  (bind _returnvalue_2 (* (`KismetMathLibrary.Normal` (- Location (`self.K2_GetActorLocation` _returnvalue)) 0.0) (`self.Damage`) 20000.0))
  (bind _asbp_player (cast `/Game/Characters/Player/BP_Player` _returnvalue)
    (:`then`
      (`CharacterMovementComponent.AddImpulse` (`Character.CharacterMovement` _asbp_player) _returnvalue_2 false)
      (if (not (>= (`self.Piercing`) 1)) :!label _label_2
        (`self.K2_DestroyActor`)))
    (:`CastFailed`
      (bind _asbp_enemy_base (cast `/Game/Characters/Enemies/BP_Enemy_Base` _returnvalue)
        (:`then`
          (`CharacterMovementComponent.AddImpulse` (`Character.CharacterMovement` _asbp_enemy_base) _returnvalue_2 false)
          (goto _label_2))
        (:`CastFailed`
          (`self.K2_DestroyActor`))))))

(fn `UserConstructionScript`
  (`parent.UserConstructionScript`))