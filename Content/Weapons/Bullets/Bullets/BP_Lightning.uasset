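; BP_Lightning is a bullet that deals chain lightning damage on collision.
; A hit on a damageable actor, or the owner, starts a bounded loop whose length scales with Lifetime.
; Each jump sphere-traces pawns around the last point, damages the first living, unhit one and re-centers there, drawing a debug line trace between points.
; DamagedActors prevents repeat hits, and the bullet destroys itself unless Piercing.
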(event `self.CollisionBehavior`
  (params (Location :type "Vector Structure") (DamagedActor :type "Actor Object Reference") (HitComponent :type "PrimitiveComponent Object Reference"))
  (bind _centerpoint (`self.CenterPoint`))
  (bind _damagedactors (`self.DamagedActors`))
  (set `self.CenterPoint` Location)
  (if (== DamagedActor (`self.GetOwner`))
    (`KismetArrayLibrary.Array_Add` (`self.DamagedActors`) (`self.GetOwner`))
    (for _index (range (+ (`KismetMathLibrary.FTrunc` (* (+ (`self.Lifetime`) 1.0) 3.0)) 1)) :!label _label
      (if (`KismetArrayLibrary.Array_IsValidIndex` (`self.DamagedActors`) _index)
        (set `self.PrevPoint` (`self.CenterPoint`))
        (bind _outhits (`KismetSystemLibrary.SphereTraceMultiForObjects` _centerpoint _centerpoint (`self.Radius`) (`|MakeArray` "ObjectTypeQuery3" :!type "EObjectTypeQuery Enum") false (`|MakeArray` (`self.GetOwner`))))
        (for _array_element _outhits
          (bind (_bblockinghit _binitialoverlap _time _distance _location _impactpoint _normal _impactnormal _physmat _hitactor) (`GameplayStatics.BreakHitResult` _array_element))
          (cast `/Game/Characters/DamageSystem/BPI_Damagable` _hitactor)
          (if (not (`KismetArrayLibrary.Array_Contains` (`self.DamagedActors`) _hitactor))
            (bind _isdead (message `/Game/Characters/DamageSystem/BPI_Damagable.IsDead` _hitactor))
            (if (not _isdead)
              (bind _returnvalue (`KismetArrayLibrary.Array_Add` _damagedactors _hitactor))
              (bind _output_get (set `self.CenterPoint` (`self.K2_GetActorLocation` (`|GetArrayItem` _damagedactors _returnvalue))))
              (`KismetSystemLibrary.LineTraceSingle` :`Start` (`self.PrevPoint`) :`End` _output_get :`TraceChannel` "TraceTypeQuery1" :`DrawDebugType` "ForDuration")
              (message `/Game/Characters/DamageSystem/BPI_Damagable.TakeDamage` _hitactor (make `/Game/Characters/DamageSystem/S_DamageInfo` (`self.Damage`) "NewEnumerator4" "NewEnumerator1" false false false true))
              (`AISense_Damage.ReportDamageEvent` null (`self.GetOwner`) 20.0)
              (break))))
        (else
          (break))))
    (if (not (>= (`self.Piercing`) 1))
      (`self.K2_DestroyActor`))
    (else
      (cast `/Game/Characters/DamageSystem/BPI_Damagable` DamagedActor
        (:`then`
          (message `/Game/Characters/DamageSystem/BPI_Damagable.TakeDamage` DamagedActor (make `/Game/Characters/DamageSystem/S_DamageInfo` (`self.Damage`) "NewEnumerator4" "NewEnumerator1" false false false true))
          (`AISense_Damage.ReportDamageEvent` null (`self.GetOwner`) 20.0 Location)
          (`KismetArrayLibrary.Array_Add` (`self.DamagedActors`) DamagedActor)
          (goto _label))
        (:`CastFailed`
          (if (not (>= (`self.Piercing`) 1))
            (`self.K2_DestroyActor`)))))))

(fn `UserConstructionScript`
  (`parent.UserConstructionScript`))