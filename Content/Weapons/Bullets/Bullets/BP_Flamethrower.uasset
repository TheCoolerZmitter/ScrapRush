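; Flamethrower projectile, a child bullet Blueprint whose lifetime is tied to weapon cooldown instead of the lifetime passed in.
; SetStats combines incoming stats with its own by multiplying, adding or OR-ing, sets projectile movement velocity and enables physics calculation only below a speed threshold.
; On collision, it sends damageable actors a typed damage message that forces interruption, then reports the damage event with its owner as instigator.
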(event `self.ReceiveBeginPlay`
  (set `self.Lifetime` (* (`self.Cooldown`) 1.6))
  (`parent.ReceiveBeginPlay`))

(event `self.CollisionBehavior`
  (params (Location :type "Vector Structure") (DamagedActor :type "Actor Object Reference") (HitComponent :type "PrimitiveComponent Object Reference"))
  (cast `/Game/Characters/DamageSystem/BPI_Damagable` DamagedActor)
  (message `/Game/Characters/DamageSystem/BPI_Damagable.TakeDamage` DamagedActor (make `/Game/Characters/DamageSystem/S_DamageInfo` (`self.Damage`) "NewEnumerator3" "NewEnumerator4" false false false true))
  (`AISense_Damage.ReportDamageEvent` DamagedActor (`self.GetOwner`) (`self.Damage`)))

(event `self.SetStats`
  (params (Direction :type "Vector Structure") (Velocity :type "Float (double-precision)") (Lifetime :type "Float (double-precision)") (Damage :type "Float (double-precision)") (Piercing :type Integer) (Statis :type Boolean) (InstantActivate :type Boolean) (Gravity :type "Float (double-precision)") (Bounce :type Boolean) (PhaseEnemies :type Boolean) (Homing :type "Float (double-precision)") (Radius :type "Float (double-precision)") (AttackTarget :type "Actor Object Reference") (Knockback :type "Float (double-precision)"))
  (bind _output_get (set `self.Velocity` (* Velocity (`self.Velocity`))))
  (bind _output_get_2 (set `self.Direction` (* Direction _output_get)))
  (set `MovementComponent.Velocity` _output_get_2 (`self.ProjectileMovement`))
  (set `self.DoPhysicsCalculation` (< (`self.Velocity`) 8000.0))
  (set `self.Lifetime` (* (`self.Cooldown`) 1.6))
  (set `self.Damage` (* (`self.Damage`) Damage))
  (set `self.Piercing` (+ (`self.Piercing`) Piercing))
  (set `self.Statis` Statis)
  (set `self.InstantActivate` (or InstantActivate (`self.InstantActivate`)))
  (set `self.Gravity` (+ (`self.Gravity`) Gravity))
  (set `self.Bounce` (or Bounce (`self.Bounce`)))
  (set `self.PhaseEnemies` (or PhaseEnemies (`self.PhaseEnemies`)))
  (set `self.Homing` (+ (`self.Homing`) Homing))
  (set `self.Radius` (* (`self.Radius`) Radius))
  (set `self.AttackTarget` AttackTarget)
  (set `self.Knockback` (+ (`self.Knockback`) Knockback)))

(fn `UserConstructionScript`
  (`parent.UserConstructionScript`))