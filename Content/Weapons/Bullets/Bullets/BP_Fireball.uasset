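; BP_Fireball is a fireball projectile Blueprint that damages what it hits.
; Its CollisionBehavior event sends a forced-interrupt damage message to actors implementing BPI_Damagable, then reports the damage event with the projectile's owner as instigator.
; It destroys itself on collision unless Piercing is at least one; this graph never decrements that value.
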(event `self.CollisionBehavior`
  (params (Location :type "Vector Structure") (DamagedActor :type "Actor Object Reference") (HitComponent :type "PrimitiveComponent Object Reference"))
  (cast `/Game/Characters/DamageSystem/BPI_Damagable` DamagedActor
    (:`then`
      (message `/Game/Characters/DamageSystem/BPI_Damagable.TakeDamage` DamagedActor (make `/Game/Characters/DamageSystem/S_DamageInfo` (`self.Damage`) (`self.DamageType`) "NewEnumerator2" false false false true))
      (`AISense_Damage.ReportDamageEvent` DamagedActor (`self.GetOwner`) (`self.Damage`)))
    (:`CastFailed`
      _))
  (if (not (>= (`self.Piercing`) 1))
    (`self.K2_DestroyActor`)))

(fn `UserConstructionScript`
  (`parent.UserConstructionScript`))