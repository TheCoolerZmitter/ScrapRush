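; BP_Fix is a bullet that yanks what it hits to the location of the bullet's owner.
; On collision, damageable actors take forced-interrupt damage with lifesteal and a reported damage event, while pickups skip damage.
; Both are then moved by a swept SetActorLocation, with characters' vertical velocity zeroed first.
; Other hits destroy the bullet, as do pulls when Piercing is below one.
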(event `self.CollisionBehavior`
  (params (Location :type "Vector Structure") (DamagedActor :type "Actor Object Reference") (HitComponent :type "PrimitiveComponent Object Reference") (Normal :type "Vector Structure"))
  (cast `/Game/Characters/DamageSystem/BPI_Damagable` DamagedActor
    (:`then`
      (message `/Game/Characters/DamageSystem/BPI_Damagable.TakeDamage` DamagedActor (make `/Game/Characters/DamageSystem/S_DamageInfo` (`self.Damage`) (`self.DamageType`) "NewEnumerator1" false false false true (`self.Lifesteal`)))
      (`AISense_Damage.ReportDamageEvent` DamagedActor (`self.GetOwner`) (`self.Damage`) (`KismetMathLibrary.MakeVector` Location_X Location_Y Location_Z))
      (`/Engine/EditorBlueprintResources/StandardMacros.IsValid` DamagedActor :!label _label
        (:`Is Valid`
          (bind _ascharacter (cast `Character` DamagedActor)
            (:`then`
              (bind _charactermovement (`Character.CharacterMovement` _ascharacter))
              (bind (_velocity_x _velocity_y) (`KismetMathLibrary.BreakVector` (`MovementComponent.Velocity` _charactermovement)))
              (set `MovementComponent.Velocity` (`KismetMathLibrary.MakeVector` _velocity_x _velocity_y) _charactermovement))
            (:`CastFailed`
              _))
          (`self.K2_SetActorLocation` DamagedActor (`self.K2_GetActorLocation` (`self.GetOwner`)) true false)
          (if (not (or (>= (`self.Piercing`) 1) (not (`KismetSystemLibrary.IsValid` DamagedActor))))
            (`self.K2_DestroyActor`)))
        (:`Is Not Valid`
          (`self.K2_DestroyActor`))))
    (:`CastFailed`
      (cast `/Game/Weapons/Spawners/BP_PickupBase` DamagedActor
        (:`then`
          (goto _label))
        (:`CastFailed`
          (`self.K2_DestroyActor`))))))

(fn `UserConstructionScript`
  (`parent.UserConstructionScript`))