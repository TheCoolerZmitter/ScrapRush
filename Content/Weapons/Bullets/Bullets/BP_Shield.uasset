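; Shield projectile that, on overlapping anything but another projectile, spawns a ring of three ShieldObjects scaled by Radius, with health equal to Damage.
; The ring centres on the hit player or enemy, or otherwise on the impact point.
; If the third shield spawns, damageable targets also take a half-Damage message.
; It then re-arms after a short delay when Piercing, else destroys itself; UnStatis launches it using overlaps or a line trace.
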(event `self.Collider.OnComponentBeginOverlap`
  (params (OverlappedComponent :type "PrimitiveComponent Object Reference") (OtherActor :type "Actor Object Reference") (OtherComp :type "PrimitiveComponent Object Reference") (OtherBodyIndex :type Integer) (bFromSweep :type Boolean) (SweepResult :type "HitResult Structure (by ref)"))
  (set `PrimitiveComponent.bGenerateOverlapEvents` false (`self.Collider`))
  (if (`self.ValuesUpdated`)
    (if (not (`self.Statis`))
      (cast `/Game/Weapons/Bullets/Bullets/BP_ProjectileBase` OtherActor
        (:`CastFailed`
          (`self.CollisionBehavior` (`SceneComponent.K2_GetComponentLocation` (`self.Collider`)) OtherActor))))
    (else
      (`KismetSystemLibrary.DelayUntilNextTick`))))

(event `self.CollisionBehavior`
  (params (Location :type "Vector Structure") (DamagedActor :type "Actor Object Reference") (HitComponent :type "PrimitiveComponent Object Reference"))
  (bind _damage (`self.Damage`))
  (bind _radius (`self.Radius`))
  (bind _radius_2 (`self.Radius`))
  (bind _radius_3 (`self.Radius`))
  (bind _damage_2 (`self.Damage`))
  (bind _damage_3 (`self.Damage`))
  (bind (_returnvalue_roll _returnvalue_pitch _returnvalue_yaw) (`KismetMathLibrary.BreakRotator` (`KismetMathLibrary.MakeRotFromX` (`self.OwnerForward`))))
  (bind (_returnvalue_roll_2 _returnvalue_pitch_2 _returnvalue_yaw_2) (`KismetMathLibrary.BreakRotator` (`KismetMathLibrary.MakeRotFromX` (`self.OwnerForward`))))
  (bind (_returnvalue_roll_3 _returnvalue_pitch_3 _returnvalue_yaw_3) (`KismetMathLibrary.BreakRotator` (`KismetMathLibrary.MakeRotFromX` (`self.OwnerForward`))))
  (bind _returnvalue (/ _radius_2 200.0))
  (bind _returnvalue_2 (/ _radius 200.0))
  (bind _returnvalue_3 (/ _radius_3 200.0))
  (cast `/Game/Characters/Player/BP_Player` DamagedActor
    (:`then`
      (set `self.OwnerLocation` (- (`self.K2_GetActorLocation` DamagedActor) (0.0 0.0 225.0)) :!label _label)
      (set `self.OwnerForward` (`self.GetActorForwardVector` DamagedActor)))
    (:`CastFailed`
      (cast `/Game/Characters/Enemies/BP_Enemy_Base` DamagedActor
        (:`then`
          (goto _label))
        (:`CastFailed`
          (set `self.OwnerLocation` (- Location (0.0 0.0 130.0)))
          (set `self.OwnerForward` (`KismetMathLibrary.Normal` (* (`self.GetActorForwardVector`) (1.0 1.0 0.0)) 0.0))))))
  (bind _returnvalue_4 (`|SpawnActorFromClass` "/Game/Weapons/Bullets/Bullets/ShieldObject.ShieldObject_C" (`KismetMathLibrary.MakeTransform` (+ (`self.OwnerLocation`) (* (`KismetMathLibrary.RotateAngleAxis` (`self.OwnerForward`) -19.0 (0.0 0.0 1.0)) _radius)) (`KismetMathLibrary.MakeRotator` 0.0 0.0 (+ _returnvalue_yaw_2 200.0)) (`KismetMathLibrary.MakeVector` _returnvalue_2 _returnvalue_2 1.3)) "Undefined" "MultiplyWithRoot" null null))
  (`/Engine/EditorBlueprintResources/StandardMacros.IsValid` _returnvalue_4
    (:`Is Valid`
      (set `/Game/Weapons/Bullets/Bullets/ShieldObject.MaxHealth` _damage_2 _returnvalue_4)
      (set `/Game/Weapons/Bullets/Bullets/ShieldObject.Health` _damage_2 _returnvalue_4))
    (:`Is Not Valid`
      _))
  (bind _returnvalue_5 (`|SpawnActorFromClass` "/Game/Weapons/Bullets/Bullets/ShieldObject.ShieldObject_C" (`KismetMathLibrary.MakeTransform` (+ (`self.OwnerLocation`) (* (`KismetMathLibrary.RotateAngleAxis` (`self.OwnerForward`) -139.0 (0.0 0.0 1.0)) _radius_3)) (`KismetMathLibrary.MakeRotator` 0.0 0.0 (+ _returnvalue_yaw_3 80.0)) (`KismetMathLibrary.MakeVector` _returnvalue_3 _returnvalue_3 1.3)) "Undefined" "MultiplyWithRoot" null null))
  (`/Engine/EditorBlueprintResources/StandardMacros.IsValid` _returnvalue_5
    (:`Is Valid`
      (set `/Game/Weapons/Bullets/Bullets/ShieldObject.MaxHealth` _damage_3 _returnvalue_5)
      (set `/Game/Weapons/Bullets/Bullets/ShieldObject.Health` _damage_3 _returnvalue_5))
    (:`Is Not Valid`
      _))
  (bind _returnvalue_6 (`|SpawnActorFromClass` "/Game/Weapons/Bullets/Bullets/ShieldObject.ShieldObject_C" (`KismetMathLibrary.MakeTransform` (+ (`self.OwnerLocation`) (* (`KismetMathLibrary.RotateAngleAxis` (`self.OwnerForward`) 101.0 (0.0 0.0 1.0)) _radius_2)) (`KismetMathLibrary.MakeRotator` 0.0 0.0 (+ _returnvalue_yaw 320.0)) (`KismetMathLibrary.MakeVector` _returnvalue _returnvalue 1.3)) "Undefined" "MultiplyWithRoot" null null))
  (`/Engine/EditorBlueprintResources/StandardMacros.IsValid` _returnvalue_6
    (:`Is Valid`
      (set `/Game/Weapons/Bullets/Bullets/ShieldObject.MaxHealth` _damage _returnvalue_6)
      (set `/Game/Weapons/Bullets/Bullets/ShieldObject.Health` _damage _returnvalue_6)
      (cast `/Game/Characters/DamageSystem/BPI_Damagable` DamagedActor
        (:`then`
          (message `/Game/Characters/DamageSystem/BPI_Damagable.TakeDamage` DamagedActor (make `/Game/Characters/DamageSystem/S_DamageInfo` (/ (`self.Damage`) 2.0) (`self.DamageType`) "NewEnumerator1" false false false true (`self.Lifesteal`) (`self.GreaterLifesteal`) (`self.GetOwner`)))
          (`AISense_Damage.ReportDamageEvent` DamagedActor (`self.GetOwner`) 0.1))
        (:`CastFailed`
          _)))
    (:`Is Not Valid`
      _))
  (if (>= (`self.Piercing`) 1)
    (`KismetSystemLibrary.Delay` 0.1)
    (set `PrimitiveComponent.bGenerateOverlapEvents` true (`self.Collider`))
    (else
      (`self.K2_DestroyActor`))))

(fn `CustomStasis`
  (set `self.OwnerForward` (`KismetMathLibrary.Normal` (* (`self.GetActorForwardVector`) (1.0 1.0 0.0)) 0.0)))

(fn `UnStatis`
  (set `MovementComponent.Velocity` (`self.Direction`) (`self.ProjectileMovement`))
  (set `self.Statis` false)
  (if (`self.DoPhysicsCalculation`)
    (set `PrimitiveComponent.bGenerateOverlapEvents` true (`self.Collider`))
    (`self.KillEventually`)
    (else
      (`self.DoLineTrace`))))

(fn `UserConstructionScript`
  (`parent.UserConstructionScript`))