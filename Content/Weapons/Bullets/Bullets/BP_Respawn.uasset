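; BP_Respawn is a bullet that makes rooms regenerate their content on hit, as well as damaging damageable targets.
; CollisionBehavior deals damage through BPI_Damagable, then resets ContentGenerated and calls GenerateContent on every Master_Room overlapping the hit actor.
; A directly hit room regenerates itself, while other non-damageable actors regenerate their overlapping rooms without taking damage.
; The bullet destroys itself after a hit when Piercing is below one.
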(event `self.CollisionBehavior`
  (params (Location :type "Vector Structure") (DamagedActor :type "Actor Object Reference") (HitComponent :type "PrimitiveComponent Object Reference"))
  (cast `/Game/Characters/DamageSystem/BPI_Damagable` DamagedActor
    (:`then`
      (`self.DealDamage` DamagedActor)
      (bind _output_get (set `self.Overlapping Actors` (`self.GetOverlappingActors` DamagedActor "/Game/Rooms/Rooms/Master_Room.Master_Room_C") :!label _label))
      (for _array_element _output_get
        (bind _asmaster_room (cast `/Game/Rooms/Rooms/Master_Room` _array_element :!pure true))
        (set `/Game/Rooms/Rooms/Master_Room.ContentGenerated` false _asmaster_room)
        (`/Game/Rooms/Rooms/Master_Room.GenerateContent` _asmaster_room)))
    (:`CastFailed`
      (bind _asmaster_room_2 (cast `/Game/Rooms/Rooms/Master_Room` DamagedActor)
        (:`then`
          (set `/Game/Rooms/Rooms/Master_Room.ContentGenerated` false _asmaster_room_2)
          (`/Game/Rooms/Rooms/Master_Room.GenerateContent` _asmaster_room_2))
        (:`CastFailed`
          (goto _label)))))
  (if (not (or (>= (`self.Piercing`) 1) (not (`KismetSystemLibrary.IsValid` null))))
    (`self.K2_DestroyActor`)))

(fn `UserConstructionScript`
  (`parent.UserConstructionScript`))