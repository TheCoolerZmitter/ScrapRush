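; BP_Bubble is a bubble projectile that captures the first projectile it overlaps and carries it as a payload.
; It slows every tick, with optional spiral motion.
; The captured bullet is hidden, stilled and attached to the collider.
; Hitting a damageable deals bubble damage and triggers the payload's collision behavior, with piercing deciding what survives, while KillNow or lifetime expiry releases and triggers the payload.
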(event `self.ReceiveBeginPlay`
  (`parent.ReceiveBeginPlay`)
  (`self.SetActorTickEnabled` true))

(event `self.ReceiveTick`
  (params (DeltaSeconds :type "Float (single-precision)"))
  (bind _projectilemovement (`self.ProjectileMovement`))
  (bind _projectilemovement_2 (`self.ProjectileMovement`))
  (bind _acceleration (`self.Acceleration`))
  (bind _spiral (`self.Spiral`))
  (bind _returnvalue (* (`GameplayStatics.GetTimeSeconds`) (/ (`self.Velocity`) 200.0)))
  (set `MovementComponent.Velocity` (* (`MovementComponent.Velocity` _projectilemovement) 0.98) _projectilemovement)
  (if (not (== (`self.Spiral`) 0.0))
    (`SceneComponent.K2_AddRelativeLocation` (`self.Collider`) (`KismetMathLibrary.MakeVector` 0.0 (* (`KismetMathLibrary.Cos` _returnvalue) _spiral) (* (`KismetMathLibrary.Sin` _returnvalue) _spiral)) false false))
  (if (not (== _acceleration 1.0))
    (set `MovementComponent.Velocity` (* (`MovementComponent.Velocity` _projectilemovement_2) (`KismetMathLibrary.MultiplyMultiply_FloatFloat` _acceleration (* 0.0 60.0))) _projectilemovement_2)))

(event `self.Collider.OnComponentBeginOverlap`
  (params (OverlappedComponent :type "PrimitiveComponent Object Reference") (OtherActor :type "Actor Object Reference") (OtherComp :type "PrimitiveComponent Object Reference") (OtherBodyIndex :type Integer) (bFromSweep :type Boolean) (SweepResult :type "HitResult Structure (by ref)"))
  (`self.AbsorbOrCollide` OtherActor))

(event `self.ReceiveDestroyed`
  (`self.SetActorTickEnabled` false))

(event `AbsorbOrCollide`
  (params (Actor :type "Actor Object Reference"))
  (bind _asbp_projectile_base (cast `/Game/Weapons/Bullets/Bullets/BP_ProjectileBase` Actor)
    (:`then`
      (`PrimitiveComponent.SetCollisionResponseToChannel` (`self.Collider`) "ECC_GameTraceChannel2" "ECR_Ignore")
      (`/Engine/EditorBlueprintResources/StandardMacros.IsValid` (`self.InnerBullet`)
        (:`Is Valid`
          (if (== (`/Game/Weapons/Bullets/Bullets/BP_ProjectileBase.Piercing` _asbp_projectile_base) 0)
            (`self.BubbleCollision` (`self.K2_GetActorLocation`) Actor :!label _label)))
        (:`Is Not Valid`
          (`PrimitiveComponent.SetCollisionEnabled` (`/Game/Weapons/Bullets/Bullets/BP_ProjectileBase.Collider` _asbp_projectile_base) "NoCollision")
          (bind _output_get (set `self.InnerBullet` _asbp_projectile_base))
          (`self.SetOwner` _output_get null)
          (`SceneComponent.SetVisibility` (`/Game/Weapons/Bullets/Bullets/BP_ProjectileBase.Scene` _output_get) false true)
          (set `/Game/Weapons/Bullets/Bullets/BP_ProjectileBase.DoPhysicsCalculation` true _output_get)
          (bind _projectilemovement (`/Game/Weapons/Bullets/Bullets/BP_ProjectileBase.ProjectileMovement` _output_get))
          (set `ProjectileMovementComponent.ProjectileGravityScale` 0.0 _projectilemovement)
          (set `/Game/Weapons/Bullets/Bullets/BP_ProjectileBase.CancelDeletion` true _output_get)
          (`SceneComponent.K2_AttachToComponent` (`/Game/Weapons/Bullets/Bullets/BP_ProjectileBase.Collider` _output_get) (`self.Collider`) "None" "KeepWorld" "KeepWorld" "KeepWorld" true)
          (`ProjectileMovementComponent.SetVelocityInLocalSpace` _projectilemovement (0.0 0.0 0.0)))))
    (:`CastFailed`
      (cast `/Game/Characters/DamageSystem/BPI_Damagable` Actor)
      (if (not (`self.PhaseEnemies`))
        (goto _label)))))

(event `self.KillNow`
  (bind _innerbullet (`self.InnerBullet`))
  (`/Engine/EditorBlueprintResources/StandardMacros.IsValid` _innerbullet :!label _label_2
    (:`Is Valid`
      (`self.UnStatis` _innerbullet)
      (`PrimitiveComponent.SetCollisionEnabled` (`/Game/Weapons/Bullets/Bullets/BP_ProjectileBase.Collider` _innerbullet) "QueryOnly")
      (`self.CollisionBehavior` _innerbullet (`SceneComponent.K2_GetComponentLocation` (`self.Collider`)) null null)
      (`self.K2_DestroyActor`))
    (:`Is Not Valid`
      (`self.K2_DestroyActor`))))

(event `self.KillEventually`
  (`KismetSystemLibrary.Delay` (`self.Lifetime`))
  (if (not (`self.CancelDeletion`))
    (goto _label_2)))

(event `BubbleCollision`
  (params (Location :type "Vector Structure") (DamagedActor :type "Actor Object Reference"))
  (bind _innerbullet (`self.InnerBullet`))
  (bind _returnvalue (> (`self.Piercing`) 0))
  (cast `/Game/Characters/DamageSystem/BPI_Damagable` DamagedActor)
  (message `/Game/Characters/DamageSystem/BPI_Damagable.TakeDamage` DamagedActor (make `/Game/Characters/DamageSystem/S_DamageInfo` (`self.Damage`) (`self.DamageType`) "NewEnumerator1" false false false true (`self.Lifesteal`)))
  (`AISense_Damage.ReportDamageEvent` DamagedActor (`self.GetOwner`) (`self.Damage`) Location)
  (`/Engine/EditorBlueprintResources/StandardMacros.IsValid` _innerbullet
    (:`Is Valid`
      (if (>= (`/Game/Weapons/Bullets/Bullets/BP_ProjectileBase.Piercing` _innerbullet) 1)
        (`self.CollisionBehavior` _innerbullet Location DamagedActor null)
        (if (not _returnvalue)
          (`PrimitiveComponent.SetCollisionEnabled` (`/Game/Weapons/Bullets/Bullets/BP_ProjectileBase.Collider` _innerbullet) "QueryOnly")
          (`self.UnStatis` _innerbullet)
          (`self.K2_DestroyActor` :!label _label_3))
        (else
          (`self.CollisionBehavior` _innerbullet Location DamagedActor null)
          (if (not _returnvalue)
            (goto _label_3)))))
    (:`Is Not Valid`
      (goto _label_3))))

(event `self.ProjectileMovement.OnProjectileBounce`
  (params (ImpactResult :type "HitResult Structure (by ref)") (ImpactVelocity :type "Vector Structure (by ref)"))
  (`self.BubbleCollision` ImpactResult_ImpactPoint)
  (`self.DoCluster` ImpactResult_Normal ImpactResult_HitActor (`SceneComponent.K2_GetComponentLocation` (`self.Collider`))))

(fn `UserConstructionScript`
  (`parent.UserConstructionScript`))