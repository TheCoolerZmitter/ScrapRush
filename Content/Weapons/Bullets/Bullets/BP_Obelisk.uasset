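; Projectile Blueprint that spawns an obelisk where it collides with anything other than another projectile.
; The obelisk spawns below the impact, scaled by Radius, with health equal to Damage and yaw from the horizontal forward cached in CustomStasis.
; If the spawn succeeds, damageable targets take half Damage.
; The projectile then re-enables overlaps after a short delay when piercing or lacking a valid target, and otherwise destroys itself.
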(event `self.Collider.OnComponentBeginOverlap`
  (params (OverlappedComponent :type "PrimitiveComponent Object Reference") (OtherActor :type "Actor Object Reference") (OtherComp :type "PrimitiveComponent Object Reference") (OtherBodyIndex :type Integer) (bFromSweep :type Boolean) (SweepResult :type "HitResult Structure (by ref)"))
  (set `PrimitiveComponent.bGenerateOverlapEvents` false (`self.Collider`))
  (if (`self.ValuesUpdated`)
    (if (not (`self.Statis`))
      (cast `/Game/Weapons/Bullets/Bullets/BP_ProjectileBase` OtherActor
        (:`CastFailed`
          (`self.CollisionBehavior` (`SceneComponent.K2_GetComponentLocation` (`self.Collider`)) OtherActor))))
    (else
      (`KismetSystemLibrary.DelayUntilNextTick`))))

(event `self.CollisionBehavior`
  (params (Location :type "Vector Structure") (DamagedActor :type "Actor Object Reference") (HitComponent :type "PrimitiveComponent Object Reference"))
  (bind _damage (`self.Damage`))
  (bind (_returnvalue_roll _returnvalue_pitch _returnvalue_yaw) (`KismetMathLibrary.BreakRotator` (`KismetMathLibrary.MakeRotFromX` (`self.OwnerForward`))))
  (bind _returnvalue (/ (`self.Radius`) 200.0))
  (bind _returnvalue_2 (`|SpawnActorFromClass` "/Game/Weapons/Bullets/Bullets/ObeliskObject.ObeliskObject_C" (`KismetMathLibrary.MakeTransform` (- Location (`KismetMathLibrary.MakeVector` 0.0 0.0 (* (`self.Radius`) 6.0))) (`KismetMathLibrary.MakeRotator` _returnvalue_roll _returnvalue_pitch _returnvalue_yaw) (`KismetMathLibrary.MakeVector` _returnvalue _returnvalue _returnvalue)) "Undefined" "MultiplyWithRoot" null null))
  (`/Engine/EditorBlueprintResources/StandardMacros.IsValid` _returnvalue_2
    (:`Is Valid`
      (set `/Game/Weapons/Bullets/Bullets/ObeliskObject."radius"` (* (`self.Radius`) 4.0) _returnvalue_2)
      (set `/Game/Weapons/Bullets/Bullets/ObeliskObject.MaxHealth` _damage _returnvalue_2)
      (set `/Game/Weapons/Bullets/Bullets/ObeliskObject.Health` _damage _returnvalue_2)
      (cast `/Game/Characters/DamageSystem/BPI_Damagable` DamagedActor
        (:`then`
          (message `/Game/Characters/DamageSystem/BPI_Damagable.TakeDamage` DamagedActor (make `/Game/Characters/DamageSystem/S_DamageInfo` (/ (`self.Damage`) 2.0) (`self.DamageType`) "NewEnumerator1" false false false true (`self.Lifesteal`) (`self.GreaterLifesteal`) (`self.GetOwner`)))
          (`AISense_Damage.ReportDamageEvent` DamagedActor (`self.GetOwner`) 0.1))
        (:`CastFailed`
          _)))
    (:`Is Not Valid`
      _))
  (if (or (>= (`self.Piercing`) 1) (not (`KismetSystemLibrary.IsValid` DamagedActor)))
    (`KismetSystemLibrary.Delay` 0.1)
    (set `PrimitiveComponent.bGenerateOverlapEvents` true (`self.Collider`))
    (else
      (`self.K2_DestroyActor`))))

(fn `CustomStasis`
  (set `self.OwnerForward` (`KismetMathLibrary.Normal` (* (`self.GetActorForwardVector`) (1.0 1.0 0.0)) 0.0)))

(fn `UnStatis`
  (set `MovementComponent.Velocity` (`self.Direction`) (`self.ProjectileMovement`))
  (set `self.Statis` false)
  (if (`self.DoPhysicsCalculation`)
    (set `PrimitiveComponent.bGenerateOverlapEvents` true (`self.Collider`))
    (`self.KillEventually`)
    (else
      (`self.DoLineTrace`))))

(fn `UserConstructionScript`
  (`parent.UserConstructionScript`))