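; Condensed gas bullet that damages what it hits and leaves a CondensedGasObject at the impact point.
; The spawned gas scales with Radius, lasts ten times the bullet's Lifetime and takes its Strength from Damage.
; Without Piercing, the bullet destroys itself on hitting a valid actor.
; Unless deletion is cancelled, lifetime expiry also triggers the collision behavior before bursting, while KillNow only bursts and destroys.
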(event `self.CollisionBehavior`
  (params (Location :type "Vector Structure") (DamagedActor :type "Actor Object Reference") (HitComponent :type "PrimitiveComponent Object Reference"))
  (bind _returnvalue (/ (`self.Radius`) 75.0))
  (message `/Game/Characters/DamageSystem/BPI_Damagable.TakeDamage` DamagedActor (make `/Game/Characters/DamageSystem/S_DamageInfo` (`self.Damage`) (`self.DamageType`) "NewEnumerator1" false false false true (`self.Lifesteal`) (`self.GreaterLifesteal`) (`self.GetOwner`)))
  (`AISense_Damage.ReportDamageEvent` DamagedActor (`self.GetOwner`) (`self.Damage`))
  (bind _returnvalue_2 (`|SpawnActorFromClass` "/Game/Weapons/Bullets/Bullets/CondensedGasObject.CondensedGasObject_C" (`KismetMathLibrary.MakeTransform` Location (struct) (`KismetMathLibrary.MakeVector` _returnvalue _returnvalue _returnvalue)) "Undefined" "MultiplyWithRoot" null null))
  (`/Engine/EditorBlueprintResources/StandardMacros.IsValid` _returnvalue_2
    (:`Is Valid`
      (`/Game/Weapons/Bullets/Bullets/CondensedGasObject.SetLife` _returnvalue_2 (* (`self.Lifetime`) 10.0))
      (set `/Game/Weapons/Bullets/Bullets/CondensedGasObject.Strength` (`self.Damage`) _returnvalue_2))
    (:`Is Not Valid`
      _))
  (if (not (or (>= (`self.Piercing`) 1) (not (`KismetSystemLibrary.IsValid` DamagedActor))))
    (`self.K2_DestroyActor`)))

(event `self.KillEventually`
  (`KismetSystemLibrary.Delay` (`self.Lifetime`))
  (if (not (`self.CancelDeletion`))
    (`self.CollisionBehavior` (`SceneComponent.K2_GetComponentLocation` (`self.Collider`)))
    (`self.DoBurst` (`SceneComponent.K2_GetComponentLocation` (`self.Collider`)) :!label _label)
    (`self.K2_DestroyActor`)))

(event `self.KillNow`
  (goto _label))

(fn `UserConstructionScript`
  (`parent.UserConstructionScript`))