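; Compass bullet that damages damageable actors on collision and draws colored beams pointing toward key world locations.
; Spawns timed SplineObjects from the six elemental External actors and a point above world origin to the hit location, or StartPos when InstantActivate is set.
; Elemental beams use dynamic materials whose clamped opacity scales with Damage over distance; the origin beam is plain red.
; The bullet destroys itself unless it has Piercing left.
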(event `self.CollisionBehavior`
  (params (Location :type "Vector Structure") (DamagedActor :type "Actor Object Reference") (HitComponent :type "PrimitiveComponent Object Reference"))
  (bind _spreadlocation (`self.SpreadLocation`))
  (if (`self.InstantActivate`)
    (set `self.SpreadLocation` (`self.StartPos`))
    (else
      (set `self.SpreadLocation` Location)))
  (cast `/Game/Characters/DamageSystem/BPI_Damagable` DamagedActor
    (:`then`
      (`self.DealDamage` DamagedActor))
    (:`CastFailed`
      _))
  (bind _returnvalue (`GameplayStatics.GetActorOfClass` "/Game/Rooms/Teleporters/AirExternal.AirExternal_C"))
  (bind _returnvalue_2 (`|SpawnActorFromClass` "/Game/Weapons/Bullets/Bullets/SplineObject.SplineObject_C" (`KismetMathLibrary.MakeTransform` (0.0 0.0 0.0)) "Undefined" "MultiplyWithRoot" null null))
  (bind _returnvalue_3 (+ (`self.K2_GetActorLocation` _returnvalue) (0.0 0.0 100.0)))
  (`/Game/Weapons/Bullets/Bullets/SplineObject.SetPoints` _returnvalue_2 _returnvalue_3 _spreadlocation (`self.Lifetime`))
  (bind _returnvalue_4 (`KismetMaterialLibrary.CreateDynamicMaterialInstance` "/Game/Weapons/Bullets/BulletMaterials/Cyan.Cyan"))
  (bind _output_get (set `self.Cyan1` _returnvalue_4))
  (`MaterialInstanceDynamic.SetScalarParameterValue` _output_get "Opacity" (`KismetMathLibrary.FClamp` (/ 0.1 (/ (`KismetMathLibrary.Vector_Distance` _returnvalue_3 _spreadlocation) (`self.Damage`))) 1e-06 0.1))
  (`PrimitiveComponent.SetMaterial` (`/Game/Weapons/Bullets/Bullets/SplineObject.SplineMesh1` _returnvalue_2) 0 _output_get)
  (bind _returnvalue_5 (`GameplayStatics.GetActorOfClass` "/Game/Rooms/Teleporters/DevastationExternal.DevastationExternal_C"))
  (bind _returnvalue_6 (`|SpawnActorFromClass` "/Game/Weapons/Bullets/Bullets/SplineObject.SplineObject_C" (`KismetMathLibrary.MakeTransform` (0.0 0.0 0.0)) "Undefined" "MultiplyWithRoot" null null))
  (bind _returnvalue_7 (+ (`self.K2_GetActorLocation` _returnvalue_5) (0.0 0.0 100.0)))
  (`/Game/Weapons/Bullets/Bullets/SplineObject.SetPoints` _returnvalue_6 _returnvalue_7 _spreadlocation (`self.Lifetime`))
  (bind _returnvalue_8 (`KismetMaterialLibrary.CreateDynamicMaterialInstance` "/Game/Weapons/Bullets/BulletMaterials/Purple.Purple"))
  (bind _output_get_2 (set `self.Purple1` _returnvalue_8))
  (`MaterialInstanceDynamic.SetScalarParameterValue` _output_get_2 "Opacity" (`KismetMathLibrary.FClamp` (/ 0.1 (/ (`KismetMathLibrary.Vector_Distance` _spreadlocation _returnvalue_7) (`self.Damage`))) 1e-06 0.1))
  (`PrimitiveComponent.SetMaterial` (`/Game/Weapons/Bullets/Bullets/SplineObject.SplineMesh1` _returnvalue_6) 0 _output_get_2)
  (bind _returnvalue_9 (`GameplayStatics.GetActorOfClass` "/Game/Rooms/Teleporters/EarthExternal.EarthExternal_C"))
  (bind _returnvalue_10 (`|SpawnActorFromClass` "/Game/Weapons/Bullets/Bullets/SplineObject.SplineObject_C" (`KismetMathLibrary.MakeTransform` (0.0 0.0 0.0)) "Undefined" "MultiplyWithRoot" null null))
  (bind _returnvalue_11 (+ (`self.K2_GetActorLocation` _returnvalue_9) (0.0 0.0 100.0)))
  (`/Game/Weapons/Bullets/Bullets/SplineObject.SetPoints` _returnvalue_10 _returnvalue_11 _spreadlocation (`self.Lifetime`))
  (bind _returnvalue_12 (`KismetMaterialLibrary.CreateDynamicMaterialInstance` "/Game/Weapons/Bullets/BulletMaterials/Yellow.Yellow"))
  (bind _output_get_3 (set `self.Yellow1` _returnvalue_12))
  (`MaterialInstanceDynamic.SetScalarParameterValue` _output_get_3 "Opacity" (`KismetMathLibrary.FClamp` (/ 0.1 (/ (`KismetMathLibrary.Vector_Distance` _spreadlocation _returnvalue_11) (`self.Damage`))) 1e-06 0.1))
  (`PrimitiveComponent.SetMaterial` (`/Game/Weapons/Bullets/Bullets/SplineObject.SplineMesh1` _returnvalue_10) 0 _output_get_3)
  (bind _returnvalue_13 (`GameplayStatics.GetActorOfClass` "/Game/Rooms/Teleporters/FireExternal.FireExternal_C"))
  (bind _returnvalue_14 (`|SpawnActorFromClass` "/Game/Weapons/Bullets/Bullets/SplineObject.SplineObject_C" (`KismetMathLibrary.MakeTransform` (0.0 0.0 0.0)) "Undefined" "MultiplyWithRoot" null null))
  (bind _returnvalue_15 (+ (`self.K2_GetActorLocation` _returnvalue_13) (0.0 0.0 100.0)))
  (`/Game/Weapons/Bullets/Bullets/SplineObject.SetPoints` _returnvalue_14 _returnvalue_15 _spreadlocation (`self.Lifetime`))
  (bind _returnvalue_16 (`KismetMaterialLibrary.CreateDynamicMaterialInstance` "/Game/Weapons/Bullets/BulletMaterials/Orange.Orange"))
  (bind _output_get_4 (set `self.Orange1` _returnvalue_16))
  (`MaterialInstanceDynamic.SetScalarParameterValue` _output_get_4 "Opacity" (`KismetMathLibrary.FClamp` (/ 0.1 (/ (`KismetMathLibrary.Vector_Distance` _spreadlocation _returnvalue_15) (`self.Damage`))) 1e-06 0.1))
  (`PrimitiveComponent.SetMaterial` (`/Game/Weapons/Bullets/Bullets/SplineObject.SplineMesh1` _returnvalue_14) 0 _output_get_4)
  (bind _returnvalue_17 (`GameplayStatics.GetActorOfClass` "/Game/Rooms/Teleporters/PoisonExternal.PoisonExternal_C"))
  (bind _returnvalue_18 (`|SpawnActorFromClass` "/Game/Weapons/Bullets/Bullets/SplineObject.SplineObject_C" (`KismetMathLibrary.MakeTransform` (0.0 0.0 0.0)) "Undefined" "MultiplyWithRoot" null null))
  (bind _returnvalue_19 (+ (`self.K2_GetActorLocation` _returnvalue_17) (0.0 0.0 100.0)))
  (`/Game/Weapons/Bullets/Bullets/SplineObject.SetPoints` _returnvalue_18 _returnvalue_19 _spreadlocation (`self.Lifetime`))
  (bind _returnvalue_20 (`KismetMaterialLibrary.CreateDynamicMaterialInstance` "/Game/Weapons/Bullets/BulletMaterials/Green.Green"))
  (bind _output_get_5 (set `self.Green1` _returnvalue_20))
  (`MaterialInstanceDynamic.SetScalarParameterValue` _output_get_5 "Opacity" (`KismetMathLibrary.FClamp` (/ 0.1 (/ (`KismetMathLibrary.Vector_Distance` _spreadlocation _returnvalue_19) (`self.Damage`))) 1e-06 0.1))
  (`PrimitiveComponent.SetMaterial` (`/Game/Weapons/Bullets/Bullets/SplineObject.SplineMesh1` _returnvalue_18) 0 _output_get_5)
  (bind _returnvalue_21 (`GameplayStatics.GetActorOfClass` "/Game/Rooms/Teleporters/WaterExternal.WaterExternal_C"))
  (bind _returnvalue_22 (`|SpawnActorFromClass` "/Game/Weapons/Bullets/Bullets/SplineObject.SplineObject_C" (`KismetMathLibrary.MakeTransform` (0.0 0.0 0.0)) "Undefined" "MultiplyWithRoot" null null))
  (bind _returnvalue_23 (+ (`self.K2_GetActorLocation` _returnvalue_21) (0.0 0.0 100.0)))
  (`/Game/Weapons/Bullets/Bullets/SplineObject.SetPoints` _returnvalue_22 _returnvalue_23 _spreadlocation (`self.Lifetime`))
  (bind _returnvalue_24 (`KismetMaterialLibrary.CreateDynamicMaterialInstance` "/Game/Weapons/Bullets/BulletMaterials/Blue.Blue"))
  (bind _output_get_6 (set `self.Blue1` _returnvalue_24))
  (`MaterialInstanceDynamic.SetScalarParameterValue` _output_get_6 "Opacity" (`KismetMathLibrary.FClamp` (/ 0.1 (/ (`KismetMathLibrary.Vector_Distance` _spreadlocation _returnvalue_23) (`self.Damage`))) 1e-06 0.1))
  (`PrimitiveComponent.SetMaterial` (`/Game/Weapons/Bullets/Bullets/SplineObject.SplineMesh1` _returnvalue_22) 0 _output_get_6)
  (bind _returnvalue_25 (`|SpawnActorFromClass` "/Game/Weapons/Bullets/Bullets/SplineObject.SplineObject_C" (`KismetMathLibrary.MakeTransform` (0.0 0.0 0.0)) "Undefined" "MultiplyWithRoot" null null))
  (`/Game/Weapons/Bullets/Bullets/SplineObject.SetPoints` _returnvalue_25 (0.0 0.0 100.0) _spreadlocation (`self.Lifetime`))
  (`PrimitiveComponent.SetMaterial` (`/Game/Weapons/Bullets/Bullets/SplineObject.SplineMesh1` _returnvalue_25) 0 "/Game/Weapons/Bullets/BulletMaterials/Red.Red")
  (if (not (>= (`self.Piercing`) 1))
    (`self.K2_DestroyActor`)))

(fn `UserConstructionScript`
  (`parent.UserConstructionScript`))