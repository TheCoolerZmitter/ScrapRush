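; Floating bullet that switches off gravity on what it hits and launches it upward with a Damage-scaled impulse.
; Characters get lifted and damaged, with players also receiving the shot's rescaled Lifetime through FloatBulletHit.
; Shields only take damage, while movable pickups and other damageable props are only pushed.
; Non-piercing shots are destroyed on valid hits; KillNow, or lifetime expiry unless cancelled, triggers a burst before destruction.
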(event `self.ReceiveBeginPlay`
  (`parent.ReceiveBeginPlay`)
  (`KismetSystemLibrary.DelayUntilNextTick`)
  (set `self.Lifetime` (+ (/ (`self.Lifetime`) 3.0) 1.0)))

(event `self.KillNow`
  (`self.DoBurst` (`SceneComponent.K2_GetComponentLocation` (`self.Collider`)) :!label _label)
  (`self.K2_DestroyActor`))

(event `self.KillEventually`
  (`KismetSystemLibrary.Delay` (`self.Lifetime`))
  (if (not (`self.CancelDeletion`))
    (goto _label)))

(event `self.CollisionBehavior`
  (params (Location :type "Vector Structure") (DamagedActor :type "Actor Object Reference") (HitComponent :type "PrimitiveComponent Object Reference"))
  (bind _ascharacter (cast `Character` DamagedActor)
    (:`then`
      (bind _asbp_player (cast `/Game/Characters/Player/BP_Player` DamagedActor)
        (:`then`
          (`/Game/Characters/Player/BP_Player.FloatBulletHit` _asbp_player (`self.Lifetime`)))
        (:`CastFailed`
          _))
      (bind _charactermovement (`Character.CharacterMovement` _ascharacter))
      (set `CharacterMovementComponent.GravityScale` 0.0 _charactermovement)
      (`CharacterMovementComponent.AddImpulse` _charactermovement (`KismetMathLibrary.MakeVector` 0.0 0.0 (* (`self.Damage`) 35.0)) true)
      (cast `/Game/Characters/DamageSystem/BPI_Damagable` DamagedActor :!label _label_2
        (:`then`
          (message `/Game/Characters/DamageSystem/BPI_Damagable.TakeDamage` DamagedActor (make `/Game/Characters/DamageSystem/S_DamageInfo` (`self.Damage`) (`self.DamageType`) "NewEnumerator1" false false false true (`self.Lifesteal`)))
          (`AISense_Damage.ReportDamageEvent` DamagedActor (`self.GetOwner`) 0.1))
        (:`CastFailed`
          _)))
    (:`CastFailed`
      (cast `/Game/Weapons/Bullets/Bullets/ShieldObject` DamagedActor
        (:`then`
          (goto _label_2))
        (:`CastFailed`
          (cast `/Game/Weapons/Spawners/BP_PickupBase` DamagedActor
            (:`then`
              (switch `EComponentMobility` (`SceneComponent.Mobility` HitComponent)
                (:`Movable`
                  (`PrimitiveComponent.SetEnableGravity` HitComponent false)
                  (`PrimitiveComponent.AddImpulse` HitComponent (`KismetMathLibrary.MakeVector` 0.0 0.0 (* (`self.Damage`) 200.0)) "None" false))))
            (:`CastFailed`
              (cast `/Game/Characters/DamageSystem/BPI_Damagable` DamagedActor
                (:`then`
                  (`self.SetActorScale3D` DamagedActor (* (`self.GetActorScale3D` DamagedActor) 0.999))
                  (`PrimitiveComponent.SetMassScale` HitComponent "None" 100.0)
                  (switch `EComponentMobility` (`SceneComponent.Mobility` HitComponent)
                    (:`Movable`
                      (`PrimitiveComponent.SetEnableGravity` HitComponent false)
                      (`PrimitiveComponent.AddImpulse` HitComponent (`KismetMathLibrary.MakeVector` 0.0 0.0 (* (`self.Damage`) 3000.0)) "None" false))))
                (:`CastFailed`
                  _))))))))
  (if (not (or (>= (`self.Piercing`) 1) (not (`KismetSystemLibrary.IsValid` DamagedActor))))
    (`self.K2_DestroyActor`)))

(fn `UserConstructionScript`
  (`parent.UserConstructionScript`))