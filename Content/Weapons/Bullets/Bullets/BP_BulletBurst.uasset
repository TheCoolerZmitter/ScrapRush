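; BP_BulletBurst is a bullet Blueprint that adjusts its lifetime for burst fire.
; On BeginPlay it runs the parent logic and waits one tick before checking Burst.
; When Burst is above one, it multiplies Lifetime fivefold and calls KillEventually.
; All other behavior comes from the parent, as the overlap and tick events are disabled stubs.
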(event `self.ReceiveBeginPlay`
  (`parent.ReceiveBeginPlay`)
  (`KismetSystemLibrary.DelayUntilNextTick`)
  (if (> (`self.Burst`) 1)
    (set `self.Lifetime` (* (`self.Lifetime`) 5.0))
    (`self.KillEventually`)))

(fn `UserConstructionScript`
  (`parent.UserConstructionScript`))