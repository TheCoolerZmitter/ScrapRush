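; BP_Return is a bullet that teleports its shooter to the bullet's position.
; On spawn its collider ignores pawns and the owner is teleported in place to face the bullet's rotation.
; CollisionBehavior waits for Lifetime, moves player pawn 0 to the bullet, then destroys it unless Piercing is at least one.
; KillNow, or KillEventually after Lifetime unless CancelDeletion is set, moves the owner to the collider and destroys the bullet.
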(event `self.CollisionBehavior`
  (params (Location :type "Vector Structure") (DamagedActor :type "Actor Object Reference") (HitComponent :type "PrimitiveComponent Object Reference"))
  (bind _returnvalue (`GameplayStatics.GetPlayerPawn` 0))
  (`KismetSystemLibrary.Delay` (`self.Lifetime`))
  (`self.K2_TeleportTo` _returnvalue (`self.K2_GetActorLocation`) (`self.K2_GetActorRotation` _returnvalue))
  (if (not (>= (`self.Piercing`) 1))
    (`self.K2_DestroyActor`)))

(event `self.ReceiveBeginPlay`
  (bind _returnvalue (`self.GetOwner`))
  (`parent.ReceiveBeginPlay`)
  (`PrimitiveComponent.SetCollisionResponseToChannel` (`self.Collider`) "ECC_Pawn" "ECR_Ignore")
  (`self.K2_TeleportTo` _returnvalue (`self.K2_GetActorLocation` _returnvalue) (`self.K2_GetActorRotation`)))

(event `self.KillNow`
  (bind _returnvalue (`self.GetOwner`))
  (`self.K2_TeleportTo` _returnvalue (`SceneComponent.K2_GetComponentLocation` (`self.Collider`)) (`self.K2_GetActorRotation` _returnvalue) :!label _label)
  (`self.K2_DestroyActor`))

(event `self.KillEventually`
  (`KismetSystemLibrary.Delay` (`self.Lifetime`))
  (if (not (`self.CancelDeletion`))
    (goto _label)))

(fn `UserConstructionScript`
  (`parent.UserConstructionScript`))