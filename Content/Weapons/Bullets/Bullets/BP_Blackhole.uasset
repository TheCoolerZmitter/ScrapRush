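; Black hole projectile actor that absorbs other projectiles and damages what it touches.
; On collider overlap, non-damageable BP_ProjectileBase actors are destroyed, while damageable actors receive an interrupting damage message with lifesteal and a reported damage event.
; The PhaseEnemies flag lets it pass through Characters without harming them.
; It survives impacts, with separate events to destroy it immediately or after a cancellable lifetime delay.
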(event `self.ReceiveTick`
  (params (DeltaSeconds :type "Float (single-precision)")))

(event `self.Collider.OnComponentBeginOverlap`
  (params (OverlappedComponent :type "PrimitiveComponent Object Reference") (OtherActor :type "Actor Object Reference") (OtherComp :type "PrimitiveComponent Object Reference") (OtherBodyIndex :type Integer) (bFromSweep :type Boolean) (SweepResult :type "HitResult Structure (by ref)"))
  (`self.AbsorbOrCollide` OtherActor))

(event `self.AbsorbOrCollide`
  (params (Actor :type "Actor Object Reference"))
  (cast `/Game/Characters/DamageSystem/BPI_Damagable` Actor
    (:`then`
      (if (`self.PhaseEnemies`)
        (cast `Character` Actor
          (:`CastFailed`
            _)))
      (`self.DevastationCollision` (`self.K2_GetActorLocation`) Actor :!label _label))
    (:`CastFailed`
      (bind _asbp_projectile_base (cast `/Game/Weapons/Bullets/Bullets/BP_ProjectileBase` Actor)
        (:`then`
          (`self.K2_DestroyActor` _asbp_projectile_base))
        (:`CastFailed`
          (goto _label))))))

(event `DevastationCollision`
  (params (Location :type "Vector Structure") (DamagedActor :type "Actor Object Reference"))
  (cast `/Game/Characters/DamageSystem/BPI_Damagable` DamagedActor)
  (message `/Game/Characters/DamageSystem/BPI_Damagable.TakeDamage` DamagedActor (make `/Game/Characters/DamageSystem/S_DamageInfo` (`self.Damage`) (`self.DamageType`) "NewEnumerator1" false false false true (`self.Lifesteal`)))
  (`AISense_Damage.ReportDamageEvent` DamagedActor (`self.GetOwner`) (`self.Damage`) Location))

(event `self.KillNow`
  (`self.K2_DestroyActor` :!label _label_2))

(event `self.KillEventually`
  (`KismetSystemLibrary.Delay` (`self.Lifetime`))
  (if (not (`self.CancelDeletion`))
    (goto _label_2)))

(fn `UserConstructionScript`
  (`parent.UserConstructionScript`))