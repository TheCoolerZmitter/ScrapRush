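; BP_Devastation is a projectile that absorbs another bullet and carries its payload.
; On overlap, the first BP_ProjectileBase it meets becomes InnerBullet, stopped, attached and exempt from deletion, while other valid overlaps can trigger collision.
; Collisions fire InnerBullet's collision behavior, then apply and report its own damage on damageable actors.
; KillNow or lifetime expiry also triggers and kills InnerBullet before destroying the actor.
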(event `self.ReceiveTick`
  (params (DeltaSeconds :type "Float (single-precision)")))

(event `self.Sphere.OnComponentBeginOverlap`
  (params (OverlappedComponent :type "PrimitiveComponent Object Reference") (OtherActor :type "Actor Object Reference") (OtherComp :type "PrimitiveComponent Object Reference") (OtherBodyIndex :type Integer) (bFromSweep :type Boolean) (SweepResult :type "HitResult Structure (by ref)"))
  (`self.AbsorbOrCollide` OtherActor))

(event `self.AbsorbOrCollide`
  (params (Actor :type "Actor Object Reference"))
  (cast `/Game/Characters/DamageSystem/BPI_Damagable` Actor
    (:`then`
      (if (not (`self.PhaseEnemies`))
        (`self.CollisionBehavior` (`self.K2_GetActorLocation`) Actor :!label _label)))
    (:`CastFailed`
      (bind _asbp_projectile_base (cast `/Game/Weapons/Bullets/Bullets/BP_ProjectileBase` Actor)
        (:`then`
          (`/Engine/EditorBlueprintResources/StandardMacros.IsValid` (`self.InnerBullet`)
            (:`Is Valid`
              (if (not (== (`/Game/Weapons/Bullets/Bullets/BP_ProjectileBase.Piercing` _asbp_projectile_base) 0))
                (goto _label)))
            (:`Is Not Valid`
              (`PrimitiveComponent.SetCollisionEnabled` (`/Game/Weapons/Bullets/Bullets/BP_ProjectileBase.Sphere` _asbp_projectile_base) "NoCollision")
              (bind _output_get (set `self.InnerBullet` _asbp_projectile_base))
              (set `/Game/Weapons/Bullets/Bullets/BP_ProjectileBase.Piercing` 2 _output_get)
              (set `/Game/Weapons/Bullets/Bullets/BP_ProjectileBase.DoPhysicsCalculation` true _asbp_projectile_base)
              (bind _projectilemovement (`/Game/Weapons/Bullets/Bullets/BP_ProjectileBase.ProjectileMovement` _output_get))
              (`ProjectileMovementComponent.SetVelocityInLocalSpace` _projectilemovement (0.0 0.0 0.0))
              (set `ProjectileMovementComponent.ProjectileGravityScale` 0.0 _projectilemovement)
              (set `/Game/Weapons/Bullets/Bullets/BP_ProjectileBase.CancelDeletion` true _output_get)
              (`self.K2_AttachToActor` _output_get self "None" "SnapToTarget" "KeepWorld" "SnapToTarget" true))))
        (:`CastFailed`
          (goto _label))))))

(event `self.CollisionBehavior`
  (params (Location :type "Vector Structure") (DamagedActor :type "Actor Object Reference") (HitComponent :type "PrimitiveComponent Object Reference"))
  (bind _innerbullet (`self.InnerBullet`))
  (`/Engine/EditorBlueprintResources/StandardMacros.IsValid` _innerbullet
    (:`Is Valid`
      (`self.CollisionBehavior` _innerbullet (`self.K2_GetActorLocation` _innerbullet) DamagedActor null))
    (:`Is Not Valid`
      _))
  (cast `/Game/Characters/DamageSystem/BPI_Damagable` DamagedActor)
  (message `/Game/Characters/DamageSystem/BPI_Damagable.TakeDamage` DamagedActor (make `/Game/Characters/DamageSystem/S_DamageInfo` (`self.Damage`) "NewEnumerator2" "NewEnumerator1" false false false true))
  (`AISense_Damage.ReportDamageEvent` DamagedActor (`self.GetOwner`) (`self.Damage`) Location))

(event `self.KillNow`
  (bind _innerbullet (`self.InnerBullet`))
  (`/Engine/EditorBlueprintResources/StandardMacros.IsValid` _innerbullet :!label _label_2
    (:`Is Valid`
      (`self.CollisionBehavior` _innerbullet (`self.K2_GetActorLocation` _innerbullet) null null)
      (`self.KillNow` _innerbullet)
      (`self.K2_DestroyActor`))
    (:`Is Not Valid`
      (`self.K2_DestroyActor`))))

(event `self.KillEventually`
  (`KismetSystemLibrary.Delay` (`self.Lifetime`))
  (if (not (`self.CancelDeletion`))
    (goto _label_2)))

(event `self.ProjectileMovement.OnProjectileBounce`
  (params (ImpactResult :type "HitResult Structure (by ref)") (ImpactVelocity :type "Vector Structure (by ref)"))
  (`self.CollisionBehavior` ImpactResult_ImpactPoint))

(fn `UserConstructionScript`
  (`parent.UserConstructionScript`))