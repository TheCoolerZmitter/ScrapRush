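; BP_Force is a bullet actor that fires a radial force impulse at the collision location, then destroys itself unless it has piercing.
; If deletion is not cancelled when its lifetime expires, it fires the impulse at its current position and is destroyed.
; SetStats sets projectile velocity and stores modifiers, squaring several stats, doubling piercing, scaling impulse strength by squared damage and enabling physics calculation only below a speed threshold.
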(event `self.KillEventually`
  (`KismetSystemLibrary.Delay` (`self.Lifetime`))
  (if (not (`self.CancelDeletion`))
    (`self.CollisionBehavior` (`self.K2_GetActorLocation`))
    (`self.K2_DestroyActor`)))

(event `self.CollisionBehavior`
  (params (Location :type "Vector Structure") (DamagedActor :type "Actor Object Reference") (HitComponent :type "PrimitiveComponent Object Reference"))
  (`SceneComponent.K2_SetWorldLocation` (`self.RadialForce`) Location false false)
  (`RadialForceComponent.FireImpulse` (`self.RadialForce`))
  (if (not (>= (`self.Piercing`) 1))
    (`self.K2_DestroyActor`)))

(event `self.SetStats`
  (params (Direction :type "Vector Structure") (Velocity :type "Float (double-precision)") (Lifetime :type "Float (double-precision)") (Damage :type "Float (double-precision)") (Piercing :type Integer) (Statis :type Boolean) (InstantActivate :type Boolean) (Gravity :type "Float (double-precision)") (Bounce :type Boolean) (PhaseEnemies :type Boolean) (Homing :type "Float (double-precision)") (Radius :type "Float (double-precision)") (AttackTarget :type "Actor Object Reference") (Knockback :type "Float (double-precision)"))
  (bind _output_get (set `self.Direction` (* Direction (* Velocity (`self.Velocity`)))))
  (bind _output_get_2 (set `MovementComponent.Velocity` _output_get (`self.ProjectileMovement`)))
  (set `self.DoPhysicsCalculation` (< (`KismetMathLibrary.VSize` _output_get_2) 6000.0))
  (set `self.Lifetime` (* (`self.Lifetime`) Lifetime))
  (set `self.Damage` (* (`self.Damage`) Damage))
  (set `RadialForceComponent.ImpulseStrength` (* (`RadialForceComponent.ImpulseStrength` (`self.RadialForce`)) (`self.Damage`)) (`self.RadialForce`))
  (set `self.Piercing` (+ (`self.Piercing`) Piercing))
  (set `self.Statis` Statis)
  (set `self.InstantActivate` InstantActivate)
  (set `self.Gravity` Gravity)
  (set `self.Bounce` Bounce)
  (set `self.PhaseEnemies` PhaseEnemies)
  (set `self.Homing` Homing)
  (set `self.Radius` (* (`self.Radius`) Radius)))

(fn `UserConstructionScript`
  (`parent.UserConstructionScript`))