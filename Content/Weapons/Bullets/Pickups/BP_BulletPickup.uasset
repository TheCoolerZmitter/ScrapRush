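; BP_BulletPickup is an interactable pickup that puts its bullet type into the player's bullet inventory.
; On Interact, it fills the first unset or placeholder slot within a fixed slot range, then destroys itself.
; When the inventory is full, it looks up the first slot's bullet in DT_Bullet, spawns that row's class in front of the player, and overwrites the slot with its own type.
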(event `/Game/Weapons/Spawners/BPI_Interact.Interact`
  (params (`Character Picking Up` :type "Actor Object Reference"))
  (set `self.InventoryHadRoom` false)
  (bind _asbp_player (cast `/Game/Characters/Player/BP_Player` `Character Picking Up`))
  (for _index (range 33)
    (bind _bulletinventory (`/Game/Characters/Player/BP_Player.BulletInventory` _asbp_player))
    (if (`KismetArrayLibrary.Array_IsValidIndex` _bulletinventory _index)
      (if (`|EnumEquality` (`|GetArrayItem` _bulletinventory _index) "NewEnumerator21")
        (`KismetArrayLibrary.Array_Set` _bulletinventory _index (`self.BulletType`) true)
        (set `self.InventoryHadRoom` true :!label _label)
        (break))
      (else
        (`KismetArrayLibrary.Array_Set` _bulletinventory _index (`self.BulletType`) true)
        (goto _label))))
  (if (not (`self.InventoryHadRoom`))
    (bind _returnvalue (`|GetDataTableRow` "/Game/Characters/Player/Inventory/DataStructures/DT_Bullet.DT_Bullet" (`KismetStringLibrary.Conv_StringToName` (`|GetEnumeratorNameAsString` (`|GetArrayItem` _bulletinventory))))
      (:`then`
        (`|SpawnActorFromClass` (`.Class_9_40B038004B22AF262E05A0964CEA8F14` (break `/Game/Characters/Player/Inventory/DataStructures/Struct_E_Bullet` _returnvalue)) (`KismetMathLibrary.MakeTransform` (+ (`self.K2_GetActorLocation` `Character Picking Up`) (* (`self.GetActorForwardVector` `Character Picking Up`) (60.0 60.0 0.0))) (`self.K2_GetActorRotation` `Character Picking Up`)) "AdjustIfPossibleButAlwaysSpawn" "MultiplyWithRoot" null null)
        (`KismetArrayLibrary.Array_Set` _bulletinventory 0 (`self.BulletType`) true))))
  (`self.K2_DestroyActor`))

(fn `UserConstructionScript`
  (`parent.UserConstructionScript`))