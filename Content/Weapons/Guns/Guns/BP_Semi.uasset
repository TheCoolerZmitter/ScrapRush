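; Burst-fire gun that shoots projectiles chosen from a bullet inventory, with modifier stats, crits and twin shots.
; Shoot snapshots stats and aims at a look direction or target, then CooldownRecovery keeps the burst open for the first quarter of the cooldown.
; Each FireBullet calls QuadFire, which restores the snapshot with extra spread, re-aims and replays from the saved bullet index, advancing to the next bullet once the burst ends.
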(event `self.PlayAnimation`
  (`SkeletalMeshComponent.PlayAnimation` (`self.SkeletalMesh`) "/Game/Weapons/MilitaryWeapSilver/Weapons/Animations/Fire_GrenadeLauncher_W.Fire_GrenadeLauncher_W" false))

(event `self.CooldownRecovery`
  (params (CooldownTime :type "Float (double-precision)"))
  (bind _returnvalue (/ CooldownTime 4.0))
  (set `self.CanShoot` false)
  (`KismetSystemLibrary.Delay` _returnvalue)
  (set `self.KeepFiring` false)
  (`KismetSystemLibrary.Delay` (* _returnvalue 3.0))
  (`self.ResetAfterModifiers`)
  (set `self.CanShoot` true))

(event `QuadFire`
  (bind _returnvalue (`self.K2_GetActorLocation`))
  (bind _returnvalue_2 (`self.K2_GetActorRotation`))
  (if (`self.KeepFiring`)
    (`self.TempReset`)
    (`KismetSystemLibrary.Delay` (/ (`self.CooldownToUse`) (`self.SubCooldown`)))
    (set `self.CurrentBulletIndex` (`self.BulletIndexSaved`))
    (`/Engine/EditorBlueprintResources/StandardMacros.IsValid` (`self.Target`)
      (:`Is Valid`
        (set `self.HitLocation` (+ (`self.K2_GetActorLocation` (`self.Target`)) (0.0 0.0 50.0))))
      (:`Is Not Valid`
        (set `self.HitLocation` (`KismetMathLibrary.GreaterGreater_VectorRotator` (`KismetMathLibrary.GreaterGreater_VectorRotator` (+ (`self.HitLocation`) (- (`self.PositionLastBullet`) _returnvalue)) (`KismetMathLibrary.InverseTransformRotation` (`KismetMathLibrary.MakeTransform` (0.0 0.0 0.0) (`self.RotationLastBullet`)))) _returnvalue_2))
        (set `self.RotationLastBullet` _returnvalue_2)
        (set `self.PositionLastBullet` _returnvalue)))
    (`self.ResetAfterModifiers`)
    (`/Game/Weapons/Guns/BPI_Weapons.SelectBullet` 0)
    (else
      (`KismetSystemLibrary.DelayUntilNextTick`)
      (`/Game/Weapons/Guns/BPI_Weapons.NextBullet`))))

(event `TempStore`
  (set `self.TempCooldown` (`self.Cooldown`))
  (set `self.TempSpeed` (`self.BulletVelocity`))
  (set `self.TempDamage` (`self.Damage`))
  (set `self.TempLifetime` (`self.Lifetime`))
  (set `self.TempGravity` (`self.Gravity`))
  (set `self.TempHoming` (`self.Homing`))
  (set `self.TempRadius` (`self.Radius`))
  (set `self.TempKnockback` (`self.Knockback`))
  (set `self.TempRandom` (`self.Random`))
  (set `self.TempDamageType` (`self.DamageType`))
  (set `self.TempAcceleration` (`self.Acceleration`))
  (set `self.TempBoomerang` (`self.Boomerang`))
  (set `self.TempSpiral` (`self.Spiral`))
  (set `self.TempCrit` (`self.CritChance`))
  (set `self.TempBlink` (`self.Blink`))
  (set `self.TempMultiCollision` (`self.MultiCollision`))
  (set `self.TempLifesteal` (`self.Lifesteal`))
  (set `self.TempTwin` (`self.Twin`)))

(event `TempReset`
  (set `self.Cooldown` (`self.TempCooldown`))
  (set `self.BulletVelocity` (`self.TempSpeed`))
  (set `self.Damage` (`self.TempDamage`))
  (set `self.Lifetime` (`self.TempLifetime`))
  (set `self.Gravity` (`self.TempGravity`))
  (set `self.Homing` (`self.TempHoming`))
  (set `self.Radius` (`self.TempRadius`))
  (set `self.Knockback` (`self.TempKnockback`))
  (set `self.Random` (+ (`self.TempRandom`) 10.0))
  (set `self.DamageType` (`self.TempDamageType`))
  (set `self.Acceleration` (`self.TempAcceleration`))
  (set `self.Boomerang` (`self.TempBoomerang`))
  (set `self.Spiral` (`self.TempSpiral`))
  (set `self.CritChance` (`self.TempCrit`))
  (set `self.Blink` (`self.TempBlink`))
  (set `self.MultiCollision` (`self.TempMultiCollision`))
  (set `self.Lifesteal` (`self.TempLifesteal`))
  (set `self.Twin` (`self.TempTwin`)))

(fn `FireBullet`
  (params (BulletBP :type "Actor Class Reference"))
  (returns (Fired :type Boolean))
  (bind _statis (`self.Statis`))
  (bind _critchance (`self.CritChance`))
  (bind _radius (`self.Radius`))
  (bind _returnvalue (`SceneComponent.GetSocketLocation` (`self.SkeletalMesh`) "barrel"))
  (if (> (`self.Twin`) 0)
    (bind _fired (`self.DoTwin` BulletBP))
    (return _fired)
    (else
      (if (== _critchance 0)
        _
        (elif (> _critchance (`KismetMathLibrary.RandomInteger` 11))
          (set `self.CritBool` true)
          (set `self.Damage` (* (`self.Damage`) 2.5))))
      (if (not (== (`self.Random`) 0.0))
        (`self.RandomHitLocation`))
      (bind _returnvalue_2 (`|SpawnActorFromClass` BulletBP (`KismetMathLibrary.MakeTransform` _returnvalue (`self.K2_GetActorRotation` (`self.GetOwner`)) (`KismetMathLibrary.MakeVector` _radius _radius _radius)) "Undefined" "MultiplyWithRoot" (`self.GetOwner`) null))
      (bind _asbp_projectile_base (cast `/Game/Weapons/Bullets/Bullets/BP_ProjectileBase` _returnvalue_2))
      (`/Game/Weapons/Bullets/Bullets/BP_ProjectileBase.SetStats` _asbp_projectile_base (`KismetMathLibrary.Normal` (- (`self.HitLocation`) _returnvalue) 0.0) (`self.BulletVelocity`) (`self.Lifetime`) (* (`/Game/Characters/DamageSystem/BPC_DamageSystem.Strength` (`self.BPC Damage System`)) (`self.Damage`)) (`self.Piercing`) _statis (`self.InstantActivate`) (`self.Gravity`) (`self.Bounce`) (`self.PhaseEnemies`) (`self.Homing`) (`self.Radius`) (`self.AttackTarget`) (`self.Knockback`) (`self.DamageType`) (`self.Acceleration`) (`self.Boomerang`) (`self.Spiral`) (`self.Blink`) (`self.MultiCollision`) (`self.Lifesteal`))
      (if _statis
        (`KismetArrayLibrary.Array_Add` (`self.BulletsInStatis`) _asbp_projectile_base))
      (set `self.CooldownToUse` (* (`self.Cooldown`) (`/Game/Weapons/Bullets/Bullets/BP_ProjectileBase.Cooldown` _asbp_projectile_base)))
      (`self.QuadFire`)
      (if (`self.CritBool`)
        (set `self.CritBool` false)
        (set `self.Damage` (/ (`self.Damage`) 2.5)))
      (return true))))

(fn `Shoot`
  (params (LookingActor :type "SceneComponent Object Reference") (Target :type "Actor Object Reference"))
  (returns (Fired :type Boolean))
  (if (`self.CanShoot`)
    (`self.TempStore`)
    (set `self.BulletIndexSaved` (`self.CurrentBulletIndex`))
    (set `self.PositionLastBullet` (`self.K2_GetActorLocation`))
    (set `self.RotationLastBullet` (`self.K2_GetActorRotation`))
    (`/Engine/EditorBlueprintResources/StandardMacros.IsValid` LookingActor
      (:`Is Valid`
        (set `self.HitLocation` (+ (`SceneComponent.K2_GetComponentLocation` LookingActor) (* (`KismetMathLibrary.GetForwardVector` (`SceneComponent.GetSocketRotation` LookingActor "None")) 20000.0))))
      (:`Is Not Valid`
        (set `self.HitLocation` (+ (`self.K2_GetActorLocation` Target) (0.0 0.0 50.0)))
        (set `self.Target` Target)))
    (set `self.KeepFiring` true)
    (bind _fired (`/Game/Weapons/Guns/BPI_Weapons.SelectBullet` 0))
    (if _fired
      (`self.PlayAnimation`)
      (`self.CooldownRecovery` (`self.CooldownToUse`))
      (return true)
      (else
        (`self.CooldownRecovery` 0.5)
        (return false)))
    (else
      (return false))))

(fn `UnStasisFunc`
  (`parent.UnStasisFunc`)
  (set `self.CurrentBulletIndex` 0))

(fn `UserConstructionScript`
  (`parent.UserConstructionScript`))