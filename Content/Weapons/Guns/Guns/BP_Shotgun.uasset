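; Shotgun weapon that plays a firing animation and shoots a three-projectile fan: one at the hit location, two angled 15 degrees either side.
; FireBullet hands off to DoTwin when Twin is set; otherwise it rolls a temporary crit damage boost and spawns projectiles with the gun's stats.
; Optional random spread temporarily widens for the side shots.
; Cooldown scales by the last projectile's value, and Statis shots are stored in BulletsInStatis.
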(event `self.PlayAnimation`
  (`SkeletalMeshComponent.PlayAnimation` (`self.SkeletalMesh`) "/Game/Weapons/MilitaryWeapSilver/Weapons/Animations/Fire_Shotgun_W.Fire_Shotgun_W" false))

(fn `FireBullet`
  (params (BulletBP :type "Actor Class Reference"))
  (returns (Fired :type Boolean))
  (bind _returnvalue (`self.K2_GetActorLocation`))
  (bind _returnvalue_2 (`self.K2_GetActorLocation`))
  (bind _critchance (`self.CritChance`))
  (bind _bulletsinstatis (`self.BulletsInStatis`))
  (bind _radius (`self.Radius`))
  (bind _statis (`self.Statis`))
  (bind _skeletalmesh (`self.SkeletalMesh`))
  (bind _random (`self.Random`))
  (bind _radius_2 (`self.Radius`))
  (bind _random_2 (`self.Random`))
  (bind _radius_3 (`self.Radius`))
  (bind _skeletalmesh_2 (`self.SkeletalMesh`))
  (bind _returnvalue_3 (`SceneComponent.GetSocketLocation` (`self.SkeletalMesh`) "barrel"))
  (bind _returnvalue_4 (+ (`SceneComponent.GetSocketLocation` _skeletalmesh_2 "barrel") (* (`SceneComponent.GetForwardVector` _skeletalmesh_2) 50.0) (* (`SceneComponent.GetRightVector` _skeletalmesh_2) -20.0)))
  (bind _returnvalue_5 (+ (`SceneComponent.GetSocketLocation` _skeletalmesh "barrel") (* (`SceneComponent.GetForwardVector` _skeletalmesh) -50.0) (* (`SceneComponent.GetRightVector` _skeletalmesh) -20.0)))
  (if (> (`self.Twin`) 0)
    (bind _fired (`self.DoTwin` BulletBP))
    (return _fired)
    (else
      (if (== _critchance 0)
        _
        (elif (> _critchance (`KismetMathLibrary.RandomInteger` 11))
          (set `self.CritBool` true)
          (set `self.Damage` (* (`self.Damage`) 2.5))))
      (if (not (== (`self.Random`) 0.0))
        (`self.RandomHitLocation`))
      (bind _returnvalue_6 (`|SpawnActorFromClass` BulletBP (`KismetMathLibrary.MakeTransform` _returnvalue_3 (`self.K2_GetActorRotation` (`self.GetOwner`)) (`KismetMathLibrary.MakeVector` _radius_2 _radius_2 _radius_2)) "Undefined" "MultiplyWithRoot" (`self.GetOwner`) null))
      (bind _asbp_projectile_base (cast `/Game/Weapons/Bullets/Bullets/BP_ProjectileBase` _returnvalue_6))
      (`/Game/Weapons/Bullets/Bullets/BP_ProjectileBase.SetStats` _asbp_projectile_base (`KismetMathLibrary.Normal` (- (`self.HitLocation`) _returnvalue_3) 0.0) (`self.BulletVelocity`) (`self.Lifetime`) (* (`/Game/Characters/DamageSystem/BPC_DamageSystem.Strength` (`self.BPC Damage System`)) (`self.Damage`)) (`self.Piercing`) _statis (`self.InstantActivate`) (`self.Gravity`) (`self.Bounce`) (`self.PhaseEnemies`) (`self.Homing`) (`self.Radius`) (`self.AttackTarget`) (`self.Knockback`) (`self.DamageType`) (`self.Acceleration`) (`self.Boomerang`) (`self.Spiral`) (`self.Blink`) (`self.MultiCollision`) (`self.Lifesteal`))
      (if (not (== _random 0.0))
        (set `self.Random` (+ 10.0 _random))
        (`self.RandomHitLocation`))
      (bind _returnvalue_7 (`|SpawnActorFromClass` (`local.BulletBP`) (`KismetMathLibrary.MakeTransform` _returnvalue_5 (`self.K2_GetActorRotation` (`self.GetOwner`)) (`KismetMathLibrary.MakeVector` _radius_3 _radius_3 _radius_3)) "Undefined" "MultiplyWithRoot" (`self.GetOwner`) null))
      (bind _asbp_projectile_base_2 (cast `/Game/Weapons/Bullets/Bullets/BP_ProjectileBase` _returnvalue_7))
      (`/Game/Weapons/Bullets/Bullets/BP_ProjectileBase.SetStats` _asbp_projectile_base_2 (`KismetMathLibrary.Normal` (- _returnvalue_5 (+ (`KismetMathLibrary.RotateAngleAxis` (* (`KismetMathLibrary.Normal` (- (`self.HitLocation`) _returnvalue) 0.0) -20000.0) 15.0 (0.0 0.0 1.0)) _returnvalue)) 0.0) (`self.BulletVelocity`) (`self.Lifetime`) (* (`/Game/Characters/DamageSystem/BPC_DamageSystem.Strength` (`self.BPC Damage System`)) (`self.Damage`)) (`self.Piercing`) _statis (`self.InstantActivate`) (`self.Gravity`) (`self.Bounce`) (`self.PhaseEnemies`) (`self.Homing`) (`self.Radius`) (`self.AttackTarget`) (`self.Knockback`) (`self.DamageType`) (`self.Acceleration`) (`self.Boomerang`) (`self.Spiral`) (`self.Blink`) (`self.MultiCollision`) (`self.Lifesteal`))
      (if (not (== _random_2 0.0))
        (`self.RandomHitLocation`)
        (set `self.Random` (+ _random_2 -10.0)))
      (bind _returnvalue_8 (`|SpawnActorFromClass` (`local.BulletBP`) (`KismetMathLibrary.MakeTransform` _returnvalue_4 (`self.K2_GetActorRotation` (`self.GetOwner`)) (`KismetMathLibrary.MakeVector` _radius _radius _radius)) "Undefined" "MultiplyWithRoot" (`self.GetOwner`) null))
      (bind _asbp_projectile_base_3 (cast `/Game/Weapons/Bullets/Bullets/BP_ProjectileBase` _returnvalue_8))
      (`/Game/Weapons/Bullets/Bullets/BP_ProjectileBase.SetStats` _asbp_projectile_base_3 (`KismetMathLibrary.Normal` (- _returnvalue_4 (+ (`KismetMathLibrary.RotateAngleAxis` (* (`KismetMathLibrary.Normal` (- (`self.HitLocation`) _returnvalue_2) 0.0) -20000.0) -15.0 (0.0 0.0 1.0)) _returnvalue_2)) 0.0) (`self.BulletVelocity`) (`self.Lifetime`) (* (`/Game/Characters/DamageSystem/BPC_DamageSystem.Strength` (`self.BPC Damage System`)) (`self.Damage`)) (`self.Piercing`) _statis (`self.InstantActivate`) (`self.Gravity`) (`self.Bounce`) (`self.PhaseEnemies`) (`self.Homing`) (`self.Radius`) (`self.AttackTarget`) (`self.Knockback`) (`self.DamageType`) (`self.Acceleration`) (`self.Boomerang`) (`self.Spiral`) (`self.Blink`) (`self.MultiCollision`) (`self.Lifesteal`))
      (set `self.CooldownToUse` (* (`self.Cooldown`) (`/Game/Weapons/Bullets/Bullets/BP_ProjectileBase.Cooldown` _asbp_projectile_base_3)))
      (if _statis
        (`KismetArrayLibrary.Array_Add` _bulletsinstatis _asbp_projectile_base_3)
        (`KismetArrayLibrary.Array_Add` _bulletsinstatis _asbp_projectile_base_2)
        (`KismetArrayLibrary.Array_Add` _bulletsinstatis _asbp_projectile_base))
      (if (`self.CritBool`)
        (set `self.CritBool` false)
        (set `self.Damage` (/ (`self.Damage`) 2.5)))
      (return true))))

(fn `UserConstructionScript`
  (`parent.UserConstructionScript`))