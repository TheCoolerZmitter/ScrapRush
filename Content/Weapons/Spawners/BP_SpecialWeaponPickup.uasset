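; Weapon pickup spawner that produces a special weapon with a randomly chosen, hand-authored inventory preset.
; SpawnPickup calls SpawnWeapon, runs Special on the result, then destroys the spawner actor.
; Special picks one of sixteen presets at random and writes its enum items into the spawned weapon's Inventory slots.
; Two presets also append an item at the NumSlots index and increase the slot count by one.
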(event `self.SpawnPickup`
  (`self.SpawnWeapon`)
  (`self.Special`)
  (`self.K2_DestroyActor`))

(fn `Special`
  (bind _weaponspawned (`self.WeaponSpawned`))
  (bind _inventory (`/Game/Weapons/Guns/Pickups/BP_WeaponPickup.Inventory` _weaponspawned))
  (bind _numslots (`/Game/Weapons/Guns/Pickups/BP_WeaponPickup.NumSlots` _weaponspawned))
  (switch `int` (`KismetMathLibrary.RandomInteger` 16)
    (:`0`
      (`KismetArrayLibrary.Array_Set` _inventory 0 "NewEnumerator16")
      (`KismetArrayLibrary.Array_Set` _inventory 1 "NewEnumerator33")
      (`KismetArrayLibrary.Array_Set` _inventory 2 "NewEnumerator18")
      (`KismetArrayLibrary.Array_Set` _inventory 3 "NewEnumerator13"))
    (:`1`
      (`KismetArrayLibrary.Array_Set` _inventory 0 "NewEnumerator51")
      (`KismetArrayLibrary.Array_Set` _inventory 1 "NewEnumerator29")
      (`KismetArrayLibrary.Array_Set` _inventory 2 "NewEnumerator9"))
    (:`2`
      (`KismetArrayLibrary.Array_Set` _inventory 0 "NewEnumerator23")
      (`KismetArrayLibrary.Array_Set` _inventory 1 "NewEnumerator8")
      (`KismetArrayLibrary.Array_Set` _inventory 2 "NewEnumerator1"))
    (:`3`
      (`KismetArrayLibrary.Array_Set` _inventory 0 "NewEnumerator44")
      (`KismetArrayLibrary.Array_Set` _inventory 1 "NewEnumerator11"))
    (:`4`
      (`KismetArrayLibrary.Array_Set` _inventory 0 "NewEnumerator44")
      (`KismetArrayLibrary.Array_Set` _inventory 1 "NewEnumerator52")
      (`KismetArrayLibrary.Array_Set` _inventory 2 "NewEnumerator9"))
    (:`5`
      (`KismetArrayLibrary.Array_Set` _inventory 0 "NewEnumerator23")
      (`KismetArrayLibrary.Array_Set` _inventory 1 "NewEnumerator20")
      (`KismetArrayLibrary.Array_Set` _inventory 2 "NewEnumerator32")
      (`KismetArrayLibrary.Array_Set` _inventory 3 "NewEnumerator112"))
    (:`6`
      (`KismetArrayLibrary.Array_Set` _inventory 0 "NewEnumerator26")
      (`KismetArrayLibrary.Array_Set` _inventory 1 "NewEnumerator1")
      (`KismetArrayLibrary.Array_Set` _inventory 2 "NewEnumerator1")
      (`KismetArrayLibrary.Array_Set` _inventory 3 "NewEnumerator1")
      (`KismetArrayLibrary.Array_Set` _inventory _numslots "NewEnumerator27" true)
      (set `/Game/Weapons/Guns/Pickups/BP_WeaponPickup.NumSlots` (+ _numslots 1) _weaponspawned :!label _label))
    (:`7`
      (`KismetArrayLibrary.Array_Set` _inventory 0 "NewEnumerator30")
      (`KismetArrayLibrary.Array_Set` _inventory 1 "NewEnumerator44")
      (`KismetArrayLibrary.Array_Set` _inventory 2 "NewEnumerator4"))
    (:`8`
      (`KismetArrayLibrary.Array_Set` _inventory 0 "NewEnumerator26")
      (`KismetArrayLibrary.Array_Set` _inventory 1 "NewEnumerator31")
      (`KismetArrayLibrary.Array_Set` _inventory 2 "NewEnumerator31")
      (`KismetArrayLibrary.Array_Set` _inventory 3 "NewEnumerator57")
      (`KismetArrayLibrary.Array_Set` _inventory _numslots "NewEnumerator27" true)
      (goto _label))
    (:`9`
      (`KismetArrayLibrary.Array_Set` _inventory 0 "NewEnumerator103")
      (`KismetArrayLibrary.Array_Set` _inventory 1 "NewEnumerator46"))
    (:`10`
      (`KismetArrayLibrary.Array_Set` _inventory 0 "NewEnumerator63")
      (`KismetArrayLibrary.Array_Set` _inventory 1 "NewEnumerator22")
      (`KismetArrayLibrary.Array_Set` _inventory 2 "NewEnumerator6"))
    (:`11`
      (`KismetArrayLibrary.Array_Set` _inventory 0 "NewEnumerator23")
      (`KismetArrayLibrary.Array_Set` _inventory 1 "NewEnumerator59")
      (`KismetArrayLibrary.Array_Set` _inventory 2 "NewEnumerator112"))
    (:`12`
      (`KismetArrayLibrary.Array_Set` _inventory 0 "NewEnumerator24")
      (`KismetArrayLibrary.Array_Set` _inventory 1 "NewEnumerator65"))
    (:`13`
      (`KismetArrayLibrary.Array_Set` _inventory 0 "NewEnumerator68")
      (`KismetArrayLibrary.Array_Set` _inventory 1 "NewEnumerator74")
      (`KismetArrayLibrary.Array_Set` _inventory 2 "NewEnumerator91")
      (`KismetArrayLibrary.Array_Set` _inventory 3 "NewEnumerator77")
      (`KismetArrayLibrary.Array_Set` _inventory 4 "NewEnumerator73"))
    (:`14`
      (`KismetArrayLibrary.Array_Set` _inventory 0 "NewEnumerator41")
      (`KismetArrayLibrary.Array_Set` _inventory 1 "NewEnumerator18")
      (`KismetArrayLibrary.Array_Set` _inventory 2 "NewEnumerator43"))
    (:`15`
      (`KismetArrayLibrary.Array_Set` _inventory 0 "NewEnumerator44")
      (`KismetArrayLibrary.Array_Set` _inventory 1 "NewEnumerator49"))))

(fn `UserConstructionScript`
  (`parent.UserConstructionScript`))