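; Random weapon spawner that, on SpawnPickup, places one of six weapon pickups at its transform, then destroys itself.
; An optional FailureChance roll out of ten can cancel the spawn.
; SpawnWeapon randomizes inventory slot count and jitters cooldown, bullet velocity, damage and lifetime.
; FillBullet inserts a bullet entry at the last slot index, fixed for rocket launchers, skipped for knives, otherwise occasionally a rarer type; the SemiPickup branch is disconnected.
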(event `self.SpawnPickup`
  (`self.SpawnWeapon`)
  (`self.FillBullet`)
  (`self.K2_DestroyActor`))

(fn `FillBullet`
  (bind _weaponspawned (`self.WeaponSpawned`))
  (bind _inventory (`/Game/Weapons/Guns/Pickups/BP_WeaponPickup.Inventory` (`self.WeaponSpawned`)))
  (bind _returnvalue (- (`/Game/Weapons/Guns/Pickups/BP_WeaponPickup.NumSlots` _weaponspawned) 1))
  (if (`KismetSystemLibrary.IsValid` _weaponspawned)
    (cast `/Game/Weapons/Guns/Pickups/BP_Knife_Pickup` _weaponspawned
      (:`CastFailed`
        (cast `/Game/Weapons/Guns/Pickups/BP_RocketLauncherPickup` _weaponspawned
          (:`then`
            (`KismetArrayLibrary.Array_Insert` _inventory "NewEnumerator13" _returnvalue))
          (:`CastFailed`
            (if (> (`KismetMathLibrary.RandomFloat`) 0.85)
              (`KismetArrayLibrary.Array_Insert` _inventory "NewEnumerator3" _returnvalue)
              (else
                (`KismetArrayLibrary.Array_Insert` _inventory "NewEnumerator0" _returnvalue)))))))))

(fn `SpawnWeapon`
  (bind (_returnvalue_location _returnvalue_rotation) (`KismetMathLibrary.BreakTransform` (`self.GetTransform`)))
  (bind _weaponspawned (`self.WeaponSpawned`))
  (bind _weaponspawned_2 (`self.WeaponSpawned`))
  (bind _weaponspawned_3 (`self.WeaponSpawned`))
  (bind _weaponspawned_4 (`self.WeaponSpawned`))
  (bind _failurechance (`self.FailureChance`))
  (if (> _failurechance 0)
    (if (>= (`KismetMathLibrary.RandomInteger` 10) _failurechance)
      (switch `int` (`KismetMathLibrary.RandomInteger` 6) :!label _label
        (:`0`
          (bind _returnvalue (`|SpawnActorFromClass` "/Game/Weapons/Guns/Pickups/BP_PistolPickup.BP_PistolPickup_C" (`KismetMathLibrary.MakeTransform` _returnvalue_location _returnvalue_rotation) "Undefined" "MultiplyWithRoot" null null))
          (set `self.WeaponSpawned` _returnvalue))
        (:`1`
          (bind _returnvalue_2 (`|SpawnActorFromClass` "/Game/Weapons/Guns/Pickups/BP_ShotgunPickup.BP_ShotgunPickup_C" (`KismetMathLibrary.MakeTransform` _returnvalue_location _returnvalue_rotation) "Undefined" "MultiplyWithRoot" null null))
          (set `self.WeaponSpawned` _returnvalue_2))
        (:`2`
          (bind _returnvalue_3 (`|SpawnActorFromClass` "/Game/Weapons/Guns/Pickups/BP_SniperPickup.BP_SniperPickup_C" (`KismetMathLibrary.MakeTransform` _returnvalue_location _returnvalue_rotation) "Undefined" "MultiplyWithRoot" null null))
          (set `self.WeaponSpawned` _returnvalue_3))
        (:`3`
          (bind _returnvalue_4 (`|SpawnActorFromClass` "/Game/Weapons/Guns/Pickups/BP_Knife_Pickup.BP_Knife_Pickup_C" (`KismetMathLibrary.MakeTransform` _returnvalue_location _returnvalue_rotation) "Undefined" "MultiplyWithRoot" null null))
          (bind _output_get (set `self.WeaponSpawned` _returnvalue_4))
          (`KismetArrayLibrary.Array_Insert` (`/Game/Weapons/Guns/Pickups/BP_WeaponPickup.Inventory` _output_get) "NewEnumerator21"))
        (:`4`
          (bind _returnvalue_5 (`|SpawnActorFromClass` "/Game/Weapons/Guns/Pickups/BP_ARPickup.BP_ARPickup_C" (`KismetMathLibrary.MakeTransform` _returnvalue_location _returnvalue_rotation) "Undefined" "MultiplyWithRoot" null null))
          (set `self.WeaponSpawned` _returnvalue_5))
        (:`5`
          (bind _returnvalue_6 (`|SpawnActorFromClass` "/Game/Weapons/Guns/Pickups/BP_RocketLauncherPickup.BP_RocketLauncherPickup_C" (`KismetMathLibrary.MakeTransform` _returnvalue_location _returnvalue_rotation) "Undefined" "MultiplyWithRoot" null null))
          (bind _output_get_2 (set `self.WeaponSpawned` _returnvalue_6))
          (`KismetArrayLibrary.Array_Insert` (`/Game/Weapons/Guns/Pickups/BP_WeaponPickup.Inventory` _output_get_2) "NewEnumerator13")))
      (bind _output_get_3 (set `/Game/Weapons/Guns/Pickups/BP_WeaponPickup.NumSlots` (+ 5 (`KismetMathLibrary.RandomInteger` 10)) (`self.WeaponSpawned`)))
      (for _index (range _output_get_3)
        (`KismetArrayLibrary.Array_Insert` (`/Game/Weapons/Guns/Pickups/BP_WeaponPickup.Inventory` (`self.WeaponSpawned`)) "NewEnumerator21" _index))
      (set `/Game/Weapons/Guns/Pickups/BP_WeaponPickup.Cooldown` (+ (`/Game/Weapons/Guns/Pickups/BP_WeaponPickup.Cooldown` _weaponspawned_3) (- (* (`KismetMathLibrary.RandomFloat`) 0.2) 0.07)) _weaponspawned_3)
      (set `/Game/Weapons/Guns/Pickups/BP_WeaponPickup.BulletVelocity` (+ (`/Game/Weapons/Guns/Pickups/BP_WeaponPickup.BulletVelocity` _weaponspawned) (- (* (`KismetMathLibrary.RandomFloat`) 2.0) 1.0)) _weaponspawned)
      (set `/Game/Weapons/Guns/Pickups/BP_WeaponPickup.Damage` (+ (`/Game/Weapons/Guns/Pickups/BP_WeaponPickup.Damage` _weaponspawned_2) (- (`KismetMathLibrary.RandomFloat`) 0.5)) _weaponspawned_2)
      (set `/Game/Weapons/Guns/Pickups/BP_WeaponPickup.Lifetime` (+ (`/Game/Weapons/Guns/Pickups/BP_WeaponPickup.Lifetime` _weaponspawned_4) (- (* (`KismetMathLibrary.RandomFloat`) 0.2) 0.1)) _weaponspawned_4)
      (else
        (`self.K2_DestroyActor`)))
    (else
      (goto _label))))

(fn `UserConstructionScript`
  (`parent.UserConstructionScript`))