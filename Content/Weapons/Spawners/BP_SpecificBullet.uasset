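; BP_SpecificBullet is a weapons spawner actor that places a SpecificBullet in the world.
; Its SpawnPickup event spawns SpecificBullet at its own location and rotation, adjusting for collisions but always spawning, then destroys the spawner.
; BeginPlay, overlap and Tick are unused, and nothing in this graph calls SpawnPickup.
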(event `/Game/Weapons/Spawners/BP_BASERandomPickupSpawner.SpawnPickup`
  (bind (_returnvalue_location _returnvalue_rotation) (`KismetMathLibrary.BreakTransform` (`self.GetTransform`)))
  (`|SpawnActorFromClass` (`self.SpecificBullet`) (`KismetMathLibrary.MakeTransform` _returnvalue_location _returnvalue_rotation) "AdjustIfPossibleButAlwaysSpawn" "MultiplyWithRoot" null null)
  (`self.K2_DestroyActor`))

(fn `UserConstructionScript`
  (`parent.UserConstructionScript`))